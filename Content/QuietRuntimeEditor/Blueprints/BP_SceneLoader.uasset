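; Loads a JSON scene saved by the Quiet Runtime Editor and switches it into play when the level begins.
; On BeginPlay it spawns a temporary BP_QuietTreeManager in load mode, whose Serializer loads the named Scene from the save directory, then destroys it a tick later.
; If a Character exists, player 0 possesses it, game input captures the mouse, and BI_QuietActorsInterface actors have debug mode turned off.
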(event EventBeginPlay
  (bind _returnvalue (Game|SpawnActorfromClass "/Game/QuietRuntimeEditor/Blueprints/BP_QuietTreeManager.BP_QuietTreeManager_C" (Math|Transform|MakeTransform "0, 0, 0" "0, 0, 0" "1.000000,1.000000,1.000000") "AlwaysSpawn" 0 true 0))
  (Default|LoadScene (Variables|/Game/QuietRuntimeEditor/Blueprints/BP_QuietTreeManager.BP_QuietTreeManager_C|GetSerializer _returnvalue) (Utilities|Struct|MakeFilePath (Class|BlueprintPathsLibrary|SetExtension (Utilities|String|Append (CallFunction|GetSaveDirectory) "/" (Variables|SceneLoader|GetScene)) ".json")))
  (Utilities|FlowControl|DelayUntilNextTick)
  (Actor|DestroyActor _returnvalue)
  (bind _returnvalue_2 (Actor|GetActorOfClass "/Script/Engine.Character"))
  (Utilities|IsValid _returnvalue_2
    (:Is%20Valid
      (Pawn|Possess (Game|GetPlayerController 0) _returnvalue_2)
      (Variables|/Script/Engine.PlayerController|SetbShowMouseCursor (Game|GetPlayerController 0) false)
      (Class|GameplayStatics|SetViewportMouseCaptureMode "CapturePermanently")
      (Class|WidgetBlueprintLibrary|SetFocustoGameViewport)
      (bind _outactors (Actor|GetAllActorswithInterface "/Game/QuietRuntimeEditor/Common/QuietActors/Blueprints/BI_QuietActorsInterface.BI_QuietActorsInterface_C"))
      (for _array_element _outactors
        (Class|BIQuietActorsInterface|EnableDebugMode(Message) _array_element false)))))

(fn ConstructionScript)