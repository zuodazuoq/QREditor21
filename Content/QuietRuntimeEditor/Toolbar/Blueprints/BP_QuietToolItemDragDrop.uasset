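; Drag-and-drop operation for toolbar items in the Quiet Runtime Editor, carrying a WBP_ToolbarSmartButton as its payload.
; While dragged, it calls the button's HandleOnDragged and hides the default drag visual when that returns true.
; Both drop and cancel call the button's HandleOnSpawnEnded, so the spawn ends the same way in either case.
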(event EventDragged
  (params (PointerEvent :type Pointer%20Event%20Structure%20%28by%20ref%29))
  (bind _astoolbar_smart_button (Utilities|Casting|CastToWBP_ToolbarSmartButton (Variables|Default|GetPayload)))
  (bind _spawned (Default|HandleonDragged _astoolbar_smart_button))
  (if _spawned
    (Widget|SetVisibility (Variables|Default|GetDefaultDragVisual) "Hidden")))

(event EventDragCancelled
  (params (PointerEvent :type Pointer%20Event%20Structure%20%28by%20ref%29))
  (bind _astoolbar_smart_button (Utilities|Casting|CastToWBP_ToolbarSmartButton (Variables|Default|GetPayload)))
  (Default|HandleonSpawnEnded _astoolbar_smart_button))

(event EventDrop
  (params (PointerEvent :type Pointer%20Event%20Structure%20%28by%20ref%29))
  (bind _astoolbar_smart_button (Utilities|Casting|CastToWBP_ToolbarSmartButton (Variables|Default|GetPayload)))
  (Default|HandleonSpawnEnded _astoolbar_smart_button))