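; Actor component that makes its owner a selectable, nameable outliner item in the Quiet runtime editor, with a GUID, selection state and visibility.
; Owner clicks yield to gizmo hits or forward to thumbnail components, and otherwise request selection only if the cursor hasn't moved by release.
; Selection toggles a custom-depth outline and deselection destroys attached gizmos.
; Event dispatchers broadcast requests and state changes.
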(event Custom|SetVisibility
  (params (NewState :type Boolean))
  (bind _returnvalue (Components|GetOwner))
  ;[0 0 0] Visibility
  (Rendering|SetActorHiddenInGame _returnvalue (not NewState))
  (Collision|SetActorEnableCollision _returnvalue NewState)
  (Default|CallNotifyonVisibilityChanged NewState))

(event Custom|HandleOnReleased
  (params (TouchedActor :type Actor%20Object%20Reference) (ButtonReleased :type Key%20Structure :default "None"))
  (bind _returnvalue (Game|GetPlayerController 0))
  (bind (_locationx _locationy) (Game|Player|GetMousePosition _returnvalue))
  ;[0 0 0] Click Handlers
  (Utilities|FlowControl|Sequence
    (:then_0
      (Utilities|FlowControl|Gate true :!label _label
        (:Exit
          (if (Math|Vector|Equal(Vector) (stale Custom|HandleOnClicked _pinned) (Math|Vector2D|MakeVector2D _locationx _locationy) 0.01)
            (Default|CallRequesttoSelect (Components|GetOwner))))))
    (:then_1
      (goto _label Close))))

(event Custom|Select
  ;[0 0 0] Apply New Selection State
  (CallFunction|ShowSelectionOutline (Components|GetOwner) true)
  (Variables|Default|SetSelected true)
  (Default|CallNotifyonSelectionStateChanged true))

(event Custom|Deselect
  ;[0 0 0] Apply New Selection State
  (CallFunction|ShowSelectionOutline (Components|GetOwner) false)
  (Variables|Default|SetSelected false)
  (Default|CallNotifyonSelectionStateChanged false)
  (bind _arrayelement (Utilities|Array|ReverseforEachLoop (Actor|GetAttachedActors (Components|GetOwner) true false))
    (:LoopBody
      (if (Actor|ActorHasTag _arrayelement "QuietGizmo")
        (Actor|DestroyActor _arrayelement)))))

(event Custom|HandleOnClicked
  (params (TouchedActor :type Actor%20Object%20Reference) (ButtonPressed :type Key%20Structure :default "None"))
  (bind _returnvalue (Game|GetPlayerController 0))
  (bind _returnvalue_2 (Game|GetPlayerController 0))
  (bind (_hitresult _returnvalue_3) (Game|Player|GetHitResultUnderCursorbyChannel _returnvalue_2 "TraceTypeQuery4" true))
  (bind (_locationx _locationy) (Game|Player|GetMousePosition _returnvalue))
  (bind _returnvalue_4 (Math|Vector2D|MakeVector2D _locationx _locationy))
  ;[0 0 0] Click Handlers
  (if (not (.ReturnValue (Game|Player|GetHitResultUnderCursorbyChannel (Game|GetPlayerController 0) "TraceTypeQuery3" false)))
    (if _returnvalue_3
      ;;[0 0 0] Throw Click to Thumbnail
      (bind _treecomponent (CallFunction|GetQuietOutlinerComponent (.HitActor (Collision|BreakHitResult _hitresult))))
      (CallFunction|EmulateClick _treecomponent)
      (else
        (bind _pinned (Utilities|Pin _returnvalue_4))
        (Utilities|FlowControl|Gate true) ; enters at Open
      ))))

(event Custom|EmulateClick
  ;[0 0 0] Emulate Click
  (Default|CallRequesttoSelect (Components|GetOwner)))

(event EventBeginPlay
  (bind _returnvalue (Components|GetOwner))
  ;[0.000644 0.01182 0.03125] Setup Bindings
  (EventDispatchers|BindEventtoOnClicked _returnvalue (EventDispatchers|CreateEvent :!event Custom|HandleOnClicked))
  (EventDispatchers|BindEventtoOnReleased _returnvalue (EventDispatchers|CreateEvent :!event Custom|HandleOnReleased)))

(fn GetName
  (return (Variables|Default|GetName)))

(fn GetGuid
  (return (Variables|Default|GetGuid)))

(fn Rename
  (params (NewName :type String) (Notify :type Boolean))
  (Utilities|FlowControl|Sequence
    (:then_0
      (if Notify
        (Default|CallNotifyonRenamed (Variables|Default|GetName) NewName (Variables|Default|GetGuid))))
    (:then_1
      (Variables|Default|SetName NewName))))

(fn ShowSelectionOutline
  (params (Actor :type Actor%20Object%20Reference) (bShow :type Boolean))
  (if (not (Utilities|Array|ContainsItem (Variables|Default|GetOutlineIgnored%20Classes) (Utilities|ResolveSoftReference (Utilities|GetClass Actor))))
    (for _array_element (Actor|GetComponentsByClass Actor "/Script/Engine.PrimitiveComponent")
      (if (not (Components|ComponentHasTag _array_element "Debug"))
        (Rendering|SetRenderCustomDepth _array_element bShow)))))

(fn GetSelectionState
  (return (Variables|Default|GetSelected)))

(fn SetGuid
  (params (Guid :type Guid%20Structure))
  (Variables|Default|SetGuid Guid))

(fn UnbindAll
  (EventDispatchers|UnbindallEventsfromRequesttoRename)
  (EventDispatchers|UnbindallEventsfromRequesttoSelect)
  (EventDispatchers|UnbindallEventsfromRequesttoDestroy)
  (EventDispatchers|UnbindallEventsfromNotifyonRenamed)
  (EventDispatchers|UnbindallEventsfromNotifyonNameRestored)
  (EventDispatchers|UnbindallEventsfromRequesttoDuplicate)
  (EventDispatchers|UnbindallEventsfromNotifyonVisibilityChanged)
  (EventDispatchers|UnbindallEventsfromRequesttoChangeVisibility)
  (EventDispatchers|UnbindallEventsfromNotifyonSelectionStateChanged)
  (EventDispatchers|UnbindallEventsfromRequesttoSave))