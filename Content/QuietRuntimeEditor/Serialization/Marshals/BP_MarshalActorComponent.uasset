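; BP_MarshalActorComponent is a Quiet Runtime Editor serialization marshal that saves, reads and restores the ComponentTags of an ActorComponent as JSON.
; SerializeObject writes the tags into a target JSON object, and GetPropertyValue returns them wrapped in a new JSON object under the property name.
; RestoreObject checks that the field exists and passes it to SetPropertyValue, which assigns the tags only when they differ and then reports the change.
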(fn SerializeObject
  (params (Object :type Object%20Object%20Reference) (TargetJson :type Json%20Object%20Wrapper%20Structure%20%28by%20ref%29))
  (bind _asactor_component (Utilities|Casting|CastToActorComponent Object))
  (|SetJsonField TargetJson "ComponentTags" (Variables|/Script/Engine.ActorComponent|GetComponentTags _asactor_component))
  (return))

(fn GetPropertyValue
  (params (Object :type Object%20Object%20Reference) (Property :type String))
  (bind _asactor_component (Utilities|Casting|CastToActorComponent Object))
  (bind _outjsonobject (Class|JsonBlueprintFunctionLibrary|FromString "{ }"))
  (switch string Property
    (:ComponentTags
      (|SetJsonField _outjsonobject Property (Variables|/Script/Engine.ActorComponent|GetComponentTags _asactor_component))
      (return true _outjsonobject))))

(fn SetPropertyValue
  (params (Object :type Object%20Object%20Reference) (Property :type String) (JsonValue :type Json%20Object%20Wrapper%20Structure%20%28by%20ref%29))
  (bind _asactor_component (Utilities|Casting|CastToActorComponent Object))
  (switch string Property
    (:ComponentTags
      (bind (_outvalue _returnvalue) (|GetJsonField JsonValue "ComponentTags"))
      (if _returnvalue
        (if (not (Utilities|Array|Identical _outvalue (Variables|/Script/Engine.ActorComponent|GetComponentTags _asactor_component)))
          (Variables|/Script/Engine.ActorComponent|SetComponentTags _asactor_component _outvalue)
          (return true))))))

(fn RestoreObject
  (params (Object :type Object%20Object%20Reference) (JsonObject :type Json%20Object%20Wrapper%20Structure))
  (bind _returnvalue (Class|JsonBlueprintFunctionLibrary|HasField JsonObject "ComponentTags"))
  (if _returnvalue
    (CallFunction|SetPropertyValue Object "ComponentTags" JsonObject)))