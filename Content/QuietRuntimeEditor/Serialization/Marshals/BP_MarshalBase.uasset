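; Base marshal for the Quiet Runtime Editor, with stub serialize, restore, property and action functions for subclasses to override.
; Make*Param helpers build typed JSON property descriptors through FillJsonParam, wrapping current and default values under the property name and adding type-specific settings.
; Array and structure builders nest element descriptors, but write current values into DefaultValue too.
; GetSource fetches the owner's BP_QuietSerializer component.
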(fn SerializeObject
  (params (Object :type Object%20Object%20Reference) (TargetJson :type Json%20Object%20Wrapper%20Structure%20%28by%20ref%29))
  (return))

(fn SetPropertyValue
  (params (Object :type Object%20Object%20Reference) (Property :type String) (JsonValue :type Json%20Object%20Wrapper%20Structure%20%28by%20ref%29))
  (return false))

(fn RestoreObject
  (params (Object :type Object%20Object%20Reference) (JsonObject :type Json%20Object%20Wrapper%20Structure)))

(fn CollectProperties
  (params (Object :type Object%20Object%20Reference) (TargetJson :type Json%20Object%20Wrapper%20Structure%20%28by%20ref%29))
  (return))

(fn GetPropertyValue
  (params (Object :type Object%20Object%20Reference) (Property :type String))
  (return false ""))

(fn MakeParamJson
  (params (Type :type String) (Name :type String) (DisplayName :type String) (Description :type String))
  (bind _jsonobject (CallFunction|NewJson))
  (|SetJsonField _jsonobject "Type" Type)
  (|SetJsonField _jsonobject "Name" Name)
  (|SetJsonField _jsonobject "DisplayName" DisplayName)
  (|SetJsonField _jsonobject "Description" Description)
  (return _jsonobject))

(fn MakeFloatSettings
  (params (MinValue :type Float%20%28double-precision%29) (MinSliderValue :type Float%20%28double-precision%29) (MaxValue :type Float%20%28double-precision%29) (MaxSliderValue :type Float%20%28double-precision%29) (MinFractionalDigits :type Integer) (MaxFractionalDigits :type Integer))
  (bind _jsonobject (CallFunction|NewJson))
  (|SetJsonField _jsonobject "MinValue" MinValue)
  (|SetJsonField _jsonobject "MinSliderValue" MinSliderValue)
  (|SetJsonField _jsonobject "MaxValue" MaxValue)
  (|SetJsonField _jsonobject "MaxSliderValue" MaxSliderValue)
  (|SetJsonField _jsonobject "MinFractionalDigits" MinFractionalDigits)
  (|SetJsonField _jsonobject "MaxFractionalDigits" MaxFractionalDigits)
  (return _jsonobject))

(fn MakeFloatParam
  (params (Name :type String) (DisplayName :type String) (Description :type String) (Value :type Float%20%28double-precision%29) (DefaultValue :type Float%20%28double-precision%29) (MinValue :type Float%20%28double-precision%29) (MinSliderValue :type Float%20%28double-precision%29) (MaxValue :type Float%20%28double-precision%29) (MaxSliderValue :type Float%20%28double-precision%29) (MinFractionalDigits :type Integer) (MaxFractionalDigits :type Integer))
  (bind _jsonobject (Utilities|FillJsonParam "Float" Name DisplayName Description Value DefaultValue))
  (|SetJsonField _jsonobject "Settings" (MakeParam|MakeFloatSettings MinValue MinSliderValue MaxValue MaxSliderValue MinFractionalDigits MaxFractionalDigits))
  (return _jsonobject))

(fn MakeIntParam
  (params (Name :type String) (DisplayName :type String) (Description :type String) (Value :type Integer) (DefaultValue :type Integer) (MinValue :type Integer) (MinSliderValue :type Integer) (MaxValue :type Integer) (MaxSliderValue :type Integer))
  (bind _jsonobject (Utilities|FillJsonParam "Integer" Name DisplayName Description Value DefaultValue))
  (bind _jsonobject_2 (CallFunction|NewJson))
  (|SetJsonField _jsonobject_2 "MinValue" MinValue)
  (|SetJsonField _jsonobject_2 "MinSliderValue" MinSliderValue)
  (|SetJsonField _jsonobject_2 "MaxValue" MaxValue)
  (|SetJsonField _jsonobject_2 "MaxSliderValue" MaxSliderValue)
  (|SetJsonField _jsonobject "Settings" _jsonobject_2)
  (return _jsonobject))

(fn MakeBoolParam
  (params (Name :type String) (DisplayName :type String) (Description :type String) (Value :type Boolean) (DefaultValue :type Boolean))
  (bind _jsonobject (Utilities|FillJsonParam "Boolean" Name DisplayName Description Value DefaultValue))
  (return _jsonobject))

(fn MakeStringParam
  (params (Name :type String) (DisplayName :type String) (Description :type String) (Value :type String) (DefaultValue :type String))
  (bind _jsonobject (Utilities|FillJsonParam "String" Name DisplayName Description Value DefaultValue))
  (return _jsonobject))

(fn MakeVectorParam
  (params (Name :type String) (DisplayName :type String) (Description :type String) (Value :type Vector) (DefaultValue :type Vector))
  (bind _jsonobject (Utilities|FillJsonParam "Vector" Name DisplayName Description Value DefaultValue))
  (return _jsonobject))

(fn MakeLinearColorParam
  (params (Name :type String) (DisplayName :type String) (Description :type String) (Value :type Linear%20Color%20Structure) (DefaultValue :type Linear%20Color%20Structure))
  (bind _jsonobject (Utilities|FillJsonParam "LinearColor" Name DisplayName Description Value DefaultValue))
  (return _jsonobject))

(fn MakeObjectParam
  (params (Name :type String) (DisplayName :type String) (Description :type String) (Class :type Object%20Class%20Reference) (Value :type Object%20Object%20Reference) (DefaultValue :type Object%20Object%20Reference))
  (bind _jsonobject (Utilities|FillJsonParam "Asset" Name DisplayName Description Value DefaultValue))
  (|SetJsonField _jsonobject "ObjectClass" Class)
  (return _jsonobject))

(fn MakeComboStringParam
  (params (Name :type String) (DisplayName :type String) (Description :type String) (Options :type Array%20of%20Strings) (Value :type String) (DefaultValue :type String))
  (bind _jsonobject (Utilities|FillJsonParam "Combo" Name DisplayName Description Value DefaultValue))
  (|SetJsonField _jsonobject "Options" Options)
  (return _jsonobject))

(fn MakeStructureParam
  (params (Name :type String) (DisplayName :type String) (Description :type String) (Members :type Map%20of%20Strings%20to%20Structs))
  (bind _jsonobject (MakeParam|MakeParamJson "Structure" Name DisplayName Description))
  (|SetJsonField _jsonobject "Elements" Members)
  (bind _keys (Utilities|Map|Keys Members))
  (for _array_element _keys
    (bind _outvalue (|GetJsonField (.Value (Utilities|Map|Find Members _array_element)) "Value"))
    (Utilities|Array|Add (LocalVariables|GetArray) _outvalue)
    (bind _outvalue_2 (|GetJsonField (.Value (Utilities|Map|Find Members _array_element)) "DefaultValue"))
    (Utilities|Array|Add (LocalVariables|GetDefaultArray) _outvalue_2))
  (bind _jsonobject_2 (CallFunction|NewJson))
  (|SetJsonField _jsonobject_2 Name (LocalVariables|GetArray))
  (|SetJsonField _jsonobject "Value" _jsonobject_2)
  (bind _jsonobject_3 (CallFunction|NewJson))
  (|SetJsonField _jsonobject_3 Name (LocalVariables|GetArray))
  (|SetJsonField _jsonobject "DefaultValue" _jsonobject_3)
  (return _jsonobject))

(fn MakeArrayParam
  (params (Name :type String) (DisplayName :type String) (Description :type String) (Items :type Array%20of%20Json%20Object%20Wrapper%20Structures) (DefaultItem :type Json%20Object%20Wrapper%20Structure))
  (bind _jsonobject (MakeParam|MakeParamJson "Array" Name DisplayName Description))
  (|SetJsonField _jsonobject "Elements" Items)
  (|SetJsonField _jsonobject "DefaultElement" DefaultItem)
  (for _array_element Items
    (bind _outvalue (|GetJsonField _array_element "Value"))
    (Utilities|Array|Add (LocalVariables|GetArray) _outvalue)
    (bind _outvalue_2 (|GetJsonField _array_element "DefaultValue"))
    (Utilities|Array|Add (LocalVariables|GetDefaultArray) _outvalue_2))
  (bind _jsonobject_2 (CallFunction|NewJson))
  (|SetJsonField _jsonobject_2 Name (LocalVariables|GetArray))
  (|SetJsonField _jsonobject "Value" _jsonobject_2)
  (bind _jsonobject_3 (CallFunction|NewJson))
  (|SetJsonField _jsonobject_3 Name (LocalVariables|GetArray))
  (|SetJsonField _jsonobject "DefaultValue" _jsonobject_3)
  (return _jsonobject))

(fn MakeEnumParam
  (params (Name :type String) (DisplayName :type String) (Description :type String) (Options :type Array%20of%20Strings) (Value :type Integer) (DefaultValue :type Integer))
  (bind _jsonobject (Utilities|FillJsonParam "Enum" Name DisplayName Description Value DefaultValue))
  (|SetJsonField _jsonobject "Options" Options)
  (return _jsonobject))

(fn MakeParamSubgroup
  (params (DisplayName :type String) (Members :type Array%20of%20Json%20Object%20Wrapper%20Structures))
  (bind _jsonobject (MakeParam|MakeParamJson "Subgroup" DisplayName DisplayName))
  (|SetJsonField _jsonobject "Value" Members)
  (return _jsonobject))

(fn MakeLightingChannelsParam
  (params (Name :type String) (DisplayName :type String) (Description :type String) (Value :type Lighting%20Channels%20Structure) (DefaultValue :type Lighting%20Channels%20Structure))
  (bind _jsonobject (Utilities|FillJsonParam "LightingChannels" Name DisplayName Description Value DefaultValue))
  (return _jsonobject))

(fn GetSource
  (return (Actor|GetComponentbyClass (Components|GetOwner) "/Game/QuietRuntimeEditor/Serialization/BP_QuietSerializer.BP_QuietSerializer_C")))

(fn MakeTextureParam
  (params (Name :type String) (DisplayName :type String) (Description :type String) (Value :type Object%20Object%20Reference) (DefaultValue :type Object%20Object%20Reference) (NoneTexture :type Texture%202D%20Soft%20Object%20Reference))
  (bind _jsonobject (Utilities|FillJsonParam "Texture" Name DisplayName Description Value DefaultValue))
  (|SetJsonField _jsonobject "NoneTexture" NoneTexture)
  (return _jsonobject))

(fn CallAction
  (params (Object :type Object%20Object%20Reference) (Action :type Json%20Object%20Wrapper%20Structure))
  (return false))

(fn MakeVector2DParam
  (params (Name :type String) (DisplayName :type String) (Description :type String) (Value :type Vector%202D%20Structure) (DefaultValue :type Vector%202D%20Structure))
  (bind _jsonobject (Utilities|FillJsonParam "Vector2D" Name DisplayName Description Value DefaultValue))
  (return _jsonobject))