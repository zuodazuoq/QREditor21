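; Marshal that serializes a base material's dynamic instance parameters to JSON for the Quiet runtime editor.
; CollectProperties reads each scalar, vector and texture parameter with its default and wraps it in typed descriptors with ranges and fallback dummy textures.
; Descriptors are grouped into Diffuse, Metallic, Roughness, Emissive, Normal, UV Mapping and Fuzzy Shading, then written as JSON fields alongside a GroupsState list.
; Enable toggles are scalar parameters converted to bools.
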(fn CollectProperties
  (params (Object :type Object%20Object%20Reference) (TargetJson :type Json%20Object%20Wrapper%20Structure%20%28by%20ref%29))
  (bind _asmaterial_instance_dynamic (Utilities|Casting|CastToMaterialInstanceDynamic Object))
  (LocalVariables|SetMaterial _asmaterial_instance_dynamic)
  (Utilities|FlowControl|Sequence
    (:then_0
      ;[0 0 0] Diffuse Group
      (bind (_value _defaultvalue) (CallFunction|GetVectorValue (LocalVariables|GetMaterial) "Diffuse Color"))
      (bind _jsonobject (CallFunction|MakeLinearColorParam "Diffuse Color" "Diffuse Color" "" _value _defaultvalue))
      (Utilities|Array|Add (LocalVariables|GetDiffuse) _jsonobject)
      (bind (_value_2 _defaultvalue_2) (CallFunction|GetScalarValue (LocalVariables|GetMaterial) "Enable Diffuse Texture"))
      (bind _jsonobject_2 (CallFunction|MakeBoolParam "Enable Diffuse Texture" "Enable Diffuse Texture" "" (Math|Conversions|ToBoolean(Integer) (Math|Float|Truncate _value_2)) (Math|Conversions|ToBoolean(Integer) (Math|Float|Truncate _defaultvalue_2))))
      (Utilities|Array|Add (LocalVariables|GetDiffuse) _jsonobject_2)
      (bind (_value_3 _defaultvalue_3) (CallFunction|GetTextureValue (LocalVariables|GetMaterial) "Diffuse Texture"))
      (bind _jsonobject_3 (CallFunction|MakeTextureParam "Diffuse Texture" "Diffuse Texture" "" _value_3 _defaultvalue_3 "/Game/QuietRuntimeEditor/Common/Textures/T_Dummy_BC.T_Dummy_BC"))
      (Utilities|Array|Add (LocalVariables|GetDiffuse) _jsonobject_3))
    (:then_1
      ;[0 0 0] Metallic Group
      (bind (_value_4 _defaultvalue_4) (CallFunction|GetScalarValue (LocalVariables|GetMaterial) "Metallic"))
      (bind _jsonobject_4 (CallFunction|MakeFloatParam "Metallic" "Metallic" "" _value_4 _defaultvalue_4 0.0 0.0 1.0 1.0 1 3))
      (Utilities|Array|Add (LocalVariables|GetMetallic) _jsonobject_4)
      (bind (_value_5 _defaultvalue_5) (CallFunction|GetScalarValue (LocalVariables|GetMaterial) "Enable Metallic Texture"))
      (bind _jsonobject_5 (CallFunction|MakeBoolParam "Enable Metallic Texture" "Enable Metallic Texture" "" (Math|Conversions|ToBoolean(Integer) (Math|Float|Truncate _value_5)) (Math|Conversions|ToBoolean(Integer) (Math|Float|Truncate _defaultvalue_5))))
      (Utilities|Array|Add (LocalVariables|GetMetallic) _jsonobject_5)
      (bind (_value_6 _defaultvalue_6) (CallFunction|GetTextureValue (LocalVariables|GetMaterial) "Metallic Texture"))
      (bind _jsonobject_6 (CallFunction|MakeTextureParam "Metallic Texture" "Metallic Texture" "" _value_6 _defaultvalue_6 "/Game/QuietRuntimeEditor/Common/Textures/T_Dummy_BC.T_Dummy_BC"))
      (Utilities|Array|Add (LocalVariables|GetMetallic) _jsonobject_6))
    (:then_2
      ;[0 0 0] Roughness Group
      (bind (_value_7 _defaultvalue_7) (CallFunction|GetScalarValue (LocalVariables|GetMaterial) "Roughness"))
      (bind _jsonobject_7 (CallFunction|MakeFloatParam "Roughness" "Roughness" "" _value_7 _defaultvalue_7 0.0 0.0 1.0 1.0 1 3))
      (Utilities|Array|Add (LocalVariables|GetRoughness) _jsonobject_7)
      (bind (_value_8 _defaultvalue_8) (CallFunction|GetScalarValue (LocalVariables|GetMaterial) "Enable Roughness Texture"))
      (bind _jsonobject_8 (CallFunction|MakeBoolParam "Enable Roughness Texture" "Enable Roughness Texture" "" (Math|Conversions|ToBoolean(Integer) (Math|Float|Truncate _value_8)) (Math|Conversions|ToBoolean(Integer) (Math|Float|Truncate _defaultvalue_8))))
      (Utilities|Array|Add (LocalVariables|GetRoughness) _jsonobject_8)
      (bind (_value_9 _defaultvalue_9) (CallFunction|GetTextureValue (LocalVariables|GetMaterial) "Roughness Texture"))
      (bind _jsonobject_9 (CallFunction|MakeTextureParam "Roughness Texture" "Roughness Texture" "" _value_9 _defaultvalue_9 "/Game/QuietRuntimeEditor/Common/Textures/T_Dummy_BC.T_Dummy_BC"))
      (Utilities|Array|Add (LocalVariables|GetRoughness) _jsonobject_9)
      (bind (_value_10 _defaultvalue_10) (CallFunction|GetScalarValue (LocalVariables|GetMaterial) "Roughness Power"))
      (bind _jsonobject_10 (CallFunction|MakeFloatParam "Roughness Power" "Roughness Power" "" _value_10 _defaultvalue_10 0.1 0.1 5.0 1e+01 1 2))
      (Utilities|Array|Add (LocalVariables|GetRoughness) _jsonobject_10)
      (bind (_value_11 _defaultvalue_11) (CallFunction|GetScalarValue (LocalVariables|GetMaterial) "Specular"))
      (bind _jsonobject_11 (CallFunction|MakeFloatParam "Specular" "Specular" "" _value_11 _defaultvalue_11 0.0 0.0 1.0 1.0 1 3))
      (Utilities|Array|Add (LocalVariables|GetRoughness) _jsonobject_11))
    (:then_3
      ;[0 0 0] Metallic Group
      (bind (_value_12 _defaultvalue_12) (CallFunction|GetScalarValue (LocalVariables|GetMaterial) "Emissive Multiplier"))
      (bind _jsonobject_12 (CallFunction|MakeFloatParam "Emissive Multiplier" "Emissive Multiplier" "" _value_12 _defaultvalue_12 0.0 0.0 1.0 1.0 1 3))
      (Utilities|Array|Add (LocalVariables|GetEmissive) _jsonobject_12)
      (bind (_value_13 _defaultvalue_13) (CallFunction|GetScalarValue (LocalVariables|GetMaterial) "Enable Emissive Texture"))
      (bind _jsonobject_13 (CallFunction|MakeBoolParam "Enable Emissive Texture" "Enable Emissive Texture" "" (Math|Conversions|ToBoolean(Integer) (Math|Float|Truncate _value_13)) (Math|Conversions|ToBoolean(Integer) (Math|Float|Truncate _defaultvalue_13))))
      (Utilities|Array|Add (LocalVariables|GetEmissive) _jsonobject_13)
      (bind (_value_14 _defaultvalue_14) (CallFunction|GetTextureValue (LocalVariables|GetMaterial) "Emissive Texture"))
      (bind _jsonobject_14 (CallFunction|MakeTextureParam "Emissive Texture" "Emissive Texture" "" _value_14 _defaultvalue_14 "/Game/QuietRuntimeEditor/Common/Textures/T_Dummy_BC.T_Dummy_BC"))
      (Utilities|Array|Add (LocalVariables|GetEmissive) _jsonobject_14))
    (:then_4
      ;[0 0 0] Normal Group
      (bind (_value_15 _defaultvalue_15) (CallFunction|GetTextureValue (LocalVariables|GetMaterial) "Normal Texture"))
      (bind _jsonobject_15 (CallFunction|MakeTextureParam "Normal Texture" "Normal Texture" "" _value_15 _defaultvalue_15 "/Game/QuietRuntimeEditor/Common/Textures/T_Dummy_N.T_Dummy_N"))
      (Utilities|Array|Add (LocalVariables|GetNormal) _jsonobject_15)
      (bind (_value_16 _defaultvalue_16) (CallFunction|GetScalarValue (LocalVariables|GetMaterial) "Flatten Normal"))
      (bind _jsonobject_16 (CallFunction|MakeFloatParam "Flatten Normal" "Flatten Normal" "" _value_16 _defaultvalue_16 0.0 0.0 1.0 1.0 1 3))
      (Utilities|Array|Add (LocalVariables|GetNormal) _jsonobject_16)
      (bind (_value_17 _defaultvalue_17) (CallFunction|GetScalarValue (LocalVariables|GetMaterial) "Enable Additional Normal"))
      (bind _jsonobject_17 (CallFunction|MakeBoolParam "Enable Additional Normal" "Enable Additional Normal" "" (Math|Conversions|ToBoolean(Integer) (Math|Float|Truncate _value_17)) (Math|Conversions|ToBoolean(Integer) (Math|Float|Truncate _defaultvalue_17))))
      (Utilities|Array|Add (LocalVariables|GetNormal) _jsonobject_17)
      (bind (_value_18 _defaultvalue_18) (CallFunction|GetTextureValue (LocalVariables|GetMaterial) "Additional Normal Texture"))
      (bind _jsonobject_18 (CallFunction|MakeTextureParam "Additional Normal Texture" "Additional Normal Texture" "" _value_18 _defaultvalue_18 "/Game/QuietRuntimeEditor/Common/Textures/T_Dummy_N.T_Dummy_N"))
      (Utilities|Array|Add (LocalVariables|GetNormal) _jsonobject_18)
      (bind (_value_19 _defaultvalue_19) (CallFunction|GetScalarValue (LocalVariables|GetMaterial) "Additional Flatten Normal"))
      (bind _jsonobject_19 (CallFunction|MakeFloatParam "Additional Flatten Normal" "Additional Flatten Normal" "" _value_19 _defaultvalue_19 0.0 0.0 1.0 1.0 1 3))
      (Utilities|Array|Add (LocalVariables|GetNormal) _jsonobject_19)
      (bind (_value_20 _defaultvalue_20) (CallFunction|GetScalarValue (LocalVariables|GetMaterial) "Additional Normal Tiling"))
      (bind _jsonobject_20 (CallFunction|MakeFloatParam "Additional Normal Tiling" "Additional Normal Tiling" "" _value_20 _defaultvalue_20 0.01 0.01 1e+02 1e+03 1 3))
      (Utilities|Array|Add (LocalVariables|GetNormal) _jsonobject_20))
    (:then_5
      ;[0 0 0] UV Mapping
      (bind (_value_21 _defaultvalue_21) (CallFunction|GetScalarValue (LocalVariables|GetMaterial) "Tiling"))
      (bind _jsonobject_21 (CallFunction|MakeFloatParam "Tiling" "Tiling" "" _value_21 _defaultvalue_21 0.01 0.01 1e+02 1e+03 1 3))
      (Utilities|Array|Add (LocalVariables|GetUV%20Mapping) _jsonobject_21)
      (bind (_value_22 _defaultvalue_22) (CallFunction|GetScalarValue (LocalVariables|GetMaterial) "Angle"))
      (bind _jsonobject_22 (CallFunction|MakeFloatParam "Angle" "Angle" "" _value_22 _defaultvalue_22 0.0 0.0 3.6e+02 3.6e+02 1 1))
      (Utilities|Array|Add (LocalVariables|GetUV%20Mapping) _jsonobject_22)
      (bind (_value_23 _defaultvalue_23) (CallFunction|GetScalarValue (LocalVariables|GetMaterial) "U Offset"))
      (bind _jsonobject_23 (CallFunction|MakeFloatParam "U Offset" "U Offset" "" _value_23 _defaultvalue_23 -1e+02 -1.0 1.0 1e+02 1 3))
      (Utilities|Array|Add (LocalVariables|GetUV%20Mapping) _jsonobject_23)
      (bind (_value_24 _defaultvalue_24) (CallFunction|GetScalarValue (LocalVariables|GetMaterial) "V Offset"))
      (bind _jsonobject_24 (CallFunction|MakeFloatParam "V Offset" "V Offset" "" _value_24 _defaultvalue_24 -1e+02 -1.0 1.0 1e+02 1 3))
      (Utilities|Array|Add (LocalVariables|GetUV%20Mapping) _jsonobject_24))
    (:then_6
      ;[0 0 0] Fuzzy Shading
      (bind (_value_25 _defaultvalue_25) (CallFunction|GetScalarValue (LocalVariables|GetMaterial) "Enable Fuzzy Shading"))
      (bind _jsonobject_25 (CallFunction|MakeBoolParam "Enable Fuzzy Shading" "Enable Fuzzy Shading" "" (Math|Conversions|ToBoolean(Integer) (Math|Float|Truncate _value_25)) (Math|Conversions|ToBoolean(Integer) (Math|Float|Truncate _defaultvalue_25))))
      (Utilities|Array|Add (LocalVariables|GetFuzzy%20Shading) _jsonobject_25)
      (bind (_value_26 _defaultvalue_26) (CallFunction|GetScalarValue (LocalVariables|GetMaterial) "Fuzzy Shading Weight"))
      (bind _jsonobject_26 (CallFunction|MakeFloatParam "Fuzzy Shading Weight" "Fuzzy Shading Weight" "" _value_26 _defaultvalue_26 0.0 0.0 1.0 1.0 1 3))
      (Utilities|Array|Add (LocalVariables|GetFuzzy%20Shading) _jsonobject_26)
      (bind (_value_27 _defaultvalue_27) (CallFunction|GetTextureValue (LocalVariables|GetMaterial) "Fuzzy Normal Texture"))
      (bind _jsonobject_27 (CallFunction|MakeTextureParam "Fuzzy Normal Texture" "Fuzzy Normal Texture" "" _value_27 _defaultvalue_27 "/Game/QuietRuntimeEditor/Common/Textures/T_Dummy_N.T_Dummy_N"))
      (Utilities|Array|Add (LocalVariables|GetFuzzy%20Shading) _jsonobject_27)
      (bind (_value_28 _defaultvalue_28) (CallFunction|GetScalarValue (LocalVariables|GetMaterial) "Fuzzy Flatten Normal"))
      (bind _jsonobject_28 (CallFunction|MakeFloatParam "Fuzzy Flatten Normal" "Fuzzy Flatten Normal" "" _value_28 _defaultvalue_28 0.0 0.0 1.0 1.0 1 3))
      (Utilities|Array|Add (LocalVariables|GetFuzzy%20Shading) _jsonobject_28)
      (bind (_value_29 _defaultvalue_29) (CallFunction|GetVectorValue (LocalVariables|GetMaterial) "Fuzzy Color"))
      (bind _jsonobject_29 (CallFunction|MakeLinearColorParam "Fuzzy Color" "Fuzzy Color" "" _value_29 _defaultvalue_29))
      (Utilities|Array|Add (LocalVariables|GetFuzzy%20Shading) _jsonobject_29)
      (bind (_value_30 _defaultvalue_30) (CallFunction|GetScalarValue (LocalVariables|GetMaterial) "Fuzzy Core Darkness"))
      (bind _jsonobject_30 (CallFunction|MakeFloatParam "Fuzzy Core Darkness" "Fuzzy Core Darkness" "" _value_30 _defaultvalue_30 0.0 0.0 6.0 3.0 1 3))
      (Utilities|Array|Add (LocalVariables|GetFuzzy%20Shading) _jsonobject_30)
      (bind (_value_31 _defaultvalue_31) (CallFunction|GetScalarValue (LocalVariables|GetMaterial) "Fuzzy Power"))
      (bind _jsonobject_31 (CallFunction|MakeFloatParam "Fuzzy Power" "Fuzzy Power" "" _value_31 _defaultvalue_31 0.0 0.0 5e+01 18.0 1 3))
      (Utilities|Array|Add (LocalVariables|GetFuzzy%20Shading) _jsonobject_31)
      (bind (_value_32 _defaultvalue_32) (CallFunction|GetScalarValue (LocalVariables|GetMaterial) "Fuzzy Edge Brightness"))
      (bind _jsonobject_32 (CallFunction|MakeFloatParam "Fuzzy Edge Brightness" "Fuzzy Edge Brightness" "" _value_32 _defaultvalue_32 0.0 0.0 5e+01 18.0 1 3))
      (Utilities|Array|Add (LocalVariables|GetFuzzy%20Shading) _jsonobject_32))
    (:then_7
      ;[0 0 0] COLLECT
      (|SetJsonField TargetJson "GroupsState" (Utilities|Array|MakeArray "Diffuse" "Normal"))
      (|SetJsonField TargetJson "Diffuse" (LocalVariables|GetDiffuse))
      (|SetJsonField TargetJson "Metallic" (LocalVariables|GetMetallic))
      (|SetJsonField TargetJson "Roughness" (LocalVariables|GetRoughness))
      (|SetJsonField TargetJson "Emissive" (LocalVariables|GetEmissive))
      (|SetJsonField TargetJson "Normal" (LocalVariables|GetNormal))
      (|SetJsonField TargetJson "UV Mapping" (LocalVariables|GetUV%20Mapping))
      (|SetJsonField TargetJson "Fuzzy Shading" (LocalVariables|GetFuzzy%20Shading))
      (return))))