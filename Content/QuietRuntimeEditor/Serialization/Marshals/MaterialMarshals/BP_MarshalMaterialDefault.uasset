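; Default material marshal for the runtime editor, serializing a dynamic material instance's editable parameters to JSON.
; Walks the scalar, vector and texture overrides on the first-level instance below the root material, skipping IgnoredProperties.
; Pairs each current value with that instance's value as default, and gives textures a normal or base-color dummy as their None option.
; Writes a group list plus each non-empty parameter array into the target JSON.
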(fn CollectProperties
  (params (Object :type Object%20Object%20Reference) (TargetJson :type Json%20Object%20Wrapper%20Structure%20%28by%20ref%29))
  (bind _asmaterial_instance_dynamic (Utilities|Casting|CastToMaterialInstanceDynamic Object))
  (bind _output_get (LocalVariables|SetMaterial _asmaterial_instance_dynamic))
  (bind _firstlevelinstance (Default|FindRootParentMaterial (CallFunction|GetSource) _output_get))
  (LocalVariables|SetParent _firstlevelinstance)
  (Utilities|FlowControl|Sequence
    (:then_0
      (for _array_element (Variables|/Script/Engine.MaterialInstance|GetScalarParameterValues (LocalVariables|GetParent))
        (Utilities|FilterProperty (.name (.ParameterInfo (Utilities|Struct|BreakScalarParameterValue _array_element))) (LocalVariables|GetIgnoredProperties))
        (bind _returnvalue (Rendering|Material|GetScalarParameterValue (LocalVariables|GetMaterial) (.name (.ParameterInfo (Utilities|Struct|BreakScalarParameterValue _array_element))) :!class /Script/Engine.MaterialInstanceDynamic))
        (bind _jsonobject (CallFunction|MakeFloatParam (Utilities|String|ToString(Name) (.name (.ParameterInfo (Utilities|Struct|BreakScalarParameterValue _array_element)))) (Utilities|String|ToString(Name) (.name (.ParameterInfo (Utilities|Struct|BreakScalarParameterValue _array_element)))) "" _returnvalue (.ParameterValue (Utilities|Struct|BreakScalarParameterValue _array_element)) 0.0 0.0 0.0 0.0 1 3))
        (Utilities|Array|Add (LocalVariables|GetScalars) _jsonobject)))
    (:then_1
      (for _array_element_2 (Variables|/Script/Engine.MaterialInstance|GetVectorParameterValues (LocalVariables|GetParent))
        (Utilities|FilterProperty (.name (.ParameterInfo (Utilities|Struct|BreakVectorParameterValue _array_element_2))) (LocalVariables|GetIgnoredProperties))
        (bind _returnvalue_2 (Rendering|Material|GetVectorParameterValue (LocalVariables|GetMaterial) (.name (.ParameterInfo (Utilities|Struct|BreakVectorParameterValue _array_element_2))) :!class /Script/Engine.MaterialInstanceDynamic))
        (bind _jsonobject_2 (CallFunction|MakeLinearColorParam (Utilities|String|ToString(Name) (.name (.ParameterInfo (Utilities|Struct|BreakVectorParameterValue _array_element_2)))) (Utilities|String|ToString(Name) (.name (.ParameterInfo (Utilities|Struct|BreakVectorParameterValue _array_element_2)))) "" _returnvalue_2 (.ParameterValue (Utilities|Struct|BreakVectorParameterValue _array_element_2))))
        (Utilities|Array|Add (LocalVariables|GetColors) _jsonobject_2)))
    (:then_2
      (for _array_element_3 (Variables|/Script/Engine.MaterialInstance|GetTextureParameterValues (LocalVariables|GetParent))
        (Utilities|FilterProperty (.name (.ParameterInfo (Utilities|Struct|BreakTextureParameterValue _array_element_3))) (LocalVariables|GetIgnoredProperties))
        (bind _returnvalue_3 (Rendering|Material|GetTextureParameterValue (LocalVariables|GetMaterial) (.name (.ParameterInfo (Utilities|Struct|BreakTextureParameterValue _array_element_3))) :!class /Script/Engine.MaterialInstanceDynamic))
        (bind _jsonobject_3 (CallFunction|MakeTextureParam (Utilities|String|ToString(Name) (.name (.ParameterInfo (Utilities|Struct|BreakTextureParameterValue _array_element_3)))) (Utilities|String|ToString(Name) (.name (.ParameterInfo (Utilities|Struct|BreakTextureParameterValue _array_element_3)))) "" _returnvalue_3 (.ParameterValue (Utilities|Struct|BreakTextureParameterValue _array_element_3)) (select (Utilities|Enum|Equal(Enum) (Variables|/Script/Engine.Texture|GetCompressionSettings (.ParameterValue (Utilities|Struct|BreakTextureParameterValue _array_element_3))) "TC_Normalmap") "/Game/QuietRuntimeEditor/Common/Textures/T_Dummy_N.T_Dummy_N" "/Game/QuietRuntimeEditor/Common/Textures/T_Dummy_BC.T_Dummy_BC")))
        (Utilities|Array|Add (LocalVariables|GetTextures) _jsonobject_3)))
    (:then_3
      ;[0 0 0] COLLECT
      (|SetJsonField TargetJson "GroupsState" (Utilities|Array|MakeArray "Scalar Parameters" "Vector Parameters" "Texture Parameters"))
      (Utilities|FlowControl|Sequence
        (:then_0
          (if (Utilities|Array|IsNotEmpty (LocalVariables|GetScalars))
            (|SetJsonField TargetJson "Scalar Parameters" (LocalVariables|GetScalars))))
        (:then_1
          (if (Utilities|Array|IsNotEmpty (LocalVariables|GetColors))
            (|SetJsonField TargetJson "Vector Parameters" (LocalVariables|GetColors))))
        (:then_2
          (if (Utilities|Array|IsNotEmpty (LocalVariables|GetTextures))
            (|SetJsonField TargetJson "Texture Parameters" (LocalVariables|GetTextures))))
        (:then_3
          (return))))))