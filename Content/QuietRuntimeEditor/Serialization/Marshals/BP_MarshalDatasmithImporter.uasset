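; Marshal for BP_DatasmithImporter in the runtime editor, handling its JSON serialization, property editing and actions.
; Property and action calls try the parent first, then handle importer fields, an Importer panel group, and Import and BrowseFile.
; Saving stores options, file and attached static mesh actors' components keyed by first tag.
; Restore replays each JSON field through SetPropertyValue, where File triggers an import and Content calls RestoreContent.
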(fn GetPropertyValue
  (params (Object :type Object%20Object%20Reference) (Property :type String))
  (bind (_success _value) (|CallParentFunction Object Property))
  (if (not _success)
    (bind _asbp_datasmith_importer (Utilities|Casting|CastToBP_DatasmithImporter Object))
    (bind _jsonobject (CallFunction|NewJson))
    (switch string Property
      (:File
        (|SetJsonField _jsonobject Property (Variables|/Game/QuietRuntimeEditor/Common/QuietActors/BP_DatasmithImporter.BP_DatasmithImporter_C|GetFile _asbp_datasmith_importer)))
      (:ExternalFile
        (|SetJsonField _jsonobject Property (Variables|/Script/DatasmithRuntime.DatasmithRuntimeActor|GetExternalFile _asbp_datasmith_importer)))
      (:ImportOptions
        (|SetJsonField _jsonobject Property (Variables|/Script/DatasmithRuntime.DatasmithRuntimeActor|GetImportOptions _asbp_datasmith_importer))))
    (return true _jsonobject)
    (else
      (return true _value))))

(fn SetPropertyValue
  (params (Object :type Object%20Object%20Reference) (Property :type String) (JsonValue :type Json%20Object%20Wrapper%20Structure%20%28by%20ref%29))
  (bind _success (|CallParentFunction Object Property JsonValue))
  (if (not _success)
    (bind _asbp_datasmith_importer (Utilities|Casting|CastToBP_DatasmithImporter Object))
    (switch string Property
      (:File
        (bind _outvalue (|GetJsonField JsonValue Property))
        (Variables|/Game/QuietRuntimeEditor/Common/QuietActors/BP_DatasmithImporter.BP_DatasmithImporter_C|SetFile _asbp_datasmith_importer _outvalue)
        (Default|Import _asbp_datasmith_importer))
      (:ImportOptions
        (bind _outvalue_2 (|GetJsonField JsonValue Property))
        (Variables|/Script/DatasmithRuntime.DatasmithRuntimeActor|SetImportOptions _asbp_datasmith_importer _outvalue_2))
      (:Content
        (bind _outvalue_3 (|GetJsonField JsonValue Property))
        (Default|RestoreContent _asbp_datasmith_importer _outvalue_3)))
    (return true)
    (else
      (return true))))

(fn SerializeObject
  (params (Object :type Object%20Object%20Reference) (TargetJson :type Json%20Object%20Wrapper%20Structure%20%28by%20ref%29))
  (|CallParentFunction Object TargetJson)
  (bind _asbp_datasmith_importer (Utilities|Casting|CastToBP_DatasmithImporter Object))
  (|SetJsonField TargetJson "ImportOptions" (Variables|/Script/DatasmithRuntime.DatasmithRuntimeActor|GetImportOptions _asbp_datasmith_importer))
  (|SetJsonField TargetJson "File" (Variables|/Game/QuietRuntimeEditor/Common/QuietActors/BP_DatasmithImporter.BP_DatasmithImporter_C|GetFile _asbp_datasmith_importer))
  (bind _jsonobject (CallFunction|SerializeContent _asbp_datasmith_importer))
  (|SetJsonField TargetJson "Content" _jsonobject)
  (return))

(fn RestoreObject
  (params (Object :type Object%20Object%20Reference) (JsonObject :type Json%20Object%20Wrapper%20Structure))
  (|CallParentFunction Object JsonObject)
  (bind _fieldnames (Class|JsonBlueprintFunctionLibrary|GetFieldNames JsonObject))
  (for _array_element _fieldnames
    (CallFunction|SetPropertyValue Object _array_element JsonObject)))

(fn CollectProperties
  (params (Object :type Object%20Object%20Reference) (TargetJson :type Json%20Object%20Wrapper%20Structure%20%28by%20ref%29))
  (Utilities|FlowControl|Sequence
    (:then_0
      (bind _asbp_datasmith_importer (Utilities|Casting|CastToBP_DatasmithImporter Object))
      (bind _jsonobject (CallFunction|MakeStringParam "File" "File" "" (Variables|/Game/QuietRuntimeEditor/Common/QuietActors/BP_DatasmithImporter.BP_DatasmithImporter_C|GetFile _asbp_datasmith_importer)))
      (Utilities|Array|Add (LocalVariables|GetImporter) _jsonobject)
      (bind _jsonobject_2 (CallFunction|NewJson))
      (|SetJsonField _jsonobject_2 "Type" (Utilities|String|MakeLiteralString "Actions"))
      (|SetJsonField _jsonobject_2 "Actions" (Utilities|Array|MakeArray "Import" "BrowseFile"))
      (Utilities|Array|Add (LocalVariables|GetImporter) _jsonobject_2))
    (:then_1
      (|SetJsonField TargetJson "GroupsState" (Utilities|Array|MakeArray "Importer"))
      (|SetJsonField TargetJson "Importer" (LocalVariables|GetImporter))
      (|CallParentFunction Object TargetJson)
      (return))))

(fn CallAction
  (params (Object :type Object%20Object%20Reference) (Action :type Json%20Object%20Wrapper%20Structure))
  (bind _success (|CallParentFunction Object Action))
  (if (not _success)
    (bind _asbp_datasmith_importer (Utilities|Casting|CastToBP_DatasmithImporter Object))
    (bind _outvalue (|GetJsonField Action "Action"))
    (switch string _outvalue
      (:Import
        (Default|Import _asbp_datasmith_importer))
      (:BrowseFile
        (Default|BrowseFile _asbp_datasmith_importer)))
    (else
      (return true))))

(fn SerializeContent
  (params (Actor :type Actor%20Object%20Reference))
  (bind _jsonobject (CallFunction|NewJson))
  (for _array_element (Actor|GetAttachedActors Actor true true)
    (bind _asstatic_mesh_actor (Utilities|Casting|CastToStaticMeshActor _array_element))
    (bind _json (Default|Serialize (CallFunction|GetSource) (Variables|/Script/Engine.StaticMeshActor|GetStaticMeshComponent _asstatic_mesh_actor)))
    (|SetJsonField _jsonobject (Utilities|String|ToString(Name) (Utilities|Array|Get(acopy) (Variables|/Script/Engine.Actor|GetTags _array_element))) _json))
  (return _jsonobject))