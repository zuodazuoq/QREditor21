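; Marshal for Audio Components in the Quiet Runtime Editor, exposing their properties for runtime editing and JSON serialization.
; It reads and writes sound, volume, pitch and attenuation, deferring to the parent marshal first for property access and actions.
; CollectProperties builds a Sound group with those parameters plus Play and Stop buttons, which CallAction runs on the component.
; RestoreObject replays each saved JSON field through SetPropertyValue.
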(fn SetPropertyValue
  (params (Object :type Object%20Object%20Reference) (Property :type String) (JsonValue :type Json%20Object%20Wrapper%20Structure%20%28by%20ref%29))
  (bind _success (|CallParentFunction Object Property JsonValue))
  (if (not _success)
    (bind _asaudio_component (Utilities|Casting|CastToAudioComponent Object))
    (switch string Property
      (:Sound
        (bind _outvalue (|GetJsonField JsonValue Property))
        (Audio|Components|Audio|SetSound _asaudio_component _outvalue))
      (:VolumeMultiplier
        (bind _newvalue (Utilities|ReadFloatwithCheck JsonValue Property (Variables|/Script/Engine.AudioComponent|GetVolumeMultiplier _asaudio_component))
          (:then
            (Audio|Components|Audio|SetVolumeMultiplier _asaudio_component _newvalue :!class /Script/Engine.AudioComponent))))
      (:PitchMultiplier
        (bind _newvalue_2 (Utilities|ReadFloatwithCheck JsonValue Property (Variables|/Script/Engine.AudioComponent|GetPitchMultiplier _asaudio_component))
          (:then
            (Audio|Components|Audio|SetPitchMultiplier _asaudio_component _newvalue_2))))
      (:AttenuationSettings
        (bind _outvalue_2 (|GetJsonField JsonValue Property))
        (Variables|/Script/Engine.AudioComponent|SetAttenuationSettings _asaudio_component _outvalue_2)))
    (return true)
    (else
      (return true))))

(fn GetPropertyValue
  (params (Object :type Object%20Object%20Reference) (Property :type String))
  (bind (_success _value) (|CallParentFunction Object Property))
  (if (not _success)
    (bind _outjsonobject (Class|JsonBlueprintFunctionLibrary|FromString "{ }"))
    (bind _asaudio_component (Utilities|Casting|CastToAudioComponent Object))
    (switch string Property
      (:Sound
        (|SetJsonField _outjsonobject Property (Variables|/Script/Engine.AudioComponent|GetSound _asaudio_component)))
      (:VolumeMultiplier
        (|SetJsonField _outjsonobject Property (Variables|/Script/Engine.AudioComponent|GetVolumeMultiplier _asaudio_component)))
      (:PitchMultiplier
        (|SetJsonField _outjsonobject Property (Variables|/Script/Engine.AudioComponent|GetPitchMultiplier _asaudio_component)))
      (:AttenuationSettings
        (|SetJsonField _outjsonobject Property (Variables|/Script/Engine.AudioComponent|GetAttenuationSettings _asaudio_component))))
    (return true _outjsonobject)
    (else
      (return true _value))))

(fn RestoreObject
  (params (Object :type Object%20Object%20Reference) (JsonObject :type Json%20Object%20Wrapper%20Structure))
  (|CallParentFunction Object JsonObject)
  (bind _fieldnames (Class|JsonBlueprintFunctionLibrary|GetFieldNames JsonObject))
  (for _array_element _fieldnames
    (CallFunction|SetPropertyValue Object _array_element JsonObject)))

(fn SerializeObject
  (params (Object :type Object%20Object%20Reference) (TargetJson :type Json%20Object%20Wrapper%20Structure%20%28by%20ref%29))
  (|CallParentFunction Object TargetJson)
  (bind _asaudio_component (Utilities|Casting|CastToAudioComponent Object))
  (|SetJsonField TargetJson "Sound" (Variables|/Script/Engine.AudioComponent|GetSound _asaudio_component))
  (|SetJsonField TargetJson "VolumeMultiplier" (Variables|/Script/Engine.AudioComponent|GetVolumeMultiplier _asaudio_component))
  (|SetJsonField TargetJson "PitchMultiplier" (Variables|/Script/Engine.AudioComponent|GetPitchMultiplier _asaudio_component))
  (|SetJsonField TargetJson "AttenuationSettings" (Variables|/Script/Engine.AudioComponent|GetAttenuationSettings _asaudio_component))
  (return))

(fn CollectProperties
  (params (Object :type Object%20Object%20Reference) (TargetJson :type Json%20Object%20Wrapper%20Structure%20%28by%20ref%29))
  (Utilities|FlowControl|Sequence
    (:then_0
      (bind _asaudio_component (Utilities|Casting|CastToAudioComponent Object))
      (bind _jsonobject (CallFunction|MakeObjectParam "Sound" "Sound" "" "/Script/Engine.SoundWave" (Variables|/Script/Engine.AudioComponent|GetSound _asaudio_component)))
      (Utilities|Array|Add (LocalVariables|GetSoundParams) _jsonobject)
      (bind _jsonobject_2 (CallFunction|MakeFloatParam "VolumeMultiplier" "Volume Multiplier" "" (Variables|/Script/Engine.AudioComponent|GetVolumeMultiplier _asaudio_component) 1.0 0.0 0.0 1e+02 1e+01 1 1))
      (Utilities|Array|Add (LocalVariables|GetSoundParams) _jsonobject_2)
      (bind _jsonobject_3 (CallFunction|MakeFloatParam "PitchMultiplier" "Pitch Multiplier" "" (Variables|/Script/Engine.AudioComponent|GetPitchMultiplier _asaudio_component) 1.0 0.0 0.0 1e+02 1e+01 1 1))
      (Utilities|Array|Add (LocalVariables|GetSoundParams) _jsonobject_3)
      (bind _jsonobject_4 (CallFunction|MakeObjectParam "AttenuationSettings" "Attenuation Settings" "" "/Script/Engine.SoundAttenuation" (Variables|/Script/Engine.AudioComponent|GetAttenuationSettings _asaudio_component)))
      (Utilities|Array|Add (LocalVariables|GetSoundParams) _jsonobject_4)
      (bind _jsonobject_5 (CallFunction|NewJson))
      (|SetJsonField _jsonobject_5 "Type" (Utilities|String|MakeLiteralString "Actions"))
      (|SetJsonField _jsonobject_5 "Actions" (Utilities|Array|MakeArray "Play" "Stop"))
      (Utilities|Array|Add (LocalVariables|GetSoundParams) _jsonobject_5))
    (:then_1
      (|SetJsonField TargetJson "GroupsState" (Utilities|Array|MakeArray "Sound"))
      (|SetJsonField TargetJson "Sound" (LocalVariables|GetSoundParams))
      (|CallParentFunction Object TargetJson)
      (return))))

(fn CallAction
  (params (Object :type Object%20Object%20Reference) (Action :type Json%20Object%20Wrapper%20Structure))
  (bind _success (|CallParentFunction Object Action))
  (if (not _success)
    (bind _asaudio_component (Utilities|Casting|CastToAudioComponent Object))
    (bind _outvalue (|GetJsonField Action "Action"))
    (switch string _outvalue
      (:Play
        (if (not (Audio|Components|Audio|IsPlaying _asaudio_component))
          (Audio|Components|Audio|Play _asaudio_component 0.0)
          (return true)))
      (:Stop
        (if (Audio|Components|Audio|IsPlaying _asaudio_component)
          (Audio|Components|Audio|Stop _asaudio_component)
          (return true))))
    (else
      (return true))))