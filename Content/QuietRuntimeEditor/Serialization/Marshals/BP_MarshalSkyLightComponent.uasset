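; Sky light component marshal for the Quiet Runtime Editor that shapes which properties are collected and how they are grouped.
; CollectProperties runs the parent collection into a scratch JSON, then copies only selected groups into the target.
; It nests the Advanced fields as a subgroup inside Light, copies Ray Tracing unchanged, and sets GroupsState to Light and Actor.
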(fn CollectProperties
  (params (Object :type Object%20Object%20Reference) (TargetJson :type Json%20Object%20Wrapper%20Structure%20%28by%20ref%29))
  (bind _jsonobject (CallFunction|NewJson))
  (|CallParentFunction Object _jsonobject)
  (|SetJsonField TargetJson "GroupsState" (Utilities|Array|MakeArray "Light" "Actor"))
  (bind _outvalue (|GetJsonField _jsonobject "Light"))
  (LocalVariables|SetLightParams _outvalue)
  (bind _outvalue_2 (|GetJsonField _jsonobject "Advanced"))
  (bind _jsonobject_2 (CallFunction|MakeParamSubgroup "Advanced" _outvalue_2))
  (Utilities|Array|Add (LocalVariables|GetLightParams) _jsonobject_2)
  (|SetJsonField TargetJson "Light" (LocalVariables|GetLightParams))
  (bind _outvalue_3 (|GetJsonField _jsonobject "Ray Tracing"))
  (|SetJsonField TargetJson "Ray Tracing" _outvalue_3)
  (return))