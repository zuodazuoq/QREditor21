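; Marshal for RectLightComponent in the Quiet runtime editor, handling JSON serialization, restore and property editing of rect lights.
; It extends a parent marshal with source size, barn door and attenuation fields, and caches the light profile on serialize.
; Property collection adds slider parameters to the parent's Light group and nests Advanced as a subgroup.
; Restore feeds each JSON field through SetPropertyValue, which tries the parent before its own setters.
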(fn SerializeObject
  (params (Object :type Object%20Object%20Reference) (TargetJson :type Json%20Object%20Wrapper%20Structure%20%28by%20ref%29))
  (|CallParentFunction Object TargetJson)
  (bind _asrect_light_component (Utilities|Casting|CastToRectLightComponent Object))
  (|SetJsonField TargetJson "SourceWidth" (Variables|/Script/Engine.RectLightComponent|GetSourceWidth _asrect_light_component))
  (|SetJsonField TargetJson "SourceHeight" (Variables|/Script/Engine.RectLightComponent|GetSourceHeight _asrect_light_component))
  (|SetJsonField TargetJson "BarnDoorAngle" (Variables|/Script/Engine.RectLightComponent|GetBarnDoorAngle _asrect_light_component))
  (|SetJsonField TargetJson "BarnDoorLength" (Variables|/Script/Engine.RectLightComponent|GetBarnDoorLength _asrect_light_component))
  (|SetJsonField TargetJson "AttenuationRadius" (Variables|/Script/Engine.LocalLightComponent|GetAttenuationRadius _asrect_light_component))
  (CallFunction|CacheLightProfile _asrect_light_component TargetJson)
  (return))

(fn GetPropertyValue
  (params (Object :type Object%20Object%20Reference) (Property :type String))
  (bind _asrect_light_component (Utilities|Casting|CastToRectLightComponent Object))
  (bind _outjsonobject (Class|JsonBlueprintFunctionLibrary|FromString "{ }"))
  (switch string Property
    (:Default
      (bind (_success _value) (|CallParentFunction Object Property))
      (return _success _value))
    (:SourceWidth
      (|SetJsonField _outjsonobject Property (Variables|/Script/Engine.RectLightComponent|GetSourceWidth _asrect_light_component)))
    (:SourceHeight
      (|SetJsonField _outjsonobject Property (Variables|/Script/Engine.RectLightComponent|GetSourceHeight _asrect_light_component)))
    (:BarnDoorAngle
      (|SetJsonField _outjsonobject Property (Variables|/Script/Engine.RectLightComponent|GetBarnDoorAngle _asrect_light_component)))
    (:BarnDoorLength
      (|SetJsonField _outjsonobject Property (Variables|/Script/Engine.RectLightComponent|GetBarnDoorLength _asrect_light_component)))
    (:AttenuationRadius
      (|SetJsonField _outjsonobject Property (Variables|/Script/Engine.LocalLightComponent|GetAttenuationRadius _asrect_light_component))))
  (return true _outjsonobject))

(fn SetPropertyValue
  (params (Object :type Object%20Object%20Reference) (Property :type String) (JsonValue :type Json%20Object%20Wrapper%20Structure%20%28by%20ref%29))
  (bind _success (|CallParentFunction Object Property JsonValue))
  (if (not _success)
    (bind _asrect_light_component (Utilities|Casting|CastToRectLightComponent Object))
    (switch string Property
      (:Default
        (return false))
      (:SourceWidth
        (bind _newvalue (Utilities|ReadFloatwithCheck JsonValue Property (Variables|/Script/Engine.RectLightComponent|GetSourceWidth _asrect_light_component))
          (:then
            (Class|RectLightComponent|SetSourceWidth _asrect_light_component _newvalue))))
      (:SourceHeight
        (bind _newvalue_2 (Utilities|ReadFloatwithCheck JsonValue Property (Variables|/Script/Engine.RectLightComponent|GetSourceHeight _asrect_light_component))
          (:then
            (Class|RectLightComponent|SetSourceHeight _asrect_light_component _newvalue_2))))
      (:BarnDoorAngle
        (bind _newvalue_3 (Utilities|ReadFloatwithCheck JsonValue Property (Variables|/Script/Engine.RectLightComponent|GetBarnDoorAngle _asrect_light_component))
          (:then
            (Class|RectLightComponent|SetBarnDoorAngle _asrect_light_component _newvalue_3))))
      (:BarnDoorLength
        (bind _newvalue_4 (Utilities|ReadFloatwithCheck JsonValue Property (Variables|/Script/Engine.RectLightComponent|GetBarnDoorLength _asrect_light_component))
          (:then
            (Class|RectLightComponent|SetBarnDoorLength _asrect_light_component _newvalue_4))))
      (:AttenuationRadius
        (bind _newvalue_5 (Utilities|ReadFloatwithCheck JsonValue Property (Variables|/Script/Engine.LocalLightComponent|GetAttenuationRadius _asrect_light_component))
          (:then
            (Rendering|Lighting|SetAttenuationRadius _asrect_light_component _newvalue_5)))))
    (return true)))

(fn CollectProperties
  (params (Object :type Object%20Object%20Reference) (TargetJson :type Json%20Object%20Wrapper%20Structure%20%28by%20ref%29))
  (bind _asrect_light_component (Utilities|Casting|CastToRectLightComponent Object))
  (Utilities|FlowControl|Sequence
    (:then_0
      (bind _jsonobject (CallFunction|NewJson))
      (|CallParentFunction _asrect_light_component _jsonobject)
      (bind _outvalue (|GetJsonField _jsonobject "Light"))
      (LocalVariables|SetLightParams _outvalue)
      (bind _outvalue_2 (|GetJsonField _jsonobject "Advanced"))
      (LocalVariables|SetAdvancedParams _outvalue_2)
      (bind _outvalue_3 (|GetJsonField _jsonobject "Ray Tracing"))
      (LocalVariables|SetRayTracing _outvalue_3)
      (bind _jsonobject_2 (CallFunction|MakeFloatParam "SourceWidth" "Source Width" "" (Variables|/Script/Engine.RectLightComponent|GetSourceWidth _asrect_light_component) 64.0 1.0 1.0 1e+04 1e+03 1 3))
      (Utilities|Array|Add (LocalVariables|GetLightParams) _jsonobject_2)
      (bind _jsonobject_3 (CallFunction|MakeFloatParam "SourceHeight" "Source Height" "" (Variables|/Script/Engine.RectLightComponent|GetSourceHeight _asrect_light_component) 64.0 1.0 1.0 1e+04 1e+03 1 3))
      (Utilities|Array|Add (LocalVariables|GetLightParams) _jsonobject_3)
      (bind _jsonobject_4 (CallFunction|MakeFloatParam "BarnDoorAngle" "Barn Door Angle" "" (Variables|/Script/Engine.RectLightComponent|GetBarnDoorAngle _asrect_light_component) 88.0 0.0 0.0 9e+01 9e+01 1 3))
      (Utilities|Array|Add (LocalVariables|GetLightParams) _jsonobject_4)
      (bind _jsonobject_5 (CallFunction|MakeFloatParam "BarnDoorLength" "Barn Door Length" "" (Variables|/Script/Engine.RectLightComponent|GetBarnDoorLength _asrect_light_component) 2e+01 0.0 0.0 1e+04 1e+03 1 3))
      (Utilities|Array|Add (LocalVariables|GetLightParams) _jsonobject_5)
      (bind _jsonobject_6 (CallFunction|MakeFloatParam "AttenuationRadius" "Attenuation Radius" "" (Variables|/Script/Engine.LocalLightComponent|GetAttenuationRadius _asrect_light_component) 1e+03 0.0 8.0 1e+05 16384.0 1 4))
      (Utilities|Array|Add (LocalVariables|GetLightParams) _jsonobject_6))
    (:then_1
      (|SetJsonField TargetJson "GroupsState" (Utilities|Array|MakeArray "Light" "Actor"))
      (bind _jsonobject_7 (CallFunction|MakeParamSubgroup "Advanced" (LocalVariables|GetAdvancedParams)))
      (Utilities|Array|Add (LocalVariables|GetLightParams) _jsonobject_7)
      (|SetJsonField TargetJson "Light" (LocalVariables|GetLightParams))
      (|SetJsonField TargetJson "Ray Tracing" (LocalVariables|GetRayTracing))
      (return))))

(fn RestoreObject
  (params (Object :type Object%20Object%20Reference) (JsonObject :type Json%20Object%20Wrapper%20Structure))
  (|CallParentFunction Object JsonObject)
  (bind _fieldnames (Class|JsonBlueprintFunctionLibrary|GetFieldNames JsonObject))
  (for _array_element _fieldnames
    (CallFunction|SetPropertyValue Object _array_element JsonObject)))