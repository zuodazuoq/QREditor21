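; Runtime editor marshal that saves, restores and exposes DirectionalLightComponent settings as JSON: source angles, shadows, light shafts and cascades.
; Serialize, get and set handle directional-specific fields by name and defer the rest to the parent marshal.
; RestoreObject calls the parent, then replays each JSON field through SetPropertyValue.
; CollectProperties extends the parent's parameter groups with Light Shafts and Cascaded Shadow Maps, nesting Advanced under Light.
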(fn SerializeObject
  (params (Object :type Object%20Object%20Reference) (TargetJson :type Json%20Object%20Wrapper%20Structure%20%28by%20ref%29))
  (bind _asdirectional_light_component (Utilities|Casting|CastToDirectionalLightComponent Object))
  (Utilities|FlowControl|Sequence
    (:then_0
      (Utilities|FlowControl|Sequence
        (:then_0
          (|SetJsonField TargetJson "SourceAngle" (Variables|/Script/Engine.DirectionalLightComponent|GetLightSourceAngle _asdirectional_light_component)))
        (:then_1
          (|SetJsonField TargetJson "SourceSoftAngle" (Variables|/Script/Engine.DirectionalLightComponent|GetLightSourceSoftAngle _asdirectional_light_component)))
        (:then_2
          (|SetJsonField TargetJson "ShadowCascadeBiasDistribution" (Variables|/Script/Engine.DirectionalLightComponent|GetShadowCascadeBiasDistribution _asdirectional_light_component)))
        (:then_3
          (|SetJsonField TargetJson "ShadowAmount" (Variables|/Script/Engine.DirectionalLightComponent|GetShadowAmount _asdirectional_light_component)))))
    (:then_1
      (Utilities|FlowControl|Sequence
        (:then_0
          (|SetJsonField TargetJson "LightShaftOcclusion" (Variables|/Script/Engine.DirectionalLightComponent|GetbEnableLightShaftOcclusion _asdirectional_light_component)))
        (:then_1
          (|SetJsonField TargetJson "OcclusionMaskDarkness" (Variables|/Script/Engine.DirectionalLightComponent|GetOcclusionMaskDarkness _asdirectional_light_component)))
        (:then_2
          (|SetJsonField TargetJson "OcclusionDepthRange" (Variables|/Script/Engine.DirectionalLightComponent|GetOcclusionDepthRange _asdirectional_light_component)))
        (:then_3
          (|SetJsonField TargetJson "LightShaftBloom" (Variables|/Script/Engine.LightComponent|GetbEnableLightShaftBloom _asdirectional_light_component)))
        (:then_4
          (|SetJsonField TargetJson "BloomScale" (Variables|/Script/Engine.LightComponent|GetBloomScale _asdirectional_light_component)))
        (:then_5
          (|SetJsonField TargetJson "BloomMaxDarkness" (Variables|/Script/Engine.LightComponent|GetBloomMaxBrightness _asdirectional_light_component)))
        (:then_6
          (|SetJsonField TargetJson "BloomTint" (Variables|/Script/Engine.LightComponent|GetBloomTint _asdirectional_light_component)))
        (:then_7
          (|SetJsonField TargetJson "LightShaftOverrideDirection" (Variables|/Script/Engine.DirectionalLightComponent|GetLightShaftOverrideDirection _asdirectional_light_component)))))
    (:then_2
      (Utilities|FlowControl|Sequence
        (:then_0
          (|SetJsonField TargetJson "DynamicShadowCascades" (Variables|/Script/Engine.DirectionalLightComponent|GetDynamicShadowCascades _asdirectional_light_component)))
        (:then_1
          (|SetJsonField TargetJson "DistributionExponent" (Variables|/Script/Engine.DirectionalLightComponent|GetCascadeDistributionExponent _asdirectional_light_component)))
        (:then_2
          (|SetJsonField TargetJson "TransitionFraction" (Variables|/Script/Engine.DirectionalLightComponent|GetCascadeTransitionFraction _asdirectional_light_component)))
        (:then_3
          (|SetJsonField TargetJson "DistanceFadeoutFraction" (Variables|/Script/Engine.DirectionalLightComponent|GetShadowDistanceFadeoutFraction _asdirectional_light_component)))
        (:then_4
          (|SetJsonField TargetJson "DynamicShadowDistanceMovableLight" (Variables|/Script/Engine.DirectionalLightComponent|GetDynamicShadowDistanceMovableLight _asdirectional_light_component)))))
    (:then_3
      (|CallParentFunction _asdirectional_light_component TargetJson)
      (return))))

(fn GetPropertyValue
  (params (Object :type Object%20Object%20Reference) (Property :type String))
  (bind _asdirectional_light_component (Utilities|Casting|CastToDirectionalLightComponent Object))
  (bind _outjsonobject (Class|JsonBlueprintFunctionLibrary|FromString "{ }"))
  (switch string Property
    (:Default
      (bind (_success _value) (|CallParentFunction _asdirectional_light_component Property))
      (return _success _value))
    (:SourceAngle
      (|SetJsonField _outjsonobject Property (Variables|/Script/Engine.DirectionalLightComponent|GetLightSourceAngle _asdirectional_light_component)))
    (:SourceSoftAngle
      (|SetJsonField _outjsonobject Property (Variables|/Script/Engine.DirectionalLightComponent|GetLightSourceSoftAngle _asdirectional_light_component)))
    (:ShadowCascadeBiasDistribution
      (|SetJsonField _outjsonobject Property (Variables|/Script/Engine.DirectionalLightComponent|GetShadowCascadeBiasDistribution _asdirectional_light_component)))
    (:ShadowAmount
      (|SetJsonField _outjsonobject Property (Variables|/Script/Engine.DirectionalLightComponent|GetShadowAmount _asdirectional_light_component)))
    (:LightShaftOcclusion
      (|SetJsonField _outjsonobject Property (Variables|/Script/Engine.DirectionalLightComponent|GetbEnableLightShaftOcclusion _asdirectional_light_component)))
    (:OcclusionMaskDarkness
      (|SetJsonField _outjsonobject Property (Variables|/Script/Engine.DirectionalLightComponent|GetOcclusionMaskDarkness _asdirectional_light_component)))
    (:OcclusionDepthRange
      (|SetJsonField _outjsonobject Property (Variables|/Script/Engine.DirectionalLightComponent|GetOcclusionDepthRange _asdirectional_light_component)))
    (:LightShaftBloom
      (|SetJsonField _outjsonobject Property (Variables|/Script/Engine.LightComponent|GetbEnableLightShaftBloom _asdirectional_light_component)))
    (:BloomScale
      (|SetJsonField _outjsonobject Property (Variables|/Script/Engine.LightComponent|GetBloomScale _asdirectional_light_component)))
    (:BloomMaxDarkness
      (|SetJsonField _outjsonobject Property (Variables|/Script/Engine.LightComponent|GetBloomMaxBrightness _asdirectional_light_component)))
    (:BloomTint
      (|SetJsonField _outjsonobject Property (Variables|/Script/Engine.LightComponent|GetBloomTint _asdirectional_light_component)))
    (:LightShaftOverrideDirection
      (|SetJsonField _outjsonobject Property (Variables|/Script/Engine.DirectionalLightComponent|GetLightShaftOverrideDirection _asdirectional_light_component)))
    (:DynamicShadowCascades
      (|SetJsonField _outjsonobject Property (Variables|/Script/Engine.DirectionalLightComponent|GetDynamicShadowCascades _asdirectional_light_component)))
    (:DistributionExponent
      (|SetJsonField _outjsonobject Property (Variables|/Script/Engine.DirectionalLightComponent|GetCascadeDistributionExponent _asdirectional_light_component)))
    (:TransitionFraction
      (|SetJsonField _outjsonobject Property (Variables|/Script/Engine.DirectionalLightComponent|GetCascadeTransitionFraction _asdirectional_light_component)))
    (:DistanceFadeoutFraction
      (|SetJsonField _outjsonobject Property (Variables|/Script/Engine.DirectionalLightComponent|GetShadowDistanceFadeoutFraction _asdirectional_light_component)))
    (:DynamicShadowDistanceMovableLight
      (|SetJsonField _outjsonobject Property (Variables|/Script/Engine.DirectionalLightComponent|GetDynamicShadowDistanceMovableLight _asdirectional_light_component))))
  (return true _outjsonobject))

(fn SetPropertyValue
  (params (Object :type Object%20Object%20Reference) (Property :type String) (JsonValue :type Json%20Object%20Wrapper%20Structure%20%28by%20ref%29))
  (bind _asdirectional_light_component (Utilities|Casting|CastToDirectionalLightComponent Object))
  (switch string Property
    (:Default
      (bind _success (|CallParentFunction Object Property JsonValue))
      (return _success))
    (:SourceAngle
      (bind _newvalue (Utilities|ReadFloatwithCheck JsonValue Property (Variables|/Script/Engine.DirectionalLightComponent|GetLightSourceAngle _asdirectional_light_component))
        (:then
          (Class|DirectionalLightComponent|SetLightSourceAngle _asdirectional_light_component _newvalue)
          (return true))))
    (:SourceSoftAngle
      (bind _newvalue_2 (Utilities|ReadFloatwithCheck JsonValue Property (Variables|/Script/Engine.DirectionalLightComponent|GetLightSourceSoftAngle _asdirectional_light_component))
        (:then
          (Class|DirectionalLightComponent|SetLightSourceSoftAngle _asdirectional_light_component _newvalue_2)
          (return true))))
    (:ShadowCascadeBiasDistribution
      (bind _newvalue_3 (Utilities|ReadFloatwithCheck JsonValue Property (Variables|/Script/Engine.DirectionalLightComponent|GetShadowCascadeBiasDistribution _asdirectional_light_component))
        (:then
          (Class|DirectionalLightComponent|SetShadowCascadeBiasDistribution _asdirectional_light_component _newvalue_3)
          (return true))))
    (:ShadowAmount
      (bind _newvalue_4 (Utilities|ReadFloatwithCheck JsonValue Property (Variables|/Script/Engine.DirectionalLightComponent|GetShadowAmount _asdirectional_light_component))
        (:then
          (Class|DirectionalLightComponent|SetShadowAmount _asdirectional_light_component _newvalue_4)
          (return true))))
    (:LightShaftOcclusion
      (bind _newvalue_5 (Utilities|ReadBoolwithCheck JsonValue Property (Variables|/Script/Engine.DirectionalLightComponent|GetbEnableLightShaftOcclusion _asdirectional_light_component))
        (:then
          (Class|DirectionalLightComponent|SetEnableLightShaftOcclusion _asdirectional_light_component _newvalue_5)
          (return true))))
    (:OcclusionMaskDarkness
      (bind _newvalue_6 (Utilities|ReadFloatwithCheck JsonValue Property (Variables|/Script/Engine.DirectionalLightComponent|GetOcclusionMaskDarkness _asdirectional_light_component))
        (:then
          (Class|DirectionalLightComponent|SetOcclusionMaskDarkness _asdirectional_light_component _newvalue_6)
          (return true))))
    (:OcclusionDepthRange
      (bind _newvalue_7 (Utilities|ReadFloatwithCheck JsonValue Property (Variables|/Script/Engine.DirectionalLightComponent|GetOcclusionDepthRange _asdirectional_light_component))
        (:then
          (Class|DirectionalLightComponent|SetOcclusionDepthRange _asdirectional_light_component _newvalue_7)
          (return true))))
    (:LightShaftBloom
      (bind _newvalue_8 (Utilities|ReadBoolwithCheck JsonValue Property (Variables|/Script/Engine.LightComponent|GetbEnableLightShaftBloom _asdirectional_light_component))
        (:then
          (Class|LightComponent|SetEnableLightShaftBloom _asdirectional_light_component _newvalue_8)
          (return true))))
    (:BloomScale
      (bind _newvalue_9 (Utilities|ReadFloatwithCheck JsonValue Property (Variables|/Script/Engine.LightComponent|GetBloomScale _asdirectional_light_component))
        (:then
          (Class|LightComponent|SetBloomScale _asdirectional_light_component _newvalue_9)
          (return true))))
    (:BloomMaxDarkness
      (bind _newvalue_10 (Utilities|ReadFloatwithCheck JsonValue Property (Variables|/Script/Engine.LightComponent|GetBloomMaxBrightness _asdirectional_light_component))
        (:then
          (Class|LightComponent|SetBloomMaxBrightness _asdirectional_light_component _newvalue_10)
          (return true))))
    (:BloomTint
      (bind (_outvalue _returnvalue) (|GetJsonField JsonValue Property))
      (if _returnvalue
        (Class|LightComponent|SetBloomTint _asdirectional_light_component _outvalue)
        (return true)))
    (:LightShaftOverrideDirection
      (bind _newvalue_11 (Utilities|ReadVectorwithCheck JsonValue Property (Variables|/Script/Engine.DirectionalLightComponent|GetLightShaftOverrideDirection _asdirectional_light_component))
        (:then
          (Class|DirectionalLightComponent|SetLightShaftOverrideDirection _asdirectional_light_component _newvalue_11)
          (return true))))
    (:DynamicShadowCascades
      (bind _newvalue_12 (Utilities|ReadIntegerwithCheck JsonValue Property (Variables|/Script/Engine.DirectionalLightComponent|GetDynamicShadowCascades _asdirectional_light_component))
        (:then
          (Class|DirectionalLightComponent|SetDynamicShadowCascades _asdirectional_light_component _newvalue_12)
          (return true))))
    (:DistributionExponent
      (bind _newvalue_13 (Utilities|ReadFloatwithCheck JsonValue Property (Variables|/Script/Engine.DirectionalLightComponent|GetCascadeDistributionExponent _asdirectional_light_component))
        (:then
          (Class|DirectionalLightComponent|SetCascadeDistributionExponent _asdirectional_light_component _newvalue_13)
          (return true))))
    (:TransitionFraction
      (bind _newvalue_14 (Utilities|ReadFloatwithCheck JsonValue Property (Variables|/Script/Engine.DirectionalLightComponent|GetCascadeTransitionFraction _asdirectional_light_component))
        (:then
          (Class|DirectionalLightComponent|SetCascadeTransitionFraction _asdirectional_light_component _newvalue_14)
          (return true))))
    (:DistanceFadeoutFraction
      (bind _newvalue_15 (Utilities|ReadFloatwithCheck JsonValue Property (Variables|/Script/Engine.DirectionalLightComponent|GetShadowDistanceFadeoutFraction _asdirectional_light_component))
        (:then
          (Class|DirectionalLightComponent|SetShadowDistanceFadeoutFraction _asdirectional_light_component _newvalue_15)
          (return true))))
    (:DynamicShadowDistanceMovableLight
      (bind _newvalue_16 (Utilities|ReadFloatwithCheck JsonValue Property (Variables|/Script/Engine.DirectionalLightComponent|GetDynamicShadowDistanceMovableLight _asdirectional_light_component))
        (:then
          (Class|DirectionalLightComponent|SetDynamicShadowDistanceMovableLight _asdirectional_light_component _newvalue_16)
          (return true))))))

(fn CollectProperties
  (params (Object :type Object%20Object%20Reference) (TargetJson :type Json%20Object%20Wrapper%20Structure%20%28by%20ref%29))
  (bind _asdirectional_light_component (Utilities|Casting|CastToDirectionalLightComponent Object))
  (Utilities|FlowControl|Sequence
    (:then_0
      (bind _jsonobject (CallFunction|NewJson))
      (|CallParentFunction _asdirectional_light_component _jsonobject)
      (bind _outvalue (|GetJsonField _jsonobject "Light"))
      (LocalVariables|SetLightParams _outvalue)
      (bind _outvalue_2 (|GetJsonField _jsonobject "Advanced"))
      (LocalVariables|SetAdvancedParams _outvalue_2)
      (bind _outvalue_3 (|GetJsonField _jsonobject "Ray Tracing"))
      (LocalVariables|SetRayTracing _outvalue_3)
      (Utilities|FlowControl|Sequence
        (:then_0
          (bind _jsonobject_2 (CallFunction|MakeBoolParam "LightShaftOcclusion" "Light Shaft Occlusion" "" (Variables|/Script/Engine.DirectionalLightComponent|GetbEnableLightShaftOcclusion _asdirectional_light_component) false))
          (Utilities|Array|Add (LocalVariables|GetLightShafts) _jsonobject_2)
          (bind _jsonobject_3 (CallFunction|MakeFloatParam "OcclusionMaskDarkness" "Occlusion Mask Darkness" "" (Variables|/Script/Engine.DirectionalLightComponent|GetOcclusionMaskDarkness _asdirectional_light_component) 0.05 0.0 0.0 1e+02 1.0 1 3))
          (Utilities|Array|Add (LocalVariables|GetLightShafts) _jsonobject_3)
          (bind _jsonobject_4 (CallFunction|MakeFloatParam "OcclusionDepthRange" "Occlusion Depth Range" "" (Variables|/Script/Engine.DirectionalLightComponent|GetOcclusionDepthRange _asdirectional_light_component) 1e+05 0.0 0.0 5e+05 5e+05 1 1))
          (Utilities|Array|Add (LocalVariables|GetLightShafts) _jsonobject_4)
          (bind _jsonobject_5 (CallFunction|MakeBoolParam "LightShaftBloom" "Light Shaft Bloom" "" (Variables|/Script/Engine.LightComponent|GetbEnableLightShaftBloom _asdirectional_light_component) false))
          (Utilities|Array|Add (LocalVariables|GetLightShafts) _jsonobject_5)
          (bind _jsonobject_6 (CallFunction|MakeFloatParam "BloomScale" "Bloom Scale" "" (Variables|/Script/Engine.LightComponent|GetBloomScale _asdirectional_light_component) 0.2 0.0 0.0 1e+02 1e+01 1 2))
          (Utilities|Array|Add (LocalVariables|GetLightShafts) _jsonobject_6)
          (bind _jsonobject_7 (CallFunction|MakeFloatParam "BloomMaxBrightness" "Bloom Max Brightness" "" (Variables|/Script/Engine.LightComponent|GetBloomMaxBrightness _asdirectional_light_component) 1e+02 0.0 0.0 1e+03 1e+02 1 2))
          (Utilities|Array|Add (LocalVariables|GetLightShafts) _jsonobject_7)
          (bind _jsonobject_8 (CallFunction|MakeLinearColorParam "BloomTint" "Bloom Tint" "" (Math|Conversions|ToLinearColor(Color) (Variables|/Script/Engine.LightComponent|GetBloomTint _asdirectional_light_component)) "(R=1.000000,G=1.000000,B=1.000000,A=1.000000)"))
          (Utilities|Array|Add (LocalVariables|GetLightShafts) _jsonobject_8)
          (bind _jsonobject_9 (CallFunction|MakeVectorParam "LightShaftOverrideDirection" "Override Direction" "" (Variables|/Script/Engine.DirectionalLightComponent|GetLightShaftOverrideDirection _asdirectional_light_component) "0, 0, 0"))
          (Utilities|Array|Add (LocalVariables|GetLightShafts) _jsonobject_9))
        (:then_1
          (bind _jsonobject_10 (CallFunction|MakeIntParam "NumDynamicCascadedShadows" "Num Dynamic Cascaded Shadows" "" (Variables|/Script/Engine.DirectionalLightComponent|GetDynamicShadowCascades _asdirectional_light_component) 4 0 0 10 4))
          (Utilities|Array|Add (LocalVariables|GetCascadedShadows) _jsonobject_10)
          (bind _jsonobject_11 (CallFunction|MakeFloatParam "DistributionExponent" "Distribution Exponent" "" (Variables|/Script/Engine.DirectionalLightComponent|GetCascadeDistributionExponent _asdirectional_light_component) 3.0 0.1 1.0 1e+01 4.0 1 3))
          (Utilities|Array|Add (LocalVariables|GetCascadedShadows) _jsonobject_11)
          (bind _jsonobject_12 (CallFunction|MakeFloatParam "TransitionFraction" "Transition Fraction" "" (Variables|/Script/Engine.DirectionalLightComponent|GetCascadeTransitionFraction _asdirectional_light_component) 0.0 0.0 0.0 0.0 0.0 1 6))
          (Utilities|Array|Add (LocalVariables|GetCascadedShadows) _jsonobject_12)
          (bind _jsonobject_13 (CallFunction|MakeFloatParam "DistanceFadeoutFraction" "Distance Fadeout Fraction" "" (Variables|/Script/Engine.DirectionalLightComponent|GetShadowDistanceFadeoutFraction _asdirectional_light_component) 0.0 0.0 0.0 0.0 0.0 1 6))
          (Utilities|Array|Add (LocalVariables|GetCascadedShadows) _jsonobject_13)
          (bind _jsonobject_14 (CallFunction|MakeFloatParam "DynamicShadowDistanceMovableLight" "Dynamic Shadow Distance" "" (Variables|/Script/Engine.DirectionalLightComponent|GetDynamicShadowDistanceMovableLight _asdirectional_light_component) 0.0 0.0 0.0 0.0 0.0 1 6))
          (Utilities|Array|Add (LocalVariables|GetCascadedShadows) _jsonobject_14)
          (bind _jsonobject_15 (CallFunction|MakeFloatParam "SourceAngle" "Source Angle" "" (Variables|/Script/Engine.DirectionalLightComponent|GetLightSourceAngle _asdirectional_light_component) 0.5357 0.0 0.0 1e+02 5.0 1 4))
          (Utilities|Array|Add (LocalVariables|GetLightParams) _jsonobject_15)
          (bind _jsonobject_16 (CallFunction|MakeFloatParam "SourceSoftAngle" "Source Soft Angle" "" (Variables|/Script/Engine.DirectionalLightComponent|GetLightSourceSoftAngle _asdirectional_light_component) 0.0 0.0 0.0 1e+02 5.0 1 4))
          (Utilities|Array|Add (LocalVariables|GetLightParams) _jsonobject_16)
          (bind _jsonobject_17 (CallFunction|MakeFloatParam "ShadowAmount" "Shadow Amount" "" (Variables|/Script/Engine.DirectionalLightComponent|GetShadowAmount _asdirectional_light_component) 1.0 0.0 0.0 1.0 1.0 1 4))
          (Utilities|Array|Insert (LocalVariables|GetAdvancedParams) _jsonobject_17)
          (bind _jsonobject_18 (CallFunction|MakeFloatParam "ShadowCascadeBiasDistribution" "Shadow Cascade Bias Distribution" "" (Variables|/Script/Engine.DirectionalLightComponent|GetShadowCascadeBiasDistribution _asdirectional_light_component) 1.0 0.0 0.0 1.0 1.0 1 4))
          (Utilities|Array|Insert (LocalVariables|GetAdvancedParams) _jsonobject_18))))
    (:then_1
      (|SetJsonField TargetJson "GroupsState" (Utilities|Array|MakeArray "Light" "Actor"))
      (bind _jsonobject_19 (CallFunction|MakeParamSubgroup "Advanced" (LocalVariables|GetAdvancedParams)))
      (Utilities|Array|Add (LocalVariables|GetLightParams) _jsonobject_19)
      (|SetJsonField TargetJson "Light" (LocalVariables|GetLightParams))
      (|SetJsonField TargetJson "Ray Tracing" (LocalVariables|GetRayTracing))
      (|SetJsonField TargetJson "Light Shafts" (LocalVariables|GetLightShafts))
      (|SetJsonField TargetJson "Cascaded Shadow Maps" (LocalVariables|GetCascadedShadows))
      (return))))

(fn RestoreObject
  (params (Object :type Object%20Object%20Reference) (JsonObject :type Json%20Object%20Wrapper%20Structure))
  (|CallParentFunction Object JsonObject)
  (bind _fieldnames (Class|JsonBlueprintFunctionLibrary|GetFieldNames JsonObject))
  (for _array_element _fieldnames
    (CallFunction|SetPropertyValue Object _array_element JsonObject)))