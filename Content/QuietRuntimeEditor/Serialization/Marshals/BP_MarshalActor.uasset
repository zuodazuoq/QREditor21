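; Actor marshal for the Quiet Runtime Editor that converts actors to and from JSON and exposes their editable properties.
; Serializes class, transform, tags, hidden state and attach socket, but restores only Tags and Hidden, through SetPropertyValue.
; CollectProperties publishes Tags as an array parameter with a default item template.
; Other property names shaped "Component.Slot" set a material on the named primitive component, with "Root" meaning the root component.
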(fn SerializeObject
  (params (Object :type Object%20Object%20Reference) (TargetJson :type Json%20Object%20Wrapper%20Structure%20%28by%20ref%29))
  (bind _asactor (Utilities|Casting|CastToActor Object))
  (Utilities|FlowControl|Sequence
    (:then_0
      (|SetJsonField TargetJson "Class" (Utilities|GetClass _asactor)))
    (:then_1
      (|SetJsonField TargetJson "Transform" (Transformation|GetActorTransform _asactor)))
    (:then_2
      (|SetJsonField TargetJson "Tags" (Variables|/Script/Engine.Actor|GetTags _asactor)))
    (:then_3
      (|SetJsonField TargetJson "Hidden" (Variables|/Script/Engine.Actor|GetbHidden _asactor)))
    (:then_4
      (|SetJsonField TargetJson "Socket" (Class|Actor|GetAttachParentSocketName _asactor))
      (return))))

(fn GetPropertyValue
  (params (Object :type Object%20Object%20Reference) (Property :type String))
  (bind _asactor (Utilities|Casting|CastToActor Object))
  (bind _outjsonobject (Class|JsonBlueprintFunctionLibrary|FromString "{ }"))
  (switch string Property
    (:Tags
      (|SetJsonField _outjsonobject Property (Variables|/Script/Engine.Actor|GetTags _asactor)))
    (:Hidden
      (|SetJsonField _outjsonobject Property (Variables|/Script/Engine.Actor|GetbHidden _asactor)))
    (:Socket
      (|SetJsonField _outjsonobject Property (Class|Actor|GetAttachParentSocketName _asactor))))
  (return true _outjsonobject))

(fn SetPropertyValue
  (params (Object :type Object%20Object%20Reference) (Property :type String) (JsonValue :type Json%20Object%20Wrapper%20Structure%20%28by%20ref%29))
  (bind _asactor (Utilities|Casting|CastToActor Object))
  (switch string Property
    (:Default
      (bind _success (CallFunction|SetMaterial _asactor Property JsonValue))
      (return _success))
    (:Tags
      (bind _outvalue (|GetJsonField JsonValue Property))
      (if (not (Utilities|Array|Identical _outvalue (Variables|/Script/Engine.Actor|GetTags _asactor)))
        (Variables|/Script/Engine.Actor|SetTags _asactor _outvalue)
        (return true)))
    (:Hidden
      (bind _outvalue_2 (|GetJsonField JsonValue Property))
      (if (Math|Boolean|NotEqual(Boolean) _outvalue_2 (Variables|/Script/Engine.Actor|GetbHidden _asactor))
        (Rendering|SetActorHiddenInGame _asactor _outvalue_2)
        (return true)))))

(fn RestoreObject
  (params (Object :type Object%20Object%20Reference) (JsonObject :type Json%20Object%20Wrapper%20Structure))
  (bind _fieldnames (Class|JsonBlueprintFunctionLibrary|GetFieldNames JsonObject))
  (Utilities|FlowControl|Sequence
    (:then_0
      (if (Utilities|Array|ContainsItem _fieldnames "Tags")
        (CallFunction|SetPropertyValue Object "Tags" JsonObject)))
    (:then_1
      (if (Utilities|Array|ContainsItem _fieldnames "Hidden")
        (CallFunction|SetPropertyValue Object "Hidden" JsonObject)))))

(fn CollectProperties
  (params (Object :type Object%20Object%20Reference) (TargetJson :type Json%20Object%20Wrapper%20Structure%20%28by%20ref%29))
  (bind _asactor (Utilities|Casting|CastToActor Object))
  (bind _jsonobject (Utilities|MakeArrayJsonParam "Name" "Tags" "Tags" "" (Variables|/Script/Engine.Actor|GetTags _asactor) (Utilities|Name|MakeLiteralName "None") (CallFunction|NewJsonPure)))
  (|SetJsonField TargetJson "Actor" (Utilities|Array|MakeArray _jsonobject))
  (return))

(fn SetMaterial
  (params (Actor :type Actor%20Object%20Reference) (Property :type String) (Json :type Json%20Object%20Wrapper%20Structure))
  (bind (_lefts _rights) (Utilities|String|Split Property "."))
  (if (Utilities|String|Contains Property ".")
    (bind (_outvalue _returnvalue) (|GetJsonField Json Property))
    (if _returnvalue
      (bind _asmaterial_interface (Utilities|Casting|CastToMaterialInterface _outvalue))
      (bind _component (CallFunction|GetPrimitivebyName Actor _lefts))
      (bind _asprimitive_component (Utilities|Casting|CastToPrimitiveComponent _component))
      (Rendering|Material|SetMaterialbyName _asprimitive_component (Utilities|String|StringToName _rights) _asmaterial_interface)
      (return true))))

(fn GetPrimitivebyName
  (params (Actor :type Actor%20Object%20Reference) (Name :type String))
  (if (Utilities|Enum|Equal(Enum) Name "Root")
    (return (Variables|/Script/Engine.Actor|GetRootComponent Actor))
    (else
      (for _array_element (Actor|GetComponentsByClass Actor "/Script/Engine.ActorComponent")
        (if (Utilities|Enum|Equal(Enum) (Utilities|GetDisplayName _array_element) Name)
          (return _array_element))))))