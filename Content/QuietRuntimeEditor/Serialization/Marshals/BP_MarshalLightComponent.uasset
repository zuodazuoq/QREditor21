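; Runtime editor marshal that converts LightComponent properties to and from JSON, extending its parent marshal.
; Serializes and reads shared light settings by name, with a separate helper that writes IES profile fields.
; Restoring feeds each JSON field into SetPropertyValue, which also handles IES, intensity and color, mostly comparing against current values before applying.
; CollectProperties merges parent parameters with temperature, shadow and channel parameters into Light, Advanced and Ray Tracing groups.
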(fn SerializeObject
  (params (Object :type Object%20Object%20Reference) (TargetJson :type Json%20Object%20Wrapper%20Structure%20%28by%20ref%29))
  (|CallParentFunction Object TargetJson)
  (bind _aslight_component (Utilities|Casting|CastToLightComponent Object))
  (Utilities|FlowControl|Sequence
    (:then_0
      (Utilities|FlowControl|Sequence
        (:then_0
          (|SetJsonField TargetJson "Temperature" (Variables|/Script/Engine.LightComponent|GetTemperature _aslight_component)))
        (:then_1
          (|SetJsonField TargetJson "UseTemperature" (Variables|/Script/Engine.LightComponent|GetbUseTemperature _aslight_component)))
        (:then_2
          (|SetJsonField TargetJson "SpecularScale" (Variables|/Script/Engine.LightComponent|GetSpecularScale _aslight_component)))
        (:then_3
          (|SetJsonField TargetJson "ShadowBias" (Variables|/Script/Engine.LightComponent|GetShadowBias _aslight_component)))
        (:then_4
          (|SetJsonField TargetJson "ShadowSlopeBias" (Variables|/Script/Engine.LightComponent|GetShadowSlopeBias _aslight_component)))
        (:then_5
          (|SetJsonField TargetJson "ContactShadowLength" (Variables|/Script/Engine.LightComponent|GetContactShadowLength _aslight_component)))
        (:then_6
          (|SetJsonField TargetJson "ContactShadowInWorldSpace" (Variables|/Script/Engine.LightComponent|GetContactShadowLengthInWS _aslight_component)))
        (:then_7
          (|SetJsonField TargetJson "DynamicIndirectLighting" (Variables|/Script/Engine.LightComponent|GetbAffectDynamicIndirectLighting _aslight_component)))
        (:then_8
          (|SetJsonField TargetJson "LIghtingChannels" (Variables|/Script/Engine.LightComponent|GetLightingChannels _aslight_component)))))
    (:then_1
      (Utilities|FlowControl|Sequence
        (:then_0
          (|SetJsonField TargetJson "LightFunctionMaterial" (Variables|/Script/Engine.LightComponent|GetLightFunctionMaterial _aslight_component)))
        (:then_1
          (|SetJsonField TargetJson "LightFunctionScale" (Variables|/Script/Engine.LightComponent|GetLightFunctionScale _aslight_component)))
        (:then_2
          (|SetJsonField TargetJson "FadeDistance" (Variables|/Script/Engine.LightComponent|GetLightFunctionFadeDistance _aslight_component)))
        (:then_3
          (|SetJsonField TargetJson "DisabledBrightness" (Variables|/Script/Engine.LightComponent|GetDisabledBrightness _aslight_component)))))
    (:then_2
      (return))))

(fn GetPropertyValue
  (params (Object :type Object%20Object%20Reference) (Property :type String))
  (bind _aslight_component (Utilities|Casting|CastToLightComponent Object))
  (bind _outjsonobject (Class|JsonBlueprintFunctionLibrary|FromString "{ }"))
  (switch string Property
    (:Default
      (bind (_success _value) (|CallParentFunction _aslight_component Property))
      (return _success _value))
    (:Temperature
      (|SetJsonField _outjsonobject Property (Variables|/Script/Engine.LightComponent|GetTemperature _aslight_component)))
    (:UseTemperature
      (|SetJsonField _outjsonobject Property (Variables|/Script/Engine.LightComponent|GetbUseTemperature _aslight_component)))
    (:SpecularScale
      (|SetJsonField _outjsonobject Property (Variables|/Script/Engine.LightComponent|GetSpecularScale _aslight_component)))
    (:ShadowBias
      (|SetJsonField _outjsonobject Property (Variables|/Script/Engine.LightComponent|GetShadowBias _aslight_component)))
    (:ShadowSlopeBias
      (|SetJsonField _outjsonobject Property (Variables|/Script/Engine.LightComponent|GetShadowSlopeBias _aslight_component)))
    (:ContactShadowLength
      (|SetJsonField _outjsonobject Property (Variables|/Script/Engine.LightComponent|GetContactShadowLength _aslight_component)))
    (:ContactShadowInWorldSpace
      (|SetJsonField _outjsonobject Property (Variables|/Script/Engine.LightComponent|GetContactShadowLengthInWS _aslight_component)))
    (:DynamicIndirectLighting
      (|SetJsonField _outjsonobject Property (Variables|/Script/Engine.LightComponent|GetbAffectDynamicIndirectLighting _aslight_component)))
    (:LIghtingChannels
      (|SetJsonField _outjsonobject Property (Variables|/Script/Engine.LightComponent|GetLightingChannels _aslight_component)))
    (:LightFunctionMaterial
      (|SetJsonField _outjsonobject Property (Variables|/Script/Engine.LightComponent|GetLightFunctionMaterial _aslight_component)))
    (:LightFunctionScale
      (|SetJsonField _outjsonobject Property (Variables|/Script/Engine.LightComponent|GetLightFunctionScale _aslight_component)))
    (:FadeDistance
      (|SetJsonField _outjsonobject Property (Variables|/Script/Engine.LightComponent|GetLightFunctionFadeDistance _aslight_component)))
    (:DisabledBrightness
      (|SetJsonField _outjsonobject Property (Variables|/Script/Engine.LightComponent|GetDisabledBrightness _aslight_component))))
  (return true _outjsonobject))

(fn SetPropertyValue
  (params (Object :type Object%20Object%20Reference) (Property :type String) (JsonValue :type Json%20Object%20Wrapper%20Structure%20%28by%20ref%29))
  (bind _aslight_component (Utilities|Casting|CastToLightComponent Object))
  (switch string Property
    (:Default
      (bind _success (|CallParentFunction _aslight_component Property JsonValue))
      (return _success))
    (:Temperature
      (bind _newvalue (Utilities|ReadFloatwithCheck JsonValue Property (Variables|/Script/Engine.LightComponent|GetTemperature _aslight_component))
        (:then
          (Class|LightComponent|SetTemperature _aslight_component _newvalue)
          (return true))))
    (:UseTemperature
      (bind _newvalue_2 (Utilities|ReadBoolwithCheck JsonValue Property (Variables|/Script/Engine.LightComponent|GetbUseTemperature _aslight_component))
        (:then
          (Class|LightComponent|SetUseTemperature _aslight_component _newvalue_2)
          (return true))))
    (:SpecularScale
      (bind _newvalue_3 (Utilities|ReadFloatwithCheck JsonValue Property (Variables|/Script/Engine.LightComponent|GetSpecularScale _aslight_component))
        (:then
          (Class|LightComponent|SetSpecularScale _aslight_component _newvalue_3)
          (return true))))
    (:ShadowBias
      (bind _newvalue_4 (Utilities|ReadFloatwithCheck JsonValue Property (Variables|/Script/Engine.LightComponent|GetShadowBias _aslight_component))
        (:then
          (Class|LightComponent|SetShadowBias _aslight_component _newvalue_4)
          (return true))))
    (:ShadowSlopeBias
      (bind _newvalue_5 (Utilities|ReadFloatwithCheck JsonValue Property (Variables|/Script/Engine.LightComponent|GetShadowSlopeBias _aslight_component))
        (:then
          (Class|LightComponent|SetShadowSlopeBias _aslight_component _newvalue_5)
          (return true))))
    (:ContactShadowLength
      (bind _newvalue_6 (Utilities|ReadFloatwithCheck JsonValue Property (Variables|/Script/Engine.LightComponent|GetContactShadowLength _aslight_component))
        (:then
          (Variables|/Script/Engine.LightComponent|SetContactShadowLength _aslight_component _newvalue_6)
          (return true))))
    (:ContactShadowInWorldSpace
      (bind _newvalue_7 (Utilities|ReadBoolwithCheck JsonValue Property (Variables|/Script/Engine.LightComponent|GetContactShadowLengthInWS _aslight_component))
        (:then
          (Variables|/Script/Engine.LightComponent|SetContactShadowLengthInWS _aslight_component _newvalue_7)
          (return true))))
    (:DynamicIndirectLighting
      (bind _newvalue_8 (Utilities|ReadBoolwithCheck JsonValue Property (Variables|/Script/Engine.LightComponent|GetbAffectDynamicIndirectLighting _aslight_component))
        (:then
          (Class|LightComponent|SetAffectDynamicIndirectLighting _aslight_component _newvalue_8)
          (return true))))
    (:LIghtingChannels
      (bind (_outvalue _returnvalue) (|GetJsonField JsonValue Property))
      (if _returnvalue
        (if (not (Math|Boolean|ANDBoolean (Math|Boolean|Equal(Boolean) (.bchannel0 (Variables|/Script/Engine.LightComponent|GetLightingChannels _aslight_component)) (.bChannel0 (Utilities|Struct|BreakLightingChannels _outvalue))) (Math|Boolean|Equal(Boolean) (.bchannel1 (Variables|/Script/Engine.LightComponent|GetLightingChannels _aslight_component)) (.bChannel1 (Utilities|Struct|BreakLightingChannels _outvalue))) (Math|Boolean|Equal(Boolean) (.bchannel2 (Variables|/Script/Engine.LightComponent|GetLightingChannels _aslight_component)) (.bChannel2 (Utilities|Struct|BreakLightingChannels _outvalue)))))
          (Rendering|Components|SetLightingChannels _aslight_component (.bChannel0 (Utilities|Struct|BreakLightingChannels _outvalue)) (.bChannel1 (Utilities|Struct|BreakLightingChannels _outvalue)) (.bChannel2 (Utilities|Struct|BreakLightingChannels _outvalue)))
          (return true))))
    (:LightFunctionMaterial
      (bind (_outvalue_2 _returnvalue_2) (|GetJsonField JsonValue Property))
      (if _returnvalue_2
        (Rendering|Components|Light|SetLightFunctionMaterial _aslight_component _outvalue_2)
        (return true)))
    (:LightFunctionScale
      (bind _newvalue_9 (Utilities|ReadVectorwithCheck JsonValue Property (Variables|/Script/Engine.LightComponent|GetLightFunctionScale _aslight_component))
        (:then
          (Class|LightComponent|SetLightFunctionScale _aslight_component _newvalue_9)
          (return true))))
    (:FadeDistance
      (bind _newvalue_10 (Utilities|ReadFloatwithCheck JsonValue Property (Variables|/Script/Engine.LightComponent|GetLightFunctionFadeDistance _aslight_component))
        (:then
          (Class|LightComponent|SetLightFunctionFadeDistance _aslight_component _newvalue_10)
          (return true))))
    (:DisabledBrightness
      (bind _newvalue_11 (Utilities|ReadFloatwithCheck JsonValue Property (Variables|/Script/Engine.LightComponent|GetDisabledBrightness _aslight_component))
        (:then
          (Class|LightComponent|SetLightFunctionDisabledBrightness _aslight_component _newvalue_11)
          (return true))))
    (:IesTexture
      (bind (_outvalue_3 _returnvalue_3) (|GetJsonField JsonValue Property))
      (if _returnvalue_3
        (if (!= (Variables|/Script/Engine.LightComponent|GetIESTexture _aslight_component) _outvalue_3)
          (Class|LightComponent|SetIESTexture _aslight_component _outvalue_3)
          (return true))))
    (:IesIntensity
      (bind _newvalue_12 (Utilities|ReadBoolwithCheck JsonValue Property (Variables|/Script/Engine.LightComponent|GetbUseIESBrightness _aslight_component))
        (:then
          (Class|LightComponent|SetUseIESBrightness _aslight_component _newvalue_12)
          (return true))))
    (:IesIntensityScale
      (bind _newvalue_13 (Utilities|ReadFloatwithCheck JsonValue Property (Variables|/Script/Engine.LightComponent|GetIESBrightnessScale _aslight_component))
        (:then
          (Class|LightComponent|SetIESBrightnessScale _aslight_component _newvalue_13)
          (return true))))
    (:IndirectLightingIntensity
      (bind _newvalue_14 (Utilities|ReadFloatwithCheck JsonValue Property (Variables|/Script/Engine.LightComponentBase|GetIndirectLightingIntensity _aslight_component))
        (:then
          (Class|LightComponent|SetIndirectLightingIntensity _aslight_component _newvalue_14)
          (return true))))
    (:VolumetricScatteringIntensity
      (bind _newvalue_15 (Utilities|ReadFloatwithCheck JsonValue Property (Variables|/Script/Engine.LightComponentBase|GetVolumetricScatteringIntensity _aslight_component))
        (:then
          (Class|LightComponent|SetVolumetricScatteringIntensity _aslight_component _newvalue_15)
          (return true))))
    (:Intensity
      (bind _newvalue_16 (Utilities|ReadFloatwithCheck JsonValue Property (Variables|/Script/Engine.LightComponentBase|GetIntensity _aslight_component))
        (:then
          (Rendering|Components|Light|SetIntensity _aslight_component _newvalue_16)
          (return true))))
    (:LightColor
      (bind (_outvalue_4 _returnvalue_4) (|GetJsonField JsonValue Property))
      (if _returnvalue_4
        (if (not (Class|KismetMathLibrary|LinearColorIsNearEqual (Rendering|Components|Light|GetLightColor _aslight_component) _outvalue_4 0.0001))
          (Rendering|Components|Light|SetLightColor _aslight_component _outvalue_4 true)
          (return true))))
    (:AffectTranslucentLighting
      (bind _newvalue_17 (Utilities|ReadBoolwithCheck JsonValue Property (Variables|/Script/Engine.LightComponentBase|GetbAffectTranslucentLighting _aslight_component))
        (:then
          (Class|LightComponent|SetAffectTranslucentLighting _aslight_component _newvalue_17)
          (return true))))
    (:Transmission
      (bind _newvalue_18 (Utilities|ReadBoolwithCheck JsonValue Property (Variables|/Script/Engine.LightComponentBase|GetbTransmission _aslight_component))
        (:then
          (Class|LightComponent|SetTransmission _aslight_component _newvalue_18)
          (return true))))))

(fn RestoreObject
  (params (Object :type Object%20Object%20Reference) (JsonObject :type Json%20Object%20Wrapper%20Structure))
  (|CallParentFunction Object JsonObject)
  (bind _fieldnames (Class|JsonBlueprintFunctionLibrary|GetFieldNames JsonObject))
  (for _array_element _fieldnames
    (CallFunction|SetPropertyValue Object _array_element JsonObject)))

(fn CollectProperties
  (params (Object :type Object%20Object%20Reference) (TargetJson :type Json%20Object%20Wrapper%20Structure%20%28by%20ref%29))
  (bind _aslight_component (Utilities|Casting|CastToLightComponent Object))
  (Utilities|FlowControl|Sequence
    (:then_0
      (Utilities|FlowControl|Sequence
        (:then_0
          (bind _jsonobject (CallFunction|NewJson))
          (|CallParentFunction Object _jsonobject)
          (bind _outvalue (|GetJsonField _jsonobject "Light"))
          (LocalVariables|SetLightGroupArray _outvalue)
          (bind _outvalue_2 (|GetJsonField _jsonobject "Advanced"))
          (LocalVariables|SetAdvanced _outvalue_2)
          (bind _outvalue_3 (|GetJsonField _jsonobject "Ray Tracing"))
          (LocalVariables|SetRayTracing _outvalue_3))
        (:then_1
          (bind _jsonobject_2 (CallFunction|MakeBoolParam "UseTemperature" "Use Temperature" "" (Variables|/Script/Engine.LightComponent|GetbUseTemperature _aslight_component) false))
          (Utilities|Array|Add (LocalVariables|GetLightGroupArray) _jsonobject_2))
        (:then_2
          (bind _jsonobject_3 (CallFunction|MakeFloatParam "Temperature" "Temperature" "" (Variables|/Script/Engine.LightComponent|GetTemperature _aslight_component) 6.5e+03 1e+03 1.7e+03 1.5e+04 1.2e+04 1 1))
          (Utilities|Array|Add (LocalVariables|GetLightGroupArray) _jsonobject_3))))
    (:then_1
      (Utilities|FlowControl|Sequence
        (:then_0
          (bind _jsonobject_4 (CallFunction|MakeFloatParam "SpecularScale" "Specular Scale" "" (Variables|/Script/Engine.LightComponent|GetSpecularScale _aslight_component) 1.0 0.0 0.0 1.0 1.0 1 3))
          (Utilities|Array|Add (LocalVariables|GetAdvanced) _jsonobject_4))
        (:then_1
          (bind _jsonobject_5 (CallFunction|MakeFloatParam "ShadowBias" "Shadow Bias" "" (Variables|/Script/Engine.LightComponent|GetShadowBias _aslight_component) 0.5 0.0 0.0 4.0 1.0 1 3))
          (Utilities|Array|Add (LocalVariables|GetAdvanced) _jsonobject_5))
        (:then_2
          (bind _jsonobject_6 (CallFunction|MakeFloatParam "ShadowSlopeBias" "Shadow Slope Bias" "" (Variables|/Script/Engine.LightComponent|GetShadowSlopeBias _aslight_component) 0.5 0.0 0.0 4.0 1.0 1 3))
          (Utilities|Array|Add (LocalVariables|GetAdvanced) _jsonobject_6))
        (:then_3
          (bind _jsonobject_7 (CallFunction|MakeFloatParam "ContactShadowLength" "Contact Shadow Length" "" (Variables|/Script/Engine.LightComponent|GetContactShadowLength _aslight_component) 0.0 0.0 0.0 1.0 0.1 1 3))
          (Utilities|Array|Add (LocalVariables|GetAdvanced) _jsonobject_7))
        (:then_4
          (bind _jsonobject_8 (CallFunction|MakeBoolParam "ContactShadowLengthInWorldSpaceUnits" "Contact Shadow in World Units" "" (Variables|/Script/Engine.LightComponent|GetContactShadowLengthInWS _aslight_component) false))
          (Utilities|Array|Add (LocalVariables|GetAdvanced) _jsonobject_8))
        (:then_5
          (bind _jsonobject_9 (CallFunction|MakeBoolParam "DynamicIndirectLighting" "Dynamic Indirect Lighting" "" (Variables|/Script/Engine.LightComponent|GetbAffectDynamicIndirectLighting _aslight_component) true))
          (Utilities|Array|Add (LocalVariables|GetAdvanced) _jsonobject_9))
        (:then_6
          (bind _jsonobject_10 (CallFunction|MakeLightingChannelsParam "LightingChannels" "Lighting Channels" "" (Variables|/Script/Engine.LightComponent|GetLightingChannels _aslight_component) (LocalVariables|GetDefaultChannels)))
          (Utilities|Array|Add (LocalVariables|GetAdvanced) _jsonobject_10))))
    (:then_2
      (bind _outvalue_4 (|GetJsonField TargetJson "Light"))
      (Utilities|Array|AppendArray (LocalVariables|GetLightGroupArray) _outvalue_4)
      (|SetJsonField TargetJson "Light" (LocalVariables|GetLightGroupArray))
      (|SetJsonField TargetJson "Advanced" (LocalVariables|GetAdvanced))
      (|SetJsonField TargetJson "Ray Tracing" (LocalVariables|GetRayTracing))
      (return))))

(fn CacheLightProfile
  (params (LightComp :type Light%20Component%20Object%20Reference) (JsonObject :type Json%20Object%20Wrapper%20Structure%20%28by%20ref%29))
  (|SetJsonField JsonObject "IesTexture" (Variables|/Script/Engine.LightComponent|GetIESTexture LightComp))
  (|SetJsonField JsonObject "IesIntensity" (Variables|/Script/Engine.LightComponent|GetbUseIESBrightness LightComp))
  (|SetJsonField JsonObject "IesIntensityScale" (Variables|/Script/Engine.LightComponent|GetIESBrightnessScale LightComp))
  (return))