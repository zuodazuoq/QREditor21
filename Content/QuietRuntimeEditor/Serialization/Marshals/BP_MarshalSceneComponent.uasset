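; Marshal Blueprint in the QuietRuntimeEditor serialization system that converts a SceneComponent's Mobility to and from JSON.
; SerializeObject writes the component's Mobility into the target JSON object.
; SetPropertyValue, marked as under construction, reads Mobility from JSON, applies it only when it differs from the current value and returns true on a change.
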(fn SerializeObject
  (params (Object :type Object%20Object%20Reference) (TargetJson :type Json%20Object%20Wrapper%20Structure%20%28by%20ref%29))
  (bind _asscene_component (Utilities|Casting|CastToSceneComponent Object))
  (|SetJsonField TargetJson "Mobility" (Variables|/Script/Engine.SceneComponent|GetMobility _asscene_component))
  (return))

(fn SetPropertyValue
  (params (Object :type Object%20Object%20Reference) (Property :type String) (JsonValue :type Json%20Object%20Wrapper%20Structure%20%28by%20ref%29))
  ;[0.09896 0.009864 0] Under Construction
  (bind _asscene_component (Utilities|Casting|CastToSceneComponent Object))
  (switch string Property
    (:Mobility
      (bind _outvalue (|GetJsonField JsonValue "Mobility"))
      (if (Utilities|Enum|NotEqual(Enum) _outvalue (Variables|/Script/Engine.SceneComponent|GetMobility _asscene_component))
        (Transformation|SetMobility _asscene_component _outvalue)
        (return true)))))