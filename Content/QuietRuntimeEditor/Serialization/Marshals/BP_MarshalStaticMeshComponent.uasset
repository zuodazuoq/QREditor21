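; Marshal for StaticMeshComponent in the runtime editor, saving, restoring and exposing its properties on top of the parent marshal.
; It writes mesh, reverse culling and a cached materials array to JSON, then restores each field through SetPropertyValue, which handles properties the parent does not.
; CollectProperties builds editor parameters, including one per material slot defaulting to the mesh's material, and hides the mesh picker for Datasmith runtime-tagged actors.
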(fn SerializeObject
  (params (Object :type Object%20Object%20Reference) (TargetJson :type Json%20Object%20Wrapper%20Structure%20%28by%20ref%29))
  (|CallParentFunction Object TargetJson)
  (bind _asstatic_mesh_component (Utilities|Casting|CastToStaticMeshComponent Object))
  (Utilities|FlowControl|Sequence
    (:then_0
      (|SetJsonField TargetJson "StaticMesh" (Variables|/Script/Engine.StaticMeshComponent|GetStaticMesh _asstatic_mesh_component))
      (bind _cachedmaterials (Default|CacheMaterialArray (CallFunction|GetSource) (Rendering|Material|GetMaterials _asstatic_mesh_component)))
      (|SetJsonField TargetJson "Materials" _cachedmaterials))
    (:then_1
      (|SetJsonField TargetJson "ReverseCulling" (Variables|/Script/Engine.StaticMeshComponent|GetbReverseCulling _asstatic_mesh_component))
      (return))))

(fn GetPropertyValue
  (params (Object :type Object%20Object%20Reference) (Property :type String))
  (bind (_success _value) (|CallParentFunction Object Property))
  (if (not _success)
    (bind _asstatic_mesh_component (Utilities|Casting|CastToStaticMeshComponent Object))
    (bind _outjsonobject (Class|JsonBlueprintFunctionLibrary|FromString "{ }"))
    (switch string Property
      (:StaticMesh
        (|SetJsonField _outjsonobject Property (Variables|/Script/Engine.StaticMeshComponent|GetStaticMesh _asstatic_mesh_component))
        (return true _outjsonobject))
      (:ReverseCulling
        (bind _returnvalue (|SetJsonField _outjsonobject Property (Variables|/Script/Engine.StaticMeshComponent|GetbReverseCulling _asstatic_mesh_component)))
        (return _returnvalue _outjsonobject)))
    (else
      (return true _value))))

(fn RestoreObject
  (params (Object :type Object%20Object%20Reference) (JsonObject :type Json%20Object%20Wrapper%20Structure))
  (|CallParentFunction Object JsonObject)
  (bind _fieldnames (Class|JsonBlueprintFunctionLibrary|GetFieldNames JsonObject))
  (for _array_element _fieldnames
    (CallFunction|SetPropertyValue Object _array_element JsonObject)))

(fn SetPropertyValue
  (params (Object :type Object%20Object%20Reference) (Property :type String) (JsonValue :type Json%20Object%20Wrapper%20Structure%20%28by%20ref%29))
  (bind _success (|CallParentFunction Object Property JsonValue))
  (if (not _success)
    (bind _asstatic_mesh_component (Utilities|Casting|CastToStaticMeshComponent Object))
    (switch string Property
      (:StaticMesh
        ;[0 0 0] Restore Mesh
        (bind (_outvalue _returnvalue) (|GetJsonField JsonValue Property))
        (if _returnvalue
          (if (!= (Variables|/Script/Engine.StaticMeshComponent|GetStaticMesh _asstatic_mesh_component) _outvalue)
            (bind _asstatic_mesh (Utilities|Casting|CastToStaticMesh _outvalue)
              (:then
                (bind _returnvalue_2 (Components|StaticMesh|SetStaticMesh _asstatic_mesh_component _asstatic_mesh))
                (return _returnvalue_2))
              (:CastFailed
                (bind _returnvalue_3 (Components|StaticMesh|SetStaticMesh _asstatic_mesh_component 0))
                (return _returnvalue_3))))))
      (:ReverseCulling
        (bind _newvalue (Utilities|ReadBoolwithCheck JsonValue Property (Variables|/Script/Engine.StaticMeshComponent|GetbReverseCulling _asstatic_mesh_component))
          (:then
            (Class|StaticMeshComponent|SetReverseCulling _asstatic_mesh_component _newvalue)
            (return true))))
      (:Materials
        ;[0 0 0] Restore Materials
        (bind _outvalue_2 (|GetJsonField JsonValue Property))
        (bind _materials (Default|RestoreMaterialsArray (CallFunction|GetSource) _outvalue_2))
        (for (_array_element _array_index) _materials
          (Utilities|IsValid _array_element
            (:Is%20Valid
              (Rendering|Material|SetMaterial _asstatic_mesh_component _array_index _array_element))))))
    (else
      (return true))))

(fn CollectProperties
  (params (Object :type Object%20Object%20Reference) (TargetJson :type Json%20Object%20Wrapper%20Structure%20%28by%20ref%29))
  (bind _asstatic_mesh_component (Utilities|Casting|CastToStaticMeshComponent Object))
  (|SetJsonField TargetJson "GroupsState" (Utilities|Array|MakeArray "Static Mesh" "Materials" "Actor"))
  (if (not (Actor|ActorHasTag (Components|GetOwner _asstatic_mesh_component) "Datasmith.Runtime.Tag"))
    (bind _jsonobject (CallFunction|MakeObjectParam "StaticMesh" "Static Mesh" "" "/Script/Engine.StaticMesh" (Variables|/Script/Engine.StaticMeshComponent|GetStaticMesh _asstatic_mesh_component)))
    (|SetJsonField _jsonobject "Dependencies" (Utilities|Array|MakeArray))
    (Utilities|Array|Add (LocalVariables|GetMeshGroup) _jsonobject))
  (bind _jsonobject_2 (CallFunction|MakeBoolParam "ReverseCulling" "Reverse Culling" "" (Variables|/Script/Engine.StaticMeshComponent|GetbReverseCulling _asstatic_mesh_component) false))
  (Utilities|Array|Add (LocalVariables|GetMeshGroup) _jsonobject_2)
  (|SetJsonField TargetJson "Static Mesh" (LocalVariables|GetMeshGroup))
  (bind _params (CallFunction|CollectMeshMaterials _asstatic_mesh_component))
  (|SetJsonField TargetJson "Materials" _params)
  (|CallParentFunction _asstatic_mesh_component TargetJson)
  (return))

(fn CollectMeshMaterials
  (params (Component :type Static%20Mesh%20Component%20Object%20Reference))
  (for (_array_element _array_index) (Rendering|Material|GetMaterials Component)
    (bind _jsonobject (CallFunction|MakeObjectParam (Utilities|String|Append (Utilities|String|SelectString "Root" (Utilities|GetDisplayName Component) (== Component (Variables|/Script/Engine.Actor|GetRootComponent (Components|GetOwner Component)))) "." (Utilities|String|ToString(Name) (Utilities|Array|Get(acopy) (Class|MeshComponent|GetMaterialSlotNames Component) _array_index))) (Utilities|String|ToString(Name) (Utilities|Array|Get(acopy) (Class|MeshComponent|GetMaterialSlotNames Component) _array_index)) "" "/Script/Engine.MaterialInstanceConstant" _array_element (Rendering|Material|GetMaterial (Variables|/Script/Engine.StaticMeshComponent|GetStaticMesh Component) _array_index)))
    (Utilities|Array|Add (LocalVariables|GetParameters) _jsonobject))
  (return (LocalVariables|GetParameters)))