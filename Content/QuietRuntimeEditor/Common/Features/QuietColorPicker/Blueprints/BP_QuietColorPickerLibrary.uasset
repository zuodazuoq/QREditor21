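; Function library for the QuietRuntimeEditor color picker that compares two color themes for equality or inequality.
; EqualTheme checks that the Colors and Labels arrays are identical, and NotEqualTheme repeats the same test negated.
; Despite its name, the ExceptName flag adds the Name comparison when true, and Name is ignored when it is false.
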(fn EqualTheme
  (params (A :type F%20Color%20Theme%20Structure) (B :type F%20Color%20Theme%20Structure) (Except%20Name :type Boolean))
  (bind (_name _colors _labels) (Utilities|Struct|BreakF_ColorTheme A))
  (bind (_name_2 _colors_2 _labels_2) (Utilities|Struct|BreakF_ColorTheme B))
  (bind _returnvalue (Utilities|Array|Identical _labels _labels_2))
  (bind _returnvalue_2 (Utilities|Array|Identical _colors _colors_2))
  (bind _returnvalue_3 (and _returnvalue_2 _returnvalue))
  (if Except%20Name
    (return (and (Utilities|Enum|Equal(Enum) _name _name_2) _returnvalue_3))
    (else
      (return _returnvalue_3))))

(fn NotEqualTheme
  (params (A :type F%20Color%20Theme%20Structure) (B :type F%20Color%20Theme%20Structure) (Except%20Name :type Boolean))
  (bind (_name _colors _labels) (Utilities|Struct|BreakF_ColorTheme A))
  (bind (_name_2 _colors_2 _labels_2) (Utilities|Struct|BreakF_ColorTheme B))
  (bind _returnvalue (Utilities|Array|Identical _labels _labels_2))
  (bind _returnvalue_2 (Utilities|Array|Identical _colors _colors_2))
  (bind _returnvalue_3 (and _returnvalue_2 _returnvalue))
  (if Except%20Name
    (return (not (and (Utilities|Enum|Equal(Enum) _name _name_2) _returnvalue_3)))
    (else
      (return (not _returnvalue_3)))))