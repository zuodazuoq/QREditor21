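; SaveGame object for the Quiet color picker that stores a library of named color themes, each with colors and labels, and saves itself to a slot.
; It manages the theme map and active theme, supporting add, duplicate, rename, remove and color edits, creating a theme on initialization if empty.
; Name clashes are resolved with numeric suffixes.
; Dispatchers announce active-theme switches and theme edits, with equality checks skipping redundant updates.
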(event Custom|Initialize
  (if (Utilities|Map|IsEmpty (Variables|Default|GetThemes))
    (CallFunction|AddNewTheme)))

(event Custom|SaveThemes
  (SaveGame|SaveGametoSlot self "QuietColotLibrary"))

(event Custom|RemoveTheme
  (params (Name :type String))
  (Utilities|Map|Remove (Variables|Default|GetThemes) Name)
  (if (Utilities|Enum|Equal(Enum) Name (Variables|Default|GetActiveThemeName))
    (if (not (Utilities|Map|IsEmpty (Variables|Default|GetThemes)))
      (bind _keys (Utilities|Map|Keys (Variables|Default|GetThemes)))
      (bind _output_get (Variables|Default|SetActiveThemeName (Utilities|Array|Get(acopy) _keys)))
      (Default|CallNotifyonActiveThemeChanged _output_get))))

(event Custom|UpdateThemeByName
  (params (Theme :type F%20Color%20Theme%20Structure))
  (bind _name (Utilities|Struct|BreakF_ColorTheme Theme))
  (bind _theme (CallFunction|GetThemebyName _name))
  (if (not (Utilities|EqualTheme _theme Theme true))
    (Utilities|Map|Add (Variables|Default|GetThemes) _name Theme)
    (if (Utilities|Enum|Equal(Enum) _name (Variables|Default|GetActiveThemeName))
      (Default|CallNotifyonThemeUpdated Theme))))

(event Custom|RenameTheme
  (params (NewName :type String))
  (bind _keys (Utilities|Map|Keys (Variables|Default|GetThemes)))
  (Utilities|FixIdenticalName NewName _keys)
  (bind _theme (CallFunction|GetThemebyName (Variables|Default|GetActiveThemeName)))
  (Utilities|Map|Add (Variables|Default|GetThemes) NewName (Utilities|Struct|MakeF_ColorTheme NewName (.colors _theme) (.labels _theme)))
  (Utilities|Map|Remove (Variables|Default|GetThemes) (Variables|Default|GetActiveThemeName))
  (Variables|Default|SetActiveThemeName NewName))

(event Custom|UpdateSelectedTheme
  (params (Theme :type F%20Color%20Theme%20Structure))
  (bind _name (Utilities|Struct|BreakF_ColorTheme Theme))
  (bind _theme (CallFunction|GetThemebyName _name))
  (if (not (Utilities|EqualTheme _theme Theme true))
    (Utilities|Map|Add (Variables|Default|GetThemes) _name Theme)
    (Default|CallUpdateThemes (Variables|Default|GetThemes) (Variables|Default|GetActiveThemeName))))

(fn FixIdenticalName
  (params (SourceName :type String%20%28by%20ref%29) (ExistingNames :type Array%20of%20Strings))
  (Utilities|Set|AddItems (LocalVariables|GetCollection) ExistingNames)
  (if (Utilities|Set|Contains (LocalVariables|GetCollection) SourceName)
    (if (CallFunction|EndswithNumber SourceName)
      (bind _string (CallFunction|SplitStringbyIndex SourceName))
      (LocalVariables|SetBase _string)
      (else
        (LocalVariables|SetBase SourceName)))
    (for _index (range 0 (Utilities|Set|Length (LocalVariables|GetCollection)))
      (if (not (Utilities|Set|Contains (LocalVariables|GetCollection) (Utilities|String|Append (LocalVariables|GetBase) " " (Utilities|String|ToString(Integer) _index))))
        (|SetBy-RefVar SourceName (Utilities|String|Append (LocalVariables|GetBase) " " (Utilities|String|ToString(Integer) _index)))
        (return)))))

(fn GetActiveTheme
  (bind _themes (Variables|Default|GetThemes))
  (bind _activethemename (Variables|Default|GetActiveThemeName))
  (bind (_value _returnvalue) (Utilities|Map|Find _themes _activethemename))
  (return _returnvalue _value))

(fn SetActiveTheme
  (params (ActiveThemeName :type String))
  (bind _output_get (Variables|Default|SetActiveThemeName ActiveThemeName))
  (Default|CallNotifyonActiveThemeChanged _output_get))

(fn AddNewTheme
  (bind _newname (LocalVariables|GetNewName))
  (bind _keys (Utilities|Map|Keys (Variables|Default|GetThemes)))
  (Utilities|FixIdenticalName (LocalVariables|GetNewName) _keys)
  (Utilities|Map|Add (Variables|Default|GetThemes) _newname (Utilities|Struct|MakeF_ColorTheme _newname (Utilities|Array|MakeArray) 0))
  (Variables|Default|SetActiveThemeName (LocalVariables|GetNewName))
  (Default|CallNotifyonActiveThemeChanged (LocalVariables|GetNewName))
  (return (LocalVariables|GetNewName)))

(fn GetThemebyName
  (params (Name :type String))
  (bind _themes (Variables|Default|GetThemes))
  (bind (_value _returnvalue) (Utilities|Map|Find _themes Name))
  (if _returnvalue
    (return true _value)))

(fn DuplicateTheme
  (LocalVariables|SetNewName (Variables|Default|GetActiveThemeName))
  (bind _keys (Utilities|Map|Keys (Variables|Default|GetThemes)))
  (Utilities|FixIdenticalName (LocalVariables|GetNewName) _keys)
  (Utilities|Map|Add (Variables|Default|GetThemes) (LocalVariables|GetNewName) (Utilities|Struct|MakeF_ColorTheme (LocalVariables|GetNewName) (.colors (.Value (Utilities|Map|Find (Variables|Default|GetThemes) (Variables|Default|GetActiveThemeName)))) (.labels (.Value (Utilities|Map|Find (Variables|Default|GetThemes) (Variables|Default|GetActiveThemeName))))))
  (Default|CallUpdateThemes (Variables|Default|GetThemes) (Variables|Default|GetActiveThemeName))
  (Variables|Default|SetActiveThemeName (LocalVariables|GetNewName))
  (Default|CallNotifyonActiveThemeChanged (LocalVariables|GetNewName))
  (return (LocalVariables|GetNewName)))

(fn AddColortoTheme
  (params (ThemeName :type String%20%28by%20ref%29) (Color :type Linear%20Color%20Structure))
  (bind _themes (Variables|Default|GetThemes))
  (bind (_value _returnvalue) (Utilities|Map|Find _themes ThemeName))
  (bind (_name _colors _labels) (Utilities|Struct|BreakF_ColorTheme _value))
  (if _returnvalue
    (bind _output_get (LocalVariables|SetColors _colors))
    (Utilities|Array|Add _output_get Color)
    (bind _output_get_2 (LocalVariables|SetLabels _labels))
    (Utilities|Array|Add _output_get_2 "")
    (Utilities|Map|Add (Variables|Default|GetThemes) ThemeName (Utilities|Struct|MakeF_ColorTheme ThemeName (LocalVariables|GetColors) (LocalVariables|GetLabels)))
    (if (Utilities|Enum|Equal(Enum) ThemeName (Variables|Default|GetActiveThemeName))
      (Default|CallNotifyonThemeUpdated (Utilities|Struct|MakeF_ColorTheme ThemeName (LocalVariables|GetColors) (LocalVariables|GetLabels))))))

(fn RemoveColorfromTheme
  (params (ThemeName :type String) (Color :type Linear%20Color%20Structure))
  (bind _themes (Variables|Default|GetThemes))
  (bind (_value _returnvalue) (Utilities|Map|Find _themes ThemeName))
  (bind (_colors _labels) (Utilities|Struct|BreakF_ColorTheme _value))
  (if _returnvalue
    (LocalVariables|SetLocalLabels _labels)
    (bind _output_get (LocalVariables|SetColors _colors))
    (if (Utilities|Array|ContainsItem _output_get Color)
      (Utilities|Array|RemoveIndex (LocalVariables|GetLocalLabels) (Utilities|Array|FindItem (LocalVariables|GetColors) Color))
      (Utilities|Array|RemoveItem (LocalVariables|GetColors) Color)
      (Utilities|Map|Add (Variables|Default|GetThemes) ThemeName (Utilities|Struct|MakeF_ColorTheme ThemeName (LocalVariables|GetColors) (LocalVariables|GetLocalLabels)))
      (if (Utilities|Enum|Equal(Enum) ThemeName (Variables|Default|GetActiveThemeName))
        (Default|CallNotifyonThemeUpdated (Utilities|Struct|MakeF_ColorTheme ThemeName (LocalVariables|GetColors) (LocalVariables|GetLocalLabels)))))))

(fn EqualTheme
  (params (A :type F%20Color%20Theme%20Structure%20%28by%20ref%29) (B :type F%20Color%20Theme%20Structure%20%28by%20ref%29) (IncludingName :type Boolean))
  (bind (_name _colors _labels) (Utilities|Struct|BreakF_ColorTheme A))
  (bind (_name_2 _colors_2 _labels_2) (Utilities|Struct|BreakF_ColorTheme B))
  (bind _returnvalue (Utilities|Array|Identical _labels _labels_2))
  (bind _returnvalue_2 (Utilities|Array|Identical _colors _colors_2))
  (bind _returnvalue_3 (and _returnvalue_2 _returnvalue))
  (if IncludingName
    (return (and (Utilities|Enum|Equal(Enum) _name _name_2) _returnvalue_3))
    (else
      (return _returnvalue_3))))

(fn EndswithNumber
  (params (SourceString :type String))
  (return (Class|KismetStringLibrary|IsNumeric (Utilities|String|Right SourceString 1))))

(fn SplitStringbyIndex
  (params (InputPin :type String))
  (bind _returnvalue (Utilities|String|Len InputPin))
  (for _index (range 1 _returnvalue)
    (if (not (Math|Integer|InRange(Integer) (Utilities|String|GetCharacterasNumber InputPin (- _returnvalue _index)) 48 57))
      (return (Utilities|String|SelectString (Utilities|String|LeftChop (Utilities|String|GetSubstring InputPin 0 (+ (- _returnvalue _index) 1)) 1) (Utilities|String|GetSubstring InputPin 0 (+ (- _returnvalue _index) 1)) (Utilities|String|EndsWith (Utilities|String|GetSubstring InputPin 0 (+ (- _returnvalue _index) 1)) " ")) (Math|Conversions|ToInteger(Byte) (Utilities|String|GetSubstring InputPin (- _returnvalue _index) _index)))))
  (return "" (Math|Conversions|ToInteger(Byte) InputPin)))