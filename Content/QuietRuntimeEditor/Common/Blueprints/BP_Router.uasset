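; BP_Router is a tag-keyed message router for the Quiet runtime editor.
; Objects implementing BI_QuietRoutingInterface register under a tag in the Subscribers map, and FindSubscriberWithTag resolves them.
; Typed wrappers forward commands, actors, objects, materials and JSON, or relay data requests, actor queries and duplication through interface messages.
; Forwarding and data calls report success even without a matching subscriber, and the generic Throw is an unfinished stub.
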(fn ThrowCommand
  (params (Target :type Gameplay%20Tag%20Structure) (Command :type Gameplay%20Tag%20Structure))
  (bind _object (Utilities|FindSubscriberwithTag Target))
  (Class|BIQuietRoutingInterface|ForwardCommand(Message) _object Command)
  (return true))

(fn SubscribewithTag
  (params (Tag :type Gameplay%20Tag%20Structure) (Object :type Object%20Object%20Reference))
  (if (Utilities|DoesObjectImplementInterface Object "/Game/QuietRuntimeEditor/Common/Blueprints/BI_QuietRoutingInterface.BI_QuietRoutingInterface_C")
    (Utilities|Map|Add (Variables|Default|GetSubscribers) Tag Object)
    (return true)))

(fn Throw
  (params (Target :type Gameplay%20Tag%20Container%20Structure) (Command :type Gameplay%20Tag%20Structure) (Row :type Gameplay%20Tag%20Table%20Row%20Structure))
  (for _array_element (GameplayTags|BreakGameplayTagContainer Target)
    _))

(fn ThrowActor
  (params (Target :type Gameplay%20Tag%20Structure) (Action :type Gameplay%20Tag%20Structure) (Actor :type Actor%20Object%20Reference))
  (bind _object (Utilities|FindSubscriberwithTag Target))
  (Class|BIQuietRoutingInterface|ForwardActor(Message) _object Action Actor)
  (return true))

(fn ThrowObject
  (params (Target :type Gameplay%20Tag%20Structure) (Action :type Gameplay%20Tag%20Structure) (Object :type Object%20Object%20Reference))
  (bind _object (Utilities|FindSubscriberwithTag Target))
  (Class|BIQuietRoutingInterface|ForwardObject(Message) _object Action Object)
  (return true))

(fn ThrowMaterial
  (params (Target :type Gameplay%20Tag%20Structure) (Action :type Gameplay%20Tag%20Structure) (Material :type Material%20Interface%20Object%20Reference))
  (bind _object (Utilities|FindSubscriberwithTag Target))
  (Class|BIQuietRoutingInterface|ForwardMaterial(Message) _object Action Material)
  (return true))

(fn ThrowJson
  (params (Target :type Gameplay%20Tag%20Structure) (Action :type Gameplay%20Tag%20Structure) (Json :type Json%20Object%20Wrapper%20Structure))
  (bind _object (Utilities|FindSubscriberwithTag Target))
  (Class|BIQuietRoutingInterface|ForwardJson(Message) _object Action Json)
  (return true))

(fn RequestDatawithTag
  (params (Target :type Gameplay%20Tag%20Structure) (Request :type Gameplay%20Tag%20Structure) (InputData :type Json%20Object%20Wrapper%20Structure))
  (bind _object (Utilities|FindSubscriberwithTag Target))
  (bind _data (Class|BIQuietRoutingInterface|ReturnDatabyRequestwithTag(Message) _object Request InputData))
  (return true _data))

(fn GetDatawithTag
  (params (Target :type Gameplay%20Tag%20Structure) (Request :type Gameplay%20Tag%20Structure))
  (bind _object (Utilities|FindSubscriberwithTag Target))
  (bind _data (Class|BIQuietRoutingInterface|GetDatawithTag(Message) _object Request))
  (return true _data))

(fn GetActorswithTag
  (params (Target :type Gameplay%20Tag%20Structure) (DesiredObjects :type Gameplay%20Tag%20Structure))
  (bind _object (Utilities|FindSubscriberwithTag Target))
  (bind _actors (Class|BIQuietRoutingInterface|TakeActorswithTag(Message) _object DesiredObjects))
  (return _actors))

(fn DuplicateActor
  (params (Target :type Gameplay%20Tag%20Structure) (Actor :type Actor%20Object%20Reference))
  (bind _object (Utilities|FindSubscriberwithTag Target))
  (bind _copy (Class|BIQuietRoutingInterface|DuplicateActorwithTag(Message) _object Actor))
  (return _copy))