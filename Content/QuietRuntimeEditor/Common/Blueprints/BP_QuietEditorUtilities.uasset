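; Blueprint utility library for the Quiet Runtime Editor, with helpers for asset names and paths, actor bounds, component lookup, and warning or progress widgets.
; String sorting shuffles, then runs a recursive quicksort whose comparer orders trailing numbers numerically.
; The same suffix-splitting helper lets UnifyName generate unique indexed names.
; Directory helpers resolve user or project-saved folders and create missing ones, with the scene save location read from a string table.
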(fn RemoveAssetPrefix
  (params (Name :type String))
  (for _array_element (LocalVariables|GetPrefixes)
    (if (Utilities|String|StartsWith Name _array_element)
      (return (QuietEditorUtilities|Names|RemoveAssetSuffix (Utilities|String|Replace Name _array_element)))))
  (return (QuietEditorUtilities|Names|RemoveAssetSuffix Name)))

(fn RemoveAssetSuffix
  (params (SourceString :type String))
  (if (Utilities|String|EndsWith SourceString "_C")
    (return (Utilities|String|LeftChop SourceString 2))
    (else
      (return SourceString))))

(fn GetCenterOfActors
  (params (Actors :type Array%20of%20Actor%20Object%20References))
  (for _array_element Actors
    (Utilities|Array|Add (LocalVariables|GetLocalAverages) (.Origin (Collision|GetActorBounds _array_element false false))))
  (return (Math|Vector|GetVectorArrayAverage (LocalVariables|GetLocalAverages))))

(fn GetActorsBounds
  (params (Actors :type Array%20of%20Actor%20Object%20References))
  (bind (_center _boxextent) (Collision|GetActorArrayBounds Actors))
  (return _center (Math|Vector|VectorLength (Math|Vector|MakeVector (Math|Vector|GetMaxElement _boxextent) (Math|Vector|GetMaxElement _boxextent) (Math|Vector|GetMaxElement _boxextent)))))

(fn RemoveAssetPrefixPure
  (params (Name :type String))
  (for _array_element (LocalVariables|GetPrefixes)
    (if (Utilities|String|StartsWith Name _array_element)
      (return (QuietEditorUtilities|Names|RemoveAssetSuffix (Utilities|String|Replace Name _array_element)))))
  (return (QuietEditorUtilities|Names|RemoveAssetSuffix Name)))

(fn SortStringArray
  (params (Array :type Array%20of%20Strings))
  (Utilities|Array|Shuffle Array)
  (SortStrings|QuickSortImpl Array 0 (Utilities|Array|LastIndex Array))
  (return Array))

(fn GetComponentName
  (params (Component :type Actor%20Component%20Object%20Reference))
  (return (Utilities|String|SelectString "Root" (Utilities|GetDisplayName Component) (== Component (Variables|/Script/Engine.Actor|GetRootComponent (Components|GetOwner Component))))))

(fn GetComponentbyName
  (params (Actor :type Actor%20Object%20Reference) (Name :type String))
  (if (Utilities|Enum|Equal(Enum) Name "Root")
    (return (Variables|/Script/Engine.Actor|GetRootComponent Actor))
    (else
      (for _array_element (Actor|GetComponentsByClass Actor "/Script/Engine.ActorComponent")
        (if (Utilities|Enum|Equal(Enum) Name (Utilities|GetDisplayName _array_element))
          (return _array_element))))))

(fn CallWarningDialog
  (params (OwningPlayer :type Player%20Controller%20Object%20Reference) (MessageType :type E_QuietMsgType%20Enum :default "NewEnumerator0") (DefaultValue :type E_QuietMsgReturnValue%20Enum :default "NewEnumerator0") (Message :type Text) (Callback :type Delegate%20%28by%20ref%29))
  (bind _returnvalue (UserInterface|CreateWidget "/Game/QuietRuntimeEditor/Common/Widgets/WBP_QuietWarningDialog.WBP_QuietWarningDialog_C" OwningPlayer MessageType DefaultValue Message))
  (UserInterface|Viewport|AddtoViewport _returnvalue 0)
  (EventDispatchers|BindEventtoNotifyonMessageProcessed _returnvalue Callback))

(fn GetUserContentFolder
  (return (Utilities|String|ToString(Text) (Utilities|Text|MakeLiteralText "UserContent"))))

(fn GetSaveDirectory
  (bind _returnvalue (Class|BlueprintFileUtilsBPLibrary|GetUserDirectory))
  (bind _returnvalue_2 (Class|BlueprintPathsLibrary|ProjectSavedDir))
  (bind _returnvalue_3 (Class|KismetStringTableLibrary|GetTableEntrySourceString "/Game/QuietRuntimeEditor/Settings/ST_Resources.ST_Resources" "SaveDirectory"))
  (bind _returnvalue_4 (Class|KismetSystemLibrary|GetGameName))
  (bind _returnvalue_5 (Utilities|String|Append _returnvalue "/" _returnvalue_4 "/SaveScenes"))
  (bind _returnvalue_6 (Utilities|String|Append _returnvalue_2 "/SaveScenes"))
  (switch string _returnvalue_3
    (:Default
      (return _returnvalue_3))
    (:UserDirectory
      (bind _returnvalue_7 (Class|BlueprintFileUtilsBPLibrary|DirectoryExists _returnvalue_5))
      (if _returnvalue_7
        _
        (else
          (Class|BlueprintFileUtilsBPLibrary|MakeDirectory _returnvalue_5 true)))
      (return _returnvalue_5))
    (:ProjectSavedDir
      (bind _returnvalue_8 (Class|BlueprintFileUtilsBPLibrary|DirectoryExists _returnvalue_6))
      (if _returnvalue_8
        _
        (else
          (Class|BlueprintFileUtilsBPLibrary|MakeDirectory _returnvalue_6 false)))
      (return _returnvalue_6))))

(fn GetThumbnailsDir
  (bind _returnvalue (Utilities|Text|MakeLiteralText "SaveDirectory"))
  (bind _returnvalue_2 (Class|KismetSystemLibrary|GetGameName))
  (bind _returnvalue_3 (Class|BlueprintFileUtilsBPLibrary|GetUserDirectory))
  (bind _returnvalue_4 (Class|BlueprintPathsLibrary|ProjectSavedDir))
  (bind _returnvalue_5 (Utilities|String|ToString(Text) _returnvalue))
  (bind _returnvalue_6 (Utilities|String|Append _returnvalue_3 "/" _returnvalue_2 "/Thumbnails"))
  (bind _returnvalue_7 (Utilities|String|Append _returnvalue_4 "/Thumbnails"))
  (switch string _returnvalue_5
    (:Default
      (return _returnvalue_5))
    (:UserDirectory
      (bind _returnvalue_8 (Class|BlueprintFileUtilsBPLibrary|DirectoryExists _returnvalue_6))
      (if _returnvalue_8
        _
        (else
          (Class|BlueprintFileUtilsBPLibrary|MakeDirectory _returnvalue_6 true)))
      (return _returnvalue_6))
    (:ProjectSavedDir
      (bind _returnvalue_9 (Class|BlueprintFileUtilsBPLibrary|DirectoryExists _returnvalue_7))
      (if _returnvalue_9
        _
        (else
          (Class|BlueprintFileUtilsBPLibrary|MakeDirectory _returnvalue_7 false)))
      (return _returnvalue_7))))

(fn SplitbyIndex
  (params (String :type String))
  (bind _returnvalue (Class|KismetStringLibrary|ToUpper String))
  (bind _returnvalue_2 (Utilities|String|Len _returnvalue))
  (for _index (range 1 _returnvalue_2)
    (if (Class|KismetStringLibrary|IsNumeric (Utilities|String|Right _returnvalue _index))
      (LocalVariables|SetSuffix (Utilities|String|Right _returnvalue _index))
      (LocalVariables|SetSuccess true)
      (elif (and (> (Utilities|String|GetCharacterasNumber (Utilities|String|Right (Utilities|String|Left _returnvalue (- _returnvalue_2 (- _index 1))) 1)) 65) (< (Utilities|String|GetCharacterasNumber (Utilities|String|Right (Utilities|String|Left _returnvalue (- _returnvalue_2 (- _index 1))) 1)) 91))
        (return (LocalVariables|GetSuccess) (Utilities|String|Left _returnvalue (- _returnvalue_2 (- _index 1))) (LocalVariables|GetSuffix))
        (else
          (LocalVariables|SetSuffix (Utilities|String|Right _returnvalue _index))
          (if (and (> (Utilities|String|GetCharacterasNumber (Utilities|String|Right (Utilities|String|Left _returnvalue (- _returnvalue_2 (- _index 1))) 1)) 47) (< (Utilities|String|GetCharacterasNumber (Utilities|String|Right (Utilities|String|Left _returnvalue (- _returnvalue_2 (- _index 1))) 1)) 58))
            (LocalVariables|SetSuccess true)))))))

(fn EndswithNumber
  (params (String :type String))
  (return (Class|KismetStringLibrary|IsNumeric (Utilities|String|Right String 1))))

(fn CallWarningDialogSimple
  (params (OwningPlayer :type Player%20Controller%20Object%20Reference) (Message :type Text))
  (bind _returnvalue (UserInterface|CreateWidget "/Game/QuietRuntimeEditor/Common/Widgets/WBP_QuietWarningDialog.WBP_QuietWarningDialog_C" OwningPlayer "NewEnumerator0" "NewEnumerator0" Message))
  (UserInterface|Viewport|AddtoViewport _returnvalue 0))

(fn Greater
  (params (lhs :type String) (rhs :type String))
  (LocalVariables|SetLhsLen (Utilities|String|Len lhs))
  (LocalVariables|SetRhsLen (Utilities|String|Len rhs))
  (for _index (range 0 (- (Math|Integer|Min(Integer) (LocalVariables|GetLhsLen) (LocalVariables|GetRhsLen)) 1))
    (LocalVariables|SetLhsChar (Utilities|String|GetCharacterasNumber lhs _index))
    (LocalVariables|SetRhsChar (Utilities|String|GetCharacterasNumber rhs _index))
    (if (not (== (LocalVariables|GetLhsChar) (LocalVariables|GetRhsChar)))
      (return (> (LocalVariables|GetLhsChar) (LocalVariables|GetRhsChar)))))
  (return (> (LocalVariables|GetLhsLen) (LocalVariables|GetRhsLen))))

(fn Partition
  (params (In :type Array%20of%20Strings) (lo :type Integer) (hi :type Integer))
  (LocalVariables|SetPivot (Utilities|Array|Get(acopy) In hi))
  (LocalVariables|Seti (- lo 1))
  (for _index (range lo (- hi 1))
    (bind _returnvalue (SortStrings|GreaterwithIndices (Utilities|Array|Get(acopy) In _index) (LocalVariables|GetPivot)))
    (if (not _returnvalue)
      (bind _result (Math|Integer|IncrementInt (LocalVariables|Geti))
        (:%20%20
          (Utilities|Array|Swap In _result _index)))))
  (bind _result_2 (Math|Integer|IncrementInt (LocalVariables|Geti))
    (:%20%20
      (Utilities|Array|Swap In _result_2 hi)
      (return (LocalVariables|Geti)))))

(fn QuickSortImpl
  (params (In :type Array%20of%20Strings) (lo :type Integer) (hi :type Integer))
  (if (not (or (>= lo hi) (< lo 0)))
    (bind _pivot_index (SortStrings|Partition In lo hi))
    (SortStrings|QuickSortImpl In lo (- _pivot_index 1))
    (SortStrings|QuickSortImpl In (+ _pivot_index 1) hi)))

(fn QuickSort
  (params (In :type Array%20of%20Strings))
  (SortStrings|QuickSortImpl In 0 (Utilities|Array|LastIndex In)))

(fn GreaterwithIndices
  (params (A :type String) (B :type String))
  (if (and (SortStrings|EndswithNumber A) (SortStrings|EndswithNumber B))
    (bind (_string _index) (SortStrings|SplitStringbyIndex A))
    (bind (_string_2 _index_2) (SortStrings|SplitStringbyIndex B))
    (if (Utilities|Enum|Equal(Enum) _string _string_2)
      (return (> _index _index_2))
      (else
        (bind _returnvalue (SortStrings|Greater _string _string_2))
        (return _returnvalue)))
    (else
      (bind _returnvalue_2 (SortStrings|Greater A B))
      (return _returnvalue_2))))

(fn ExtractIndex
  (params (String :type String))
  (bind _returnvalue (Utilities|String|Len String))
  (for _index (range 1 _returnvalue)
    (if (not (Math|Integer|InRange(Integer) (Utilities|String|GetCharacterasNumber String (- _returnvalue _index)) 48 57))
      (return (Math|Conversions|ToInteger(Byte) (Utilities|String|GetSubstring String (- _returnvalue _index) _index)))))
  (return (Math|Conversions|ToInteger(Byte) String)))

(fn SplitStringbyIndex
  (params (RawString :type String))
  (bind _returnvalue (Utilities|String|Len RawString))
  (for _index (range 1 _returnvalue)
    (if (not (Math|Integer|InRange(Integer) (Utilities|String|GetCharacterasNumber RawString (- _returnvalue _index)) 48 57))
      (return (Utilities|String|SelectString (Utilities|String|LeftChop (Utilities|String|GetSubstring RawString 0 (+ (- _returnvalue _index) 1)) 1) (Utilities|String|GetSubstring RawString 0 (+ (- _returnvalue _index) 1)) (Utilities|String|EndsWith (Utilities|String|GetSubstring RawString 0 (+ (- _returnvalue _index) 1)) " ")) (Math|Conversions|ToInteger(Byte) (Utilities|String|GetSubstring RawString (- _returnvalue _index) _index)))))
  (return "" (Math|Conversions|ToInteger(Byte) RawString)))

(fn UnifyName
  (params (SourceName :type String%20%28by%20ref%29) (ExistingNames :type Array%20of%20Strings))
  (Utilities|Set|AddItems (LocalVariables|GetCollection) ExistingNames)
  (if (Utilities|Set|Contains (LocalVariables|GetCollection) SourceName)
    (if (SortStrings|EndswithNumber SourceName)
      (bind _string (SortStrings|SplitStringbyIndex SourceName))
      (LocalVariables|SetBase _string)
      (else
        (LocalVariables|SetBase SourceName)))
    (for _index (range 0 (Utilities|Set|Length (LocalVariables|GetCollection)))
      (if (not (Utilities|Set|Contains (LocalVariables|GetCollection) (Utilities|String|Append (LocalVariables|GetBase) " " (Utilities|String|ToString(Integer) _index))))
        (|SetBy-RefVar SourceName (Utilities|String|Append (LocalVariables|GetBase) " " (Utilities|String|ToString(Integer) _index)))
        (return)))))

(fn GetAssetPath
  (params (AssetData :type Asset%20Data%20Structure%20%28by%20ref%29))
  (bind (_packagename _assetname) (Utilities|Struct|BreakAssetData AssetData))
  (return (Utilities|String|Append (Utilities|String|ToString(Name) _packagename) "." (Utilities|String|ToString(Name) _assetname))))

(fn CallProgressbar
  (params (PlayerController :type Player%20Controller%20Object%20Reference))
  (bind _foundwidgets (Widget|GetAllWidgetsOfClass PlayerController "/Game/QuietRuntimeEditor/Common/Widgets/WBP_Progressbar.WBP_Progressbar_C"))
  (if (Utilities|Array|IsValidIndex _foundwidgets)
    (return (Utilities|Array|Get(acopy) _foundwidgets))
    (else
      (bind _returnvalue (UserInterface|CreateWidget "/Game/QuietRuntimeEditor/Common/Widgets/WBP_Progressbar.WBP_Progressbar_C" PlayerController))
      (UserInterface|Viewport|AddtoViewport _returnvalue 100)
      (return _returnvalue))))