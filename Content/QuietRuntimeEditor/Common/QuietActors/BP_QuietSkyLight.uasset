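; BP_QuietSkyLight is a sky light actor for the Quiet runtime editor, with a Thumbnail that is hidden on BeginPlay.
; A looping one-second timer polls for the actor's QuietOutlinerComponent, then clears itself and binds to its selection-change notification.
; The Thumbnail mirrors that selection state, including an already active selection at bind time, and EnableDebugMode toggles its visibility.
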(event Custom|TryToBindToSelect
  (bind _treecomponent (CallFunction|GetQuietOutlinerComponent self))
  (Utilities|IsValid _treecomponent
    (:Is%20Valid
      (Utilities|Time|ClearandInvalidateTimerbyHandle (stale EventBeginPlay _returnvalue))
      (EventDispatchers|BindEventtoNotifyonSelectionStateChanged _treecomponent (delegate Custom|HandleOnSelectionStateChange))
      (if (Default|GetSelectionState _treecomponent)
        (Default|ChangeSelectionState (Variables|Default|GetThumbnail) true)))))

(event Custom|HandleOnSelectionStateChange
  (params (NewState :type Boolean))
  (Default|ChangeSelectionState (Variables|Default|GetThumbnail) NewState))

(event EventBeginPlay
  (Default|SetThumbnailVisibility (Variables|Default|GetThumbnail) false)
  (bind _returnvalue (Utilities|Time|SetTimerbyEvent (delegate Custom|TryToBindToSelect) 1.0 true)))

(event EventEnableDebugMode
  (params (Enable :type Boolean))
  (bind _output_get (Variables|Default|SetDebugVisibility Enable))
  (Default|SetThumbnailVisibility (Variables|Default|GetThumbnail) _output_get))

(fn ConstructionScript)