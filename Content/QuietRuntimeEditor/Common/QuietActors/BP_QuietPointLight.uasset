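; BP_QuietPointLight is a point light actor for the Quiet runtime editor, with a thumbnail and debug spheres showing attenuation and source radius.
; A looping timer waits for the actor's QuietOutlinerComponent, then binds selection changes to the thumbnail and debug spheres.
; EnableDebugMode toggles thumbnail visibility, and the spheres show only when selected in debug mode.
; Tick rescales the spheres when either radius changes while debug is on.
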(event Custom|TryToBindToSelect
  (bind _treecomponent (CallFunction|GetQuietOutlinerComponent self))
  (Utilities|IsValid _treecomponent
    (:Is%20Valid
      (Utilities|Time|ClearandInvalidateTimerbyHandle (stale EventBeginPlay _returnvalue))
      (EventDispatchers|BindEventtoNotifyonSelectionStateChanged _treecomponent (delegate Custom|HandleOnSelectionStateChanged))
      (if (Default|GetSelectionState _treecomponent)
        (Default|ChangeSelectionState (Variables|Default|GetThumbnail) true)))))

(event Custom|HandleOnSelectionStateChanged
  (params (NewState :type Boolean))
  (Default|ChangeSelectionState (Variables|Default|GetThumbnail) NewState)
  (if (Variables|Default|GetDebugVisibility)
    (CallFunction|SetDebugMeshVisibility NewState)))

(event EventBeginPlay
  (CallFunction|UpdateDebugMesh)
  (Variables|Default|SetRadius (Variables|/Script/Engine.LocalLightComponent|GetAttenuationRadius (Variables|Default|GetPointLightComponent)))
  (Variables|Default|SetSource%20Radius (Variables|/Script/Engine.PointLightComponent|GetSourceRadius (Variables|Default|GetPointLightComponent)))
  (Default|SetThumbnailVisibility (Variables|Default|GetThumbnail) (Variables|Default|GetDebugVisibility))
  (bind _returnvalue (Utilities|Time|SetTimerbyEvent (delegate Custom|TryToBindToSelect) 0.5 true)))

(event EventEnableDebugMode
  (params (Enable :type Boolean))
  (bind _output_get (Variables|Default|SetDebugVisibility Enable))
  (Default|SetThumbnailVisibility (Variables|Default|GetThumbnail) _output_get)
  (if (Variables|Default|GetDebugVisibility)
    (if (CallFunction|IsSelected)
      (CallFunction|SetDebugMeshVisibility true))
    (elif (CallFunction|IsSelected)
      (CallFunction|SetDebugMeshVisibility false))))

(event EventTick
  (params (DeltaSeconds :type Float%20%28single-precision%29))
  (if (Variables|Default|GetDebugVisibility)
    (if (or (not (Math|Float|NearlyEqual(Float) (Variables|Default|GetRadius) (Variables|/Script/Engine.LocalLightComponent|GetAttenuationRadius (Variables|Default|GetPointLightComponent)) 0.001)) (not (Math|Float|NearlyEqual(Float) (Variables|Default|GetSource%20Radius) (Variables|/Script/Engine.PointLightComponent|GetSourceRadius (Variables|Default|GetPointLightComponent)) 0.001)))
      (Variables|Default|SetRadius (Variables|/Script/Engine.LocalLightComponent|GetAttenuationRadius (Variables|Default|GetPointLightComponent)))
      (Variables|Default|SetSource%20Radius (Variables|/Script/Engine.PointLightComponent|GetSourceRadius (Variables|Default|GetPointLightComponent)))
      (CallFunction|UpdateDebugMesh))))

(fn ConstructionScript
  (CallFunction|UpdateDebugMesh))

(fn UpdateDebugMesh
  (Transformation|SetRelativeScale3D (Variables|Default|GetPointLightSphere) (Math|Conversions|ToVector(Float) (/ (Variables|/Script/Engine.LocalLightComponent|GetAttenuationRadius (Variables|Default|GetPointLightComponent)) 5e+01)))
  (Transformation|SetRelativeScale3D (Variables|Default|GetSourceRadiusMesh) (Math|Conversions|ToVector(Float) (/ (Variables|/Script/Engine.PointLightComponent|GetSourceRadius (Variables|Default|GetPointLightComponent)) 5e+01))))

(fn SetDebugMeshVisibility
  (params (NewState :type Boolean))
  (Rendering|SetVisibility (Variables|Default|GetPointLightSphere) NewState true))

(fn IsSelected
  (bind _treecomponent (CallFunction|GetQuietOutlinerComponent self))
  (Utilities|IsValid _treecomponent
    (:Is%20Valid
      (return (Default|GetSelectionState _treecomponent)))))