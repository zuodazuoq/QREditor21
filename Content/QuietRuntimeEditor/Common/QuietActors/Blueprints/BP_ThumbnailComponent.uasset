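; A mesh component for the runtime editor that shows a clickable-style thumbnail billboard in the world.
; On BeginPlay it creates a dynamic instance of M_Thumbnail with its texture, and selection changes toggle that material's Active parameter.
; While visible, it yaws toward the player camera each tick and scales by distance, FOV and view angle, clamped, to hold a steady screen size.
; Toggling visibility also switches query-only collision.
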(event Custom|ChangeSelectionState
  (params (NewState :type Boolean))
  (Rendering|Material|SetScalarParameterValue (Variables|Thumbnail|GetMaterial) "Active" (Math|Conversions|ToFloat(Boolean) NewState) :!class /Script/Engine.MaterialInstanceDynamic))

(event Custom|SetThumbnailVisibility
  (params (NewState :type Boolean))
  (Variables|Thumbnail|SetVisible NewState)
  (Development|SetHiddeninGame self (not (Variables|Thumbnail|GetVisible)) false)
  (Rendering|SetVisibility self (Variables|Thumbnail|GetVisible) false)
  (Collision|SetCollisionEnabled self (select (Variables|Thumbnail|GetVisible) "QueryOnly" "NoCollision")))

(event EventTick
  (params (DeltaSeconds :type Float%20%28single-precision%29))
  (if (Variables|Thumbnail|GetVisible)
    (CallFunction|AligntoCamera)
    (CallFunction|ScaleThumbnail)))

(event EventBeginPlay
  (CallFunction|SetThumbnailVisibility (Variables|Thumbnail|GetVisible))
  (bind _returnvalue (Rendering|Material|CreateDynamicMaterialInstance 0 "/Game/QuietRuntimeEditor/Common/QuietActors/Materials/M_Thumbnail.M_Thumbnail" "None" :!class /Script/Engine.PrimitiveComponent))
  (bind _output_get (Variables|Thumbnail|SetMaterial _returnvalue))
  (Rendering|Material|SetTextureParameterValue _output_get "Thumbnail" (Variables|Thumbnail|GetThumbnail)))

(fn ScaleThumbnail
  (bind _returnvalue (Game|GetPlayerCameraManager 0))
  (bind _self self)
  (bind _returnvalue_2 (Transformation|GetWorldLocation _self))
  (bind _transformcomponent (Variables|/Script/Engine.PlayerCameraManager|GetTransformComponent _returnvalue))
  (bind _returnvalue_3 (Transformation|GetWorldLocation _transformcomponent))
  (bind _returnvalue_4 (- _returnvalue_3 _returnvalue_2))
  (bind _returnvalue_5 (* _returnvalue_4 _returnvalue_4))
  (Transformation|SetWorldScale3D self (Math|Conversions|ToVector(Float) (Math|Float|Clamp(Float) (* (* (Math|Float|Sqrt (+ (.x _returnvalue_5) (.y _returnvalue_5) (.z _returnvalue_5))) (Camera|GetFOVAngle _returnvalue) (Math|Vector|DotProduct (Transformation|GetActorForwardVector _returnvalue) (Math|Rotator|GetRotationXVector (Math|Rotator|FindLookatRotation (Camera|GetCameraLocation _returnvalue) _returnvalue_2)))) 1e-05 (Variables|Thumbnail|GetScreenSize)) 0.0001 0.36))))

(fn AligntoCamera
  (Transformation|SetWorldRotation self (Math|Rotator|MakeRotator 9e+01 0.0 (+ (.yaw (Math|Rotator|FindLookatRotation (Transformation|GetWorldLocation self) (Camera|GetCameraLocation (Game|GetPlayerCameraManager 0)))) -9e+01)) false false))