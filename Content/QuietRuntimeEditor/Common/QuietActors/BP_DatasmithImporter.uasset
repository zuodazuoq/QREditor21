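; Runtime Datasmith importer actor for QuietRuntimeEditor that loads a scene from a saved path or file browser, replacing its attached actors.
; Tick-driven gate reports load progress, while a delayed check warns if the external file is missing.
; On completion it calls content restore (its JSON deserialization is unwired), renames itself uniquely and registers with the tree manager's outliner.
; A debug-toggleable thumbnail mirrors outliner selection, bound by timer polling.
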(event Custom|TryToBindToSelect
  (bind _treecomponent (CallFunction|GetQuietOutlinerComponent self))
  (Utilities|IsValid _treecomponent
    (:Is%20Valid
      (Utilities|Time|ClearandInvalidateTimerbyHandle (stale EventBeginPlay _returnvalue))
      (EventDispatchers|BindEventtoNotifyonSelectionStateChanged _treecomponent (delegate Custom|HandleOnSelectionStateChanged))
      (if (Default|GetSelectionState _treecomponent)
        (Default|ChangeSelectionState (Variables|Default|GetThumbnail) true)))))

(event Custom|HandleOnSelectionStateChanged
  (params (NewState :type Boolean))
  (Default|ChangeSelectionState (Variables|Default|GetThumbnail) NewState))

(event Custom|BrowseFile
  (bind _returnvalue (Class|DatasmithRuntimeLibrary|LoadFilefromExplorer self))
  (if _returnvalue
    (CallFunction|Clear)
    (bind _progressbar (CallFunction|CallProgressbar (Game|GetPlayerController 0)))
    (Default|Subscribe _progressbar self)
    (Utilities|FlowControl|Sequence
      (:then_0
        (Utilities|FlowControl|Delay 1e+01)
        (Utilities|FlowControl|Gate true :!label _label
          (:Exit
            (bind _returnvalue_2 (Class|BlueprintFileUtilsBPLibrary|FileExists (Variables|Default|GetExternalFile)))
            (if (not _returnvalue_2)
              (Utilities|IsValid _progressbar
                (:Is%20Valid
                  (Default|End _progressbar))
                (:Is%20Not%20Valid
                  _))
              (CallFunction|CallWarningDialogSimple (Game|GetPlayerController 0) "Try again, please")))))
      (:then_1
        (goto _label Open))
      (:then_2
        (Utilities|FlowControl|Gate true) ; enters at Open
      ))))

(event Custom|Import
  (bind _returnvalue (Class|BlueprintFileUtilsBPLibrary|FileExists (Variables|DatasmithImporter|GetFile)))
  (if _returnvalue
    (bind _returnvalue_2 (Class|DatasmithRuntimeActor|LoadFile (Variables|DatasmithImporter|GetFile)))
    (if _returnvalue_2
      (CallFunction|Clear)
      (bind _progressbar (CallFunction|CallProgressbar (Game|GetPlayerController 0)))
      (Default|Subscribe _progressbar self)
      (Utilities|FlowControl|Sequence
        (:then_0
          (Utilities|FlowControl|Delay 1e+01)
          (Utilities|FlowControl|Gate true :!label _label
            (:Exit
              (bind _returnvalue_3 (Class|BlueprintFileUtilsBPLibrary|FileExists (Variables|Default|GetExternalFile)))
              (if (not _returnvalue_3)
                (Utilities|IsValid _progressbar
                  (:Is%20Valid
                    (Default|End _progressbar))
                  (:Is%20Not%20Valid
                    _))
                (CallFunction|CallWarningDialogSimple (Game|GetPlayerController 0) "Try again, please")))))
        (:then_1
          (goto _label Open))
        (:then_2
          (Utilities|FlowControl|Gate true) ; enters at Open
        )))))

(event Custom|RestoreContent
  (params (ContentJson :type Json%20Object%20Wrapper%20Structure))
  (Utilities|RestoreContentMacro ContentJson) ; enters at Request
)

(event EventBeginPlay
  (Default|SetThumbnailVisibility (Variables|Default|GetThumbnail) (Variables|Default|GetDebugVisibility))
  (bind _returnvalue (Utilities|Time|SetTimerbyEvent (delegate Custom|TryToBindToSelect) 1.0 true)))

(event EventEnableDebugMode
  (params (Enable :type Boolean))
  (bind _output_get (Variables|Default|SetDebugVisibility Enable))
  (Default|SetThumbnailVisibility (Variables|Default|GetThumbnail) _output_get))

(event EventTick
  (params (DeltaSeconds :type Float%20%28single-precision%29))
  (Utilities|FlowControl|Gate true :!label _label
    (:Exit
      (Utilities|IsValid (stale Custom|BrowseFile _progressbar)
        (:Is%20Valid
          (Default|Progress (stale Custom|BrowseFile _progressbar) self (Math|Float|Clamp(Float) (Variables|Default|GetProgress))))
        (:Is%20Not%20Valid
          _))
      (if (and (>= (Variables|Default|GetProgress) 0.5) (not (Variables|Default|GetbBuilding)))
        (Utilities|FlowControl|Sequence
          (:then_0
            (Default|Progress (stale Custom|BrowseFile _progressbar) self 1.0)
            (Utilities|FlowControl|DelayUntilNextTick)
            (Utilities|RestoreContentMacro (stale Custom|RestoreContent ContentJson))
            (Variables|DatasmithImporter|SetFile (Variables|Default|GetExternalFile))
            (bind _returnvalue (Actor|GetActorOfClass "/Game/QuietRuntimeEditor/Blueprints/BP_QuietTreeManager.BP_QuietTreeManager_C"))
            (CallFunction|RenameImporter _returnvalue)
            (Default|ThrowActor (Variables|/Game/QuietRuntimeEditor/Blueprints/BP_QuietTreeManager.BP_QuietTreeManager_C|GetRouter _returnvalue) "(TagName=\"Manager\")" "(TagName=\"Outliner.RegisterAttachment\")" self)
            (Utilities|IsValid (stale Custom|BrowseFile _progressbar)
              (:Is%20Valid
                (Default|RemoveSubscriber (stale Custom|BrowseFile _progressbar) self))))
          (:then_1
            (Utilities|FlowControl|Gate true) ; enters at Close
          )
          (:then_2
            (goto _label Close)))))))

(fn ConstructionScript)

(fn RestoreContentImpl
  (params (Json :type Json%20Object%20Wrapper%20Structure)))

(fn RenameImporter
  (params (Manager :type BP%20Quiet%20Tree%20Manager%20Object%20Reference))
  (LocalVariables|SetRawName (Variables|Default|GetLoadedScene))
  (bind _values (Utilities|Map|Values (Variables|/Game/QuietRuntimeEditor/Blueprints/BP_QuietTreeManager.BP_QuietTreeManager_C|GetFlat%20Actors%20Map Manager)))
  (bind _names (CallFunction|CollectActorNames _values))
  (CallFunction|UnifyName (LocalVariables|GetRawName) _names)
  (bind _treecomponent (CallFunction|AcquireOutlinerComponent self))
  (Default|Rename _treecomponent (LocalVariables|GetRawName) false))

(fn Clear
  (bind _arrayelement (Utilities|Array|ReverseforEachLoop (Actor|GetAttachedActors true true))
    (:LoopBody
      (Actor|DestroyActor _arrayelement))))