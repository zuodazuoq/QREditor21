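; Base transform gizmo for runtime editing of selected actors; TransformTick and TransformFromOut are empty stubs here.
; Each tick it traces under the cursor, highlights the hovered handle, maps it to an axis and keeps constant screen size, flipping axes toward the camera for one type.
; Mouse drags or external events start and end transforms, with state and settings exchanged through owner messages.
; Setup destroys other gizmos, leaving one.
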(event EventBeginPlay
  ;[0.01473 0.02728 0.07812] BEGIN PLAY - SETUP Gizmo
  (Gizmo|Setup|Setup))

(event EventTick
  (params (DeltaSeconds :type Float%20%28single-precision%29))
  (bind _returnvalue (Game|GetPlayerController 0))
  (bind (_deltax _deltay) (Class|PlayerController|GetInputMouseDelta _returnvalue))
  ;[0.08333 0.03319 0.03125] EVENT TICK - Mouse Over Gizmo and Transformation Tick
  (Gizmo|Actions|MouseOver)
  (Gizmo|Tick|FixSizeonViewport)
  (if (not (Variables|Gizmo|GetTransformingOuter))
    (if (Variables|Gizmo|GetTransforming)
      (Gizmo|Tick|TransformTick)
      (if (> (Math|Float|Max(Float) (Math|Float|Absolute(Float) _deltax) (Math|Float|Absolute(Float) _deltay)) 1e-06)
        (Utilities|FlowControl|DoOnce false
          (:Completed
            (Class|BIGizmoBlueprintInterface|NotifyonFirstChanged(Message) (Components|GetOwner))))))))

(event EventEndPlay
  (params (EndPlayReason :type EEndPlayReason%20Enum :default "Destroyed"))
  ;[0.01439 0.03693 0.09896] END PLAY
  (Utilities|IsValid (Variables|Default|GetHit%20Component)
    (:Is%20Valid
      (Gizmo|Actions|DeselectComp (Variables|Default|GetHit%20Component)))))

(event EventSendTransformfromOut
  (params (Value :type Float%20%28double-precision%29) (AccumulatedDelta :type Float%20%28double-precision%29) (TickDelta :type Float%20%28double-precision%29))
  ;[0 0 0] Handle external events (From Widget or Inputs)
  (Gizmo|Tick|TransformfromOut Value AccumulatedDelta TickDelta))

(event EventSendEndTransformfromOut
  ;[0 0 0] Handle external events (From Widget or Inputs)
  (Gizmo|Actions|DeactivatefromOut))

(event EventSendStartTransformfromOut
  (params (Axis :type E_TransformAxes%20Enum :default "NewEnumerator0"))
  ;[0 0 0] Handle external events (From Widget or Inputs)
  (Gizmo|Actions|ActivatefromOut Axis))

(event EventStartTransformfromMouse
  (Gizmo|Actions|OnMouseClick))

(event EventEndTransformfromMouse
  (Gizmo|Actions|OnMouseRelease))

(event Input|MouseEvents|LeftMouseButton
  (params (Key :type Key%20Structure))
  ;[0 0 0] Mouse Click
  (:Pressed
    (bind _state (Gizmo|Actions|MouseOver))
    (if _state
      (Gizmo|Actions|OnMouseClick)))
  (:Released
    (if (Variables|Gizmo|GetTransforming)
      (Gizmo|Actions|OnMouseRelease)
      (Utilities|FlowControl|DoOnce false) ; enters at Reset
    )))

(fn ConstructionScript)

(fn Setup
  (Input|EnableInput (Game|GetPlayerController 0))
  (Gizmo|Setup|DestroyOldGizmo))

(fn MouseOver
  (if (not (Variables|Gizmo|GetTransforming))
    (if (not (Variables|Gizmo|GetTransformingOuter))
      (Utilities|FlowControl|Sequence
        (:then_0
          (bind _hitcomponent (Utilities|Trace)
            (:true
              (Utilities|IsValid (Variables|Default|GetHit%20Component)
                (:Is%20Valid
                  (if (not (== _hitcomponent (Variables|Default|GetHit%20Component)))
                    (Gizmo|Actions|DeselectComp (Variables|Default|GetHit%20Component))
                    (Gizmo|Actions|SelectComp _hitcomponent)))
                (:Is%20Not%20Valid
                  (Gizmo|Actions|SelectComp _hitcomponent))))
            (:false
              (Utilities|IsValid (Variables|Default|GetHit%20Component)
                (:Is%20Valid
                  (Gizmo|Actions|DeselectComp (Variables|Default|GetHit%20Component))
                  (Variables|Default|SetHit%20Component 0))))))
        (:then_1
          (return (Utilities|IsValid (Variables|Default|GetHit%20Component)))))
      (else
        (return (Utilities|IsValid (Variables|Default|GetHit%20Component)))))))

(fn DeselectComp
  (params (Component :type Primitive%20Component%20Object%20Reference))
  (Gizmo|Actions|ActivateMaterial Component false)
  (Gizmo|Actions|ChangeMouseCursor "Default")
  (Gizmo|Actions|BlockMousewhenUseGizmo false))

(fn SelectComp
  (params (Component :type Primitive%20Component%20Object%20Reference))
  (bind _output_get (Variables|Default|SetHit%20Component Component))
  (Gizmo|Actions|ActivateMaterial _output_get true)
  (Gizmo|Actions|ChangeMouseCursor "CardinalCross")
  (Variables|Gizmo|SetActiveAxis (.Value (Utilities|Map|Find (Variables|Gizmo|GetTransformsMap) (Variables|Default|GetHit%20Component))))
  (Gizmo|Actions|BlockMousewhenUseGizmo true))

(fn ChangeMouseCursor
  (params (NewMouseCursor :type EMouseCursor%20Enum :default "None"))
  (bind _returnvalue (Game|GetPlayerController 0))
  (Utilities|IsValid _returnvalue
    (:Is%20Valid
      (Variables|/Script/Engine.PlayerController|SetCurrentMouseCursor _returnvalue NewMouseCursor))))

(fn ActivateMaterial
  (params (Component :type Primitive%20Component%20Object%20Reference) (Activate :type Boolean))
  (bind _returnvalue (Math|Conversions|ToFloat(Boolean) Activate))
  (bind _asstatic_mesh_component (Utilities|Casting|CastToStaticMeshComponent Component))
  (Rendering|Material|SetScalarParameterValueonMaterials _asstatic_mesh_component "Active" _returnvalue)
  (for _array_element (Components|GetChildrenComponents _asstatic_mesh_component false)
    (bind _asstatic_mesh_component_2 (Utilities|Casting|CastToStaticMeshComponent _array_element))
    (Rendering|Material|SetScalarParameterValueonMaterials _asstatic_mesh_component_2 "Active" _returnvalue)))

(fn GetActiveAxis
  (return (.Value (Utilities|Map|Find (Variables|Gizmo|GetTransformsMap) (Variables|Default|GetHit%20Component)))))

(fn IntersectwithAxisPlane
  (params (Normal :type Vector) (Location :type Vector%20%28by%20ref%29) (Direction :type Vector) (Invert :type Boolean) (Point :type Vector))
  (bind _returnvalue (Class|KismetMathLibrary|MakePlanefromPointandNormal Point Normal))
  (bind _tracedistance (Variables|Gizmo|GetTraceDistance))
  (bind _returnvalue_2 (* _tracedistance -1.0))
  (bind _returnvalue_3 (Math|Float|SelectFloat _returnvalue_2 _tracedistance Invert))
  (bind _returnvalue_4 (* Direction _returnvalue_3))
  (bind _returnvalue_5 (+ Location _returnvalue_4))
  (bind (_t _intersection _returnvalue_6) (Class|KismetMathLibrary|LinePlaneIntersection Location _returnvalue_5 _returnvalue))
  (return _intersection _returnvalue_6))

(fn TransformTick)

(fn GetAxisVectors
  (params (FirstAxis :type Vector) (SecondAxis :type Vector))
  (bind _returnvalue (Game|GetPlayerCameraManager 0))
  (bind _returnvalue_2 (Transformation|GetActorForwardVector _returnvalue))
  (if (> (Math|Float|Absolute(Float) (Math|Vector|DotProduct FirstAxis _returnvalue_2)) (Math|Float|Absolute(Float) (Math|Vector|DotProduct SecondAxis _returnvalue_2)))
    (return FirstAxis SecondAxis)
    (else
      (return SecondAxis FirstAxis))))

(fn SortAxis
  (bind _returnvalue (Transformation|GetActorUpVector))
  (bind _returnvalue_2 (Transformation|GetActorRightVector))
  (bind _returnvalue_3 (Transformation|GetActorForwardVector))
  (switch Utilities|FlowControl|Switch|SwitchonE_TransformAxes (Variables|Gizmo|GetActiveAxis)
    (:NewEnumerator0
      (return _returnvalue_3 _returnvalue _returnvalue_2))
    (:NewEnumerator1
      (return _returnvalue_2 _returnvalue _returnvalue_3))
    (:NewEnumerator2
      (return _returnvalue _returnvalue_2 _returnvalue_3))))

(fn ProjectPlaneIntersectiontoAxis
  (params (PlaneIntersection :type Vector) (Axis :type Vector) (Point :type Vector))
  (bind (_intersection _success) (Gizmo|Axis|IntersectwithAxisPlane Axis PlaneIntersection Axis false Point))
  (if _success
    (return _intersection)
    (else
      (bind _intersection_2 (Gizmo|Axis|IntersectwithAxisPlane Axis PlaneIntersection Axis true Point))
      (return _intersection_2))))

(fn FixSizeonViewport
  (bind _returnvalue (Game|GetPlayerCameraManager 0))
  (bind _returnvalue_2 (Transformation|GetActorLocation))
  (bind _scene (Variables|Default|GetScene))
  (bind _scene_2 (Variables|Default|GetScene))
  (bind _returnvalue_3 (Transformation|GetWorldScale _scene))
  (bind _returnvalue_4 (Transformation|GetWorldScale _scene_2))
  (bind _transformcomponent (Variables|/Script/Engine.PlayerCameraManager|GetTransformComponent _returnvalue))
  (bind _returnvalue_5 (Transformation|GetWorldLocation _transformcomponent))
  (bind _returnvalue_6 (- _returnvalue_5 _returnvalue_2))
  (bind _returnvalue_7 (* _returnvalue_6 _returnvalue_6))
  (Transformation|SetWorldScale3D (Variables|Default|GetScene) (* (Math|Conversions|ToVector(Float) (* (* (Math|Float|Sqrt (+ (.x _returnvalue_7) (.y _returnvalue_7) (.z _returnvalue_7))) (Camera|GetFOVAngle _returnvalue) (Math|Vector|DotProduct (Transformation|GetActorForwardVector _returnvalue) (Math|Rotator|GetRotationXVector (Math|Rotator|FindLookatRotation (Transformation|GetActorLocation _returnvalue) (Transformation|GetActorLocation))))) 1e-05 (Variables|Gizmo|GetScreenSize))) (Gizmo|Tick|GetSceneCompVectorSign)))
  (if (Utilities|Enum|Equal(Enum) (Variables|Gizmo|GetType) "NewEnumerator2")
    (Utilities|FlowControl|Sequence
      (:then_0
        (bind (_flip _invertedscale) (Gizmo|Tick|ForwardtoCamera (Math|Vector|GetForwardVector _scene_2) (.x _returnvalue_4)))
        (if _flip
          (Transformation|SetWorldScale3D (Variables|Default|GetScene) (Math|Vector|MakeVector _invertedscale (.y _returnvalue_3) (.z _returnvalue_3)))))
      (:then_1
        (bind (_flip_2 _invertedscale_2) (Gizmo|Tick|ForwardtoCamera (Math|Vector|GetRightVector _scene_2) (.y _returnvalue_4)))
        (if _flip_2
          (Transformation|SetWorldScale3D (Variables|Default|GetScene) (Math|Vector|MakeVector (.x _returnvalue_3) _invertedscale_2 (.z _returnvalue_3)))))
      (:then_2
        (bind (_flip_3 _invertedscale_3) (Gizmo|Tick|ForwardtoCamera (Math|Vector|GetUpVector _scene_2) (.z _returnvalue_4)))
        (if _flip_3
          (Transformation|SetWorldScale3D (Variables|Default|GetScene) (Math|Vector|MakeVector (.x _returnvalue_3) (.y _returnvalue_3) _invertedscale_3)))))))

(fn HandleMouseClick
  (Class|BIGizmoBlueprintInterface|NotifyStart(Message) (Components|GetOwner))
  (CallFunction|NotifyStart)
  (for _array_element (Selection|GetControlledActors)
    (Utilities|Array|Add (Variables|Default|GetStartLocations) (Transformation|GetActorLocation _array_element))))

(fn HandleMouseRelease
  (Utilities|Array|Clear (Variables|Default|GetStartLocations))
  (Class|BIGizmoBlueprintInterface|SendEndTransformfromOut(Message) (Components|GetOwner))
  (Class|BIGizmoBlueprintInterface|NotifyEnd(Message) (Components|GetOwner))
  (CallFunction|NotifyEnd))

(fn GetType
  (return (Variables|Gizmo|GetType)))

(fn BlockMousewhenUseGizmo
  (params (Block :type Boolean))
  (Utilities|IsValid (Game|GetPlayerController 0)
    (:Is%20Valid
      (Utilities|FlowControl|Sequence
        (:then_0
          (if (Variables|PlayerController|GetProjectClickEvents)
            (Variables|/Script/Engine.PlayerController|SetbEnableClickEvents (Game|GetPlayerController 0) (not Block))))
        (:then_1
          (if (Variables|PlayerController|GetProjectOverEvents)
            (Variables|/Script/Engine.PlayerController|SetbEnableMouseOverEvents (Game|GetPlayerController 0) (not Block))))))))

(fn GetSceneCompVectorSign
  (bind _scene (Variables|Default|GetScene))
  (bind _returnvalue (Transformation|GetWorldScale _scene))
  (return (Math|Vector|MakeVector (Math|Float|Sign(Float) (.x _returnvalue)) (Math|Float|Sign(Float) (.y _returnvalue)) (Math|Float|Sign(Float) (.z _returnvalue)))))

(fn ForwardtoCamera
  (params (DirectionVector :type Vector) (ScaleValue :type Float%20%28double-precision%29))
  (return (!= (Math|Float|Sign(Float) ScaleValue) (Math|Float|Sign(Float) (Math|Vector|DotProduct DirectionVector (Math|Rotator|GetRotationXVector (Math|Rotator|FindLookatRotation (Transformation|GetActorLocation) (Transformation|GetActorLocation (Game|GetPlayerCameraManager 0))))))) (* ScaleValue -1.0)))

(fn GetSnap
  (bind _state (Class|BIGizmoBlueprintInterface|GetDeltaStatebyType(Message) (Components|GetOwner)))
  (return _state))

(fn GetRelative
  (bind _state (Class|BIGizmoBlueprintInterface|GetRelativebyType(Message) (Components|GetOwner)))
  (return _state))

(fn ReturnTransformVector
  (params (NewVector :type Vector))
  (Class|BIGizmoBlueprintInterface|SendTransformVector(Message) (Components|GetOwner) NewVector))

(fn DestroyOldGizmo
  (bind _outactors (Actor|GetAllActorsOfClass "BP_QuietGizmo_C"))
  (for _array_element _outactors
    (if (!= _array_element self)
      (Actor|DestroyActor _array_element))))

(fn SetupMaterials
  (for _array_element (Actor|GetComponentsByClass "/Script/Engine.StaticMeshComponent")
    (for (_array_element_2 _array_index) (Rendering|Material|GetMaterials _array_element)
      (Rendering|Material|CreateDynamicMaterialInstance _array_element _array_index _array_element_2 "None" :!class /Script/Engine.PrimitiveComponent))))

(fn SetupPlayerController
  (bind _returnvalue (Game|GetPlayerController 0))
  (Variables|PlayerController|SetProjectClickEvents (Variables|/Script/Engine.PlayerController|GetbEnableClickEvents _returnvalue))
  (Variables|PlayerController|SetProjectOverEvents (Variables|/Script/Engine.PlayerController|GetbEnableMouseOverEvents _returnvalue)))

(fn GetSnapValue
  (bind _value (Class|BIGizmoBlueprintInterface|GetDeltaValuebyType(Message) (Components|GetOwner)))
  (return _value))

(fn GetPivotCenter
  (bind _useselectioncenter (Class|BIGizmoBlueprintInterface|GetPivotLocation(Message) (Components|GetOwner)))
  (return _useselectioncenter))

(fn GetFirstControlledActor
  (return (Utilities|Array|Get(acopy) (Variables|Default|GetSelection))))

(fn GetControlledActors
  (return (Variables|Default|GetSelection)))

(fn OnMouseClick
  (Utilities|IsValid (Variables|Default|GetHit%20Component)
    (:Is%20Valid
      (Variables|Gizmo|SetTransforming true)
      (Input|DisableInput (Game|Player|GetPlayerPawn 0) (Game|GetPlayerController 0))
      (Gizmo|Actions|HandleMouseClick))))

(fn OnMouseRelease
  (Gizmo|Actions|HandleMouseRelease)
  (Variables|Gizmo|SetTransforming false)
  (Input|EnableInput (Game|Player|GetPlayerPawn 0) (Game|GetPlayerController 0)))

(fn TransformfromOut
  (params (Value :type Float%20%28double-precision%29) (AccumulatedDelta :type Float%20%28double-precision%29) (TickDelta :type Float%20%28double-precision%29)))

(fn ActivatefromOut
  (params (Axis :type E_TransformAxes%20Enum :default "NewEnumerator0"))
  (bind _transformsmap (Variables|Gizmo|GetTransformsMap))
  (Variables|Gizmo|SetTransformingOuter true)
  (bind _mode (Class|BIGizmoBlueprintInterface|GetTransformMode(Message) (Components|GetOwner)))
  (bind _state (Class|BIGizmoBlueprintInterface|GetScaleUniformState(Message) (Components|GetOwner)))
  (Utilities|FlowControl|Sequence
    (:then_0
      (Utilities|IsValid (Variables|Default|GetHit%20Component)
        (:Is%20Valid
          (Gizmo|Actions|DeselectComp (Variables|Default|GetHit%20Component)))))
    (:then_1
      (bind _output_get (Variables|Gizmo|SetActiveAxis (select (and (Utilities|Enum|Equal(Enum) _mode "NewEnumerator3") _state) "NewEnumerator6" Axis)))
      (bind _values (Utilities|Map|Values _transformsmap))
      (bind _keys (Utilities|Map|Keys _transformsmap))
      (bind _output_get_2 (Variables|Default|SetHit%20Component (Utilities|Array|Get(acopy) _keys (Utilities|Array|FindItem _values _output_get))))
      (Gizmo|Actions|ActivateMaterial _output_get_2 true)
      (Class|BIGizmoBlueprintInterface|NotifyStart(Message) (Components|GetOwner)))))

(fn DeactivatefromOut
  (Gizmo|Actions|ActivateMaterial (Variables|Default|GetHit%20Component) false)
  (Variables|Default|SetHit%20Component 0)
  (Variables|Gizmo|SetTransformingOuter false)
  (Utilities|Array|Clear (Variables|Default|GetStartLocations))
  (Class|BIGizmoBlueprintInterface|NotifyEnd(Message) (Components|GetOwner)))

(fn IsHovered
  (return (Utilities|IsValid (Variables|Default|GetHit%20Component))))

(fn GetAlignState
  (return false))

(fn GetDeltaStatebyType
  (return false))

(fn GetDeltaValuebyType
  (return 0.0))

(fn GetMainSelectedActor
  (return 0))

(fn GetPivotLocation
  (return (Gizmo|Getters|GetPivotCenter)))

(fn GetRelativebyType
  (return (Gizmo|Getters|GetRelative)))

(fn GetScaleUniformState
  (return false))

(fn GetSelectedActors
  (return 0))

(fn GetTransformMode
  (return "NewEnumerator0"))

(fn GizmoOverState
  (bind _state (Gizmo|Actions|MouseOver))
  (return _state))