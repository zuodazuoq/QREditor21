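; Rotation gizmo for the runtime editor that rotates controlled actors around X, Y or Z by mouse drag or externally supplied deltas.
; Cursor rays hit the axis plane; projection onto the first-click tangent yields an optionally snapped angle, shown by disc segment and arrow.
; Angle deltas rotate actors locally or in world space, with pivot-center repositioning, routed through owner messages when replicated.
; A screen ring faces the camera every tick.
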(event EventBeginPlay
  (|CallParentFunction)
  (Rendering|Material|SetScalarParameterValueonMaterials (Variables|Default|GetSmallArrow_X) "Opacity" 0.3))

(event EventTick
  (params (DeltaSeconds :type Float%20%28single-precision%29))
  (|CallParentFunction DeltaSeconds)
  (CallFunction|ScreenAlign))

(fn ConstructionScript
  (|CallParentFunction))

(fn ScreenAlign
  (bind _returnvalue (Game|GetPlayerCameraManager 0))
  (bind _returnvalue_2 (Transformation|GetActorLocation))
  (bind _returnvalue_3 (Transformation|GetActorLocation _returnvalue))
  (bind _returnvalue_4 (Math|Rotator|FindLookatRotation _returnvalue_2 _returnvalue_3))
  (Transformation|SetWorldRotation (Variables|Default|GetRotate_Screen) (Math|Rotator|MakeRotator (.roll _returnvalue_4) (+ (.pitch _returnvalue_4) 9e+01) (.yaw _returnvalue_4)) false false))

(fn Setup
  (bind _transformsmap (Variables|Default|GetTransformsMap))
  (|CallParentFunction)
  (Utilities|Map|Add _transformsmap (Variables|Default|GetRotate_X) "NewEnumerator0")
  (Utilities|Map|Add _transformsmap (Variables|Default|GetRotate_Y) "NewEnumerator1")
  (Utilities|Map|Add _transformsmap (Variables|Default|GetRotate_Z) "NewEnumerator2"))

(fn TransformTick
  (bind _returnvalue (Game|GetPlayerController 0))
  (bind (_worldlocation _worlddirection) (Game|Player|ConvertMouseLocationToWorldSpace _returnvalue))
  (|CallParentFunction)
  (bind _active (CallFunction|SortAxis))
  (bind _intersection (CallFunction|IntersectwithAxisPlane _active _worldlocation _worlddirection false (Transformation|GetActorLocation)))
  (bind _tangent (CallFunction|GetTangentVector _active (Variables|Default|GetFirstClickLocation)))
  (bind _success (CallFunction|IntersectwithAxisPlane _tangent (Variables|Default|GetFirstClickLocation) _tangent false _intersection))
  (bind _angle (CallFunction|GetRawAngle _tangent _success _intersection (Variables|Default|GetFirstClickLocation)))
  (Rotation|SetDiscSegment _angle)
  (CallFunction|SetArrowDirection _angle _success)
  (bind (_discrotator _actorrotator) (CallFunction|MakeRotatorsbyActiveAxis (- _angle (Variables|Default|GetLastAngle))))
  (if (CallFunction|GetRelative)
    (Transformation|AddActorLocalRotation _actorrotator false false))
  (for (_array_element _array_index) (CallFunction|GetControlledActors)
    (CallFunction|RotateActor _actorrotator _array_element _array_index _angle))
  (Variables|Default|SetLastAngle _angle)
  (Rotation|RotateCircle _discrotator)
  (bind _actorrotator_2 (CallFunction|MakeRotatorsbyActiveAxis _angle))
  (CallFunction|ReturnTransformVector (Math|Vector|MakeVector (.roll _actorrotator_2) (.pitch _actorrotator_2) (.yaw _actorrotator_2))))

(fn HandleMouseClick
  (bind _returnvalue (Game|GetPlayerController 0))
  (bind _scene (Variables|Default|GetScene))
  (bind (_worldlocation _worlddirection) (Game|Player|ConvertMouseLocationToWorldSpace _returnvalue))
  (bind _relativescale3d (Variables|/Script/Engine.SceneComponent|GetRelativeScale3D _scene))
  (|CallParentFunction)
  (Utilities|FlowControl|Sequence
    (:then_0
      (Utilities|Array|Clear (Variables|Default|GetInitialLocation))
      (for _array_element (CallFunction|GetControlledActors)
        (bind _state (Class|BIGizmoBlueprintInterface|GetRelativebyType(Message) (Components|GetOwner)))
        (if _state
          (Utilities|Array|Add (Variables|Default|GetInitialLocation) (.Origin (Collision|GetActorBounds _array_element false false)))
          (else
            (Utilities|Array|Add (Variables|Default|GetInitialLocation) (Transformation|GetActorLocation _array_element))))))
    (:then_1
      (bind _active (CallFunction|SortAxis))
      (bind _intersection (CallFunction|IntersectwithAxisPlane _active _worldlocation _worlddirection false (Transformation|GetActorLocation)))
      (Variables|Default|SetFirstClickLocation (+ (Transformation|GetActorLocation) (* (Math|Rotator|GetRotationXVector (Math|Rotator|FindLookatRotation (Transformation|GetActorLocation) _intersection)) (* (Utilities|Select :Index (CallFunction|GetActiveAxis) :NewEnumerator0 (.x _relativescale3d) :NewEnumerator1 (.y _relativescale3d) :NewEnumerator2 (.z _relativescale3d) :NewEnumerator3 0.0 :NewEnumerator4 0.0 :NewEnumerator5 0.0 :NewEnumerator6 0.0) 15.0))))
      (bind (_success _disc) (CallFunction|GetActiveDisc))
      (if _success
        (Transformation|SetWorldRotation _disc (Math|Rotator|FindLookatRotation (Transformation|GetWorldLocation _disc) (Variables|Default|GetFirstClickLocation)) false false)
        (Transformation|SetRelativeRotation _disc (Math|Rotator|MakeRotator 0.0 0.0 (.yaw (Variables|/Script/Engine.SceneComponent|GetRelativeRotation _disc))) false false)))))

(fn MakeRotatorsbyActiveAxis
  (params (Angle :type Float%20%28double-precision%29))
  (bind _returnvalue (Math|Rotator|MakeRotator 0.0 0.0 Angle))
  (bind _returnvalue_2 (Class|KismetMathLibrary|NegateRotator _returnvalue))
  (switch Utilities|FlowControl|Switch|SwitchonE_TransformAxes (CallFunction|GetActiveAxis)
    (:NewEnumerator0
      (return _returnvalue_2 (Math|Rotator|MakeRotator Angle 0.0 0.0)))
    (:NewEnumerator1
      (return _returnvalue (Math|Rotator|MakeRotator 0.0 Angle 0.0)))
    (:NewEnumerator2
      (return _returnvalue_2 (Math|Rotator|MakeRotator 0.0 0.0 Angle)))))

(fn HandleMouseRelease
  (|CallParentFunction)
  (Variables|Default|SetLastAngle 0.0)
  (bind (_success _disc) (CallFunction|GetActiveDisc))
  (if _success
    (Rendering|Material|SetScalarParameterValueonMaterials _disc "Angle" 0.0)
    (Transformation|SetRelativeScale3D (Components|GetChildComponent _disc 0) "0, 0, 0")))

(fn GetActiveDisc
  (bind _hit_component (Variables|Default|GetHit%20Component))
  (Utilities|IsValid _hit_component
    (:Is%20Valid
      (bind _asstatic_mesh_component (Utilities|Casting|CastToStaticMeshComponent (Components|GetChildComponent _hit_component 0))
        (:then
          (return true _asstatic_mesh_component))
        (:CastFailed
          _)))
    (:Is%20Not%20Valid
      _))
  (return false 0))

(fn SetDiscSegment
  (params (RawAngle :type Float%20%28double-precision%29))
  (bind (_success _disc) (CallFunction|GetActiveDisc))
  (if _success
    (bind _output_get (LocalVariables|SetResultAngle RawAngle))
    (Rendering|Material|SetScalarParameterValueonMaterials _disc "Angle" (Math|Float|SelectFloat (* _output_get -1.0) _output_get (Utilities|Enum|Equal(Enum) (CallFunction|GetActiveAxis) "NewEnumerator1")))))

(fn RotateCircle
  (params (DiscRotator :type Rotator))
  (bind (_success _disc) (CallFunction|GetActiveDisc))
  (if _success
    (if (CallFunction|GetRelative)
      (Transformation|AddRelativeRotation _disc DiscRotator false false))))

(fn ApplyDelta
  (params (FullAngle :type Float%20%28double-precision%29))
  (bind _snapvalue (CallFunction|GetSnapValue))
  (bind _returnvalue (Math|Float|Division(WholeandRemainder) FullAngle _snapvalue))
  (if (!= (Variables|Default|GetCurrentSegment) _returnvalue)
    (bind _output_get (Variables|Default|SetCurrentSegment _returnvalue))
    (return (* _output_get (CallFunction|GetSnapValue)) true)
    (else
      (return (* (Variables|Default|GetCurrentSegment) (CallFunction|GetSnapValue)) false))))

(fn GetTangentVector
  (params (ActiveAxis :type Vector) (FirctClick :type Vector))
  (bind _returnvalue (Transformation|GetActorLocation))
  (bind _returnvalue_2 (Math|Rotator|FindLookatRotation _returnvalue FirctClick))
  (bind _returnvalue_3 (Math|Rotator|GetRotationXVector _returnvalue_2))
  (bind _returnvalue_4 (Math|Vector|CrossProduct _returnvalue_3 ActiveAxis))
  (return (Math|Vector|SelectVector (* _returnvalue_4 -1.0) _returnvalue_4 (Utilities|Enum|Equal(Enum) (CallFunction|GetActiveAxis) "NewEnumerator2"))))

(fn GetRawAngle
  (params (Normal :type Vector) (Up :type Boolean) (Start :type Vector) (End :type Vector))
  (bind _returnvalue (Math|Float|SelectFloat 1.0 -1.0 Up))
  (bind _returnvalue_2 (Class|KismetMathLibrary|VectorProjectontoNormal Start Normal))
  (bind _returnvalue_3 (Class|KismetMathLibrary|VectorProjectontoNormal End Normal))
  (bind _returnvalue_4 (Math|Vector|Distance(Vector) _returnvalue_3 _returnvalue_2))
  (bind _returnvalue_5 (* _returnvalue_4 _returnvalue))
  (bind _returnvalue_6 (* _returnvalue_5 2.0))
  (bind _returnvalue_7 (Math|Float|%(Float) _returnvalue_6 3.6e+02))
  (if (CallFunction|GetSnap)
    (bind _returnvalue_8 (Rotation|ApplyDelta _returnvalue_7))
    (return _returnvalue_8)
    (else
      (return _returnvalue_7))))

(fn SetArrowDirection
  (params (Angle :type Float%20%28double-precision%29) (Up :type Boolean))
  (bind _axis (CallFunction|GetActiveAxis))
  (bind _returnvalue (not Up))
  (bind _returnvalue_2 (Utilities|Enum|NotEqual(Enum) _axis "NewEnumerator1"))
  (bind _returnvalue_3 (select _returnvalue_2 _returnvalue Up))
  (bind (_success _disc) (CallFunction|GetActiveDisc))
  (if _success
    (Transformation|SetRelativeScale3D (Components|GetChildComponent _disc 0) (* (Math|Vector|MakeVector (Math|Float|SelectFloat -1.0 1.0 _returnvalue_3) 1.0 1.0) (Math|Float|SelectFloat 0.0 0.5 (== Angle 0.0))))
    (Transformation|SetRelativeLocation (Components|GetChildComponent _disc 0) (Math|Vector|MakeVector 15.0 (Math|Float|SelectFloat 1.5 -1.5 _returnvalue_3) 0.0) false false)))

(fn RotateActor
  (params (Rotator :type Rotator) (Actor :type Actor%20Object%20Reference) (Index :type Integer) (Angle :type Float%20%28double-precision%29))
  (bind _returnvalue (Transformation|GetActorLocation))
  (bind _returnvalue_2 (Transformation|GetActorLocation))
  (bind _axis (CallFunction|GetActiveAxis))
  (bind _initiallocation (Variables|Default|GetInitialLocation))
  (bind _initiallocation_2 (Variables|Default|GetInitialLocation))
  (bind _origin (Collision|GetActorBounds Actor false false))
  (bind _returnvalue_3 (Transformation|GetActorLocation Actor))
  (bind _output (Utilities|Array|Get(acopy) _initiallocation Index))
  (bind _output_2 (Utilities|Array|Get(acopy) _initiallocation_2 Index))
  (bind _returnvalue_4 (Utilities|Select :Index _axis :NewEnumerator0 "-1.000000, 0, 0" :NewEnumerator1 "0,-1.000000, 0" :NewEnumerator2 "0, 0,1.000000" :NewEnumerator3 "0, 0, 0" :NewEnumerator4 "0, 0, 0" :NewEnumerator5 "0, 0, 0" :NewEnumerator6 "0, 0, 0"))
  (bind _returnvalue_5 (- _output _returnvalue))
  (bind _returnvalue_6 (Math|Vector|Normalize _returnvalue_4))
  (bind _returnvalue_7 (- _origin _returnvalue_3))
  (bind _returnvalue_8 (Math|Vector|RotateVectorAroundAxis _returnvalue_5 Angle _returnvalue_6))
  (bind _returnvalue_9 (- _output_2 _returnvalue_7))
  (bind _returnvalue_10 (+ _returnvalue_2 _returnvalue_8))
  (if (CallFunction|GetRelative)
    (if (Variables|/Script/Engine.Actor|GetbReplicates (Components|GetOwner))
      (Class|BIGizmoBlueprintInterface|TransferTransformfromGizmo(Message) (Components|GetOwner) Actor "AddLocalRotation" (Math|Transform|MakeTransform "0, 0, 0" Rotator "1.000000,1.000000,1.000000"))
      (else
        (Transformation|AddActorLocalRotation Actor Rotator false false)))
    (if (CallFunction|GetPivotCenter)
      (if (Variables|/Script/Engine.Actor|GetbReplicates (Components|GetOwner))
        (Class|BIGizmoBlueprintInterface|TransferTransformfromGizmo(Message) (Components|GetOwner) Actor "SetActorLocation" (Math|Transform|MakeTransform _returnvalue_9 "0, 0, 0" "1.000000,1.000000,1.000000"))
        (else
          (Transformation|SetActorLocation Actor _returnvalue_9 false false))))
    (else
      (if (Variables|/Script/Engine.Actor|GetbReplicates (Components|GetOwner))
        (Class|BIGizmoBlueprintInterface|TransferTransformfromGizmo(Message) (Components|GetOwner) Actor "AddWorldRotation" (Math|Transform|MakeTransform "0, 0, 0" Rotator "1.000000,1.000000,1.000000"))
        (else
          (Class|Actor|AddActorWorldRotation Actor Rotator)))
      (if (CallFunction|GetPivotCenter)
        (if (Variables|/Script/Engine.Actor|GetbReplicates (Components|GetOwner))
          (Class|BIGizmoBlueprintInterface|TransferTransformfromGizmo(Message) (Components|GetOwner) Actor "SetActorLocation" (Math|Transform|MakeTransform _returnvalue_10 "0, 0, 0" "1.000000,1.000000,1.000000"))
          (else
            (Transformation|SetActorLocation Actor _returnvalue_10 false false)))))))

(fn TransformfromOut
  (params (Value :type Float%20%28double-precision%29) (AccumulatedDelta :type Float%20%28double-precision%29) (TickDelta :type Float%20%28double-precision%29))
  (Rotation|SetDiscSegment AccumulatedDelta)
  (CallFunction|SetArrowDirection AccumulatedDelta (> AccumulatedDelta 0.0))
  (bind (_discrotator _actorrotator) (CallFunction|MakeRotatorsbyActiveAxis (- AccumulatedDelta (Variables|Default|GetLastAngle))))
  (if (CallFunction|GetRelative)
    (Transformation|AddActorLocalRotation _actorrotator false false))
  (for (_array_element _array_index) (CallFunction|GetControlledActors)
    (CallFunction|RotateActor _actorrotator _array_element _array_index AccumulatedDelta))
  (Variables|Default|SetLastAngle AccumulatedDelta)
  (Rotation|RotateCircle _discrotator))

(fn ActivatefromOut
  (params (Axis :type E_TransformAxes%20Enum :default "NewEnumerator0"))
  (|CallParentFunction Axis)
  (Utilities|FlowControl|Sequence
    (:then_0
      (Utilities|Array|Clear (Variables|Default|GetInitialLocation))
      (for _array_element (CallFunction|GetControlledActors)
        (bind _state (Class|BIGizmoBlueprintInterface|GetRelativebyType(Message) (Components|GetOwner)))
        (if _state
          (Utilities|Array|Add (Variables|Default|GetInitialLocation) (.Origin (Collision|GetActorBounds _array_element false false)))
          (else
            (Utilities|Array|Add (Variables|Default|GetInitialLocation) (Transformation|GetActorLocation _array_element))))))
    (:then_1
      (bind (_success _disc) (CallFunction|GetActiveDisc))
      (if _success
        (Transformation|SetWorldRotation _disc (Math|Rotator|FindLookatRotation (Transformation|GetWorldLocation _disc) (Variables|Default|GetFirstClickLocation)) false false)
        (Transformation|SetRelativeRotation _disc (Math|Rotator|MakeRotator 0.0 0.0 (.yaw (Variables|/Script/Engine.SceneComponent|GetRelativeRotation _disc))) false false)))))

(fn DeactivatefromOut
  (Variables|Default|SetLastAngle 0.0)
  (bind (_success _disc) (CallFunction|GetActiveDisc))
  (if _success
    (Rendering|Material|SetScalarParameterValueonMaterials _disc "Angle" 0.0)
    (Transformation|SetRelativeScale3D (Components|GetChildComponent _disc 0) "0, 0, 0")
    (|CallParentFunction)))