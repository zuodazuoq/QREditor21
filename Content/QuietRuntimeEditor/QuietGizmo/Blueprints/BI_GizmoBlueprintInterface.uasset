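; Blueprint interface for the runtime editor's transform gizmo, declaring messages between the gizmo and the systems that use it, with no logic of its own.
; It covers transform mode, relative, delta, pivot, align and uniform-scale states, plus the gizmo and selected or controlled actors.
; Other messages pass transform values, start and end transforms from mouse or external input, and signal undo, redo, change and widget-close events.
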(fn ChangeRelativeState
  (params (NewState :type Boolean)))

(fn ChangeDeltaState
  (params (NewState :type Boolean)))

(fn SwitchTransformMode
  (params (Mode :type E_TransfotmType%20Enum :default "NewEnumerator0")))

(fn GetTransformMode
  (return "NewEnumerator0"))

(fn SendDeltaValue
  (params (Value :type Float%20%28double-precision%29)))

(fn GetDeltaValuebyType
  (return 0.0))

(fn SendTransformVector
  (params (NewVector :type Vector)))

(fn SendNewGizmo
  (params (NewActor :type Actor%20Object%20Reference)))

(fn GetRelativebyType
  (return false))

(fn GetDeltaStatebyType
  (return false))

(fn SendNewControlledActor
  (params (NewControlledActor :type Actor%20Object%20Reference)))

(fn GetPivotLocation
  (return false))

(fn ChangePivotState
  (params (Center :type Boolean)))

(fn GetSelectedActors
  (return 0))

(fn GetMainSelectedActor
  (return 0))

(fn SendTransformfromOut
  (params (Value :type Float%20%28double-precision%29) (AccumulatedDelta :type Float%20%28double-precision%29) (TickDelta :type Float%20%28double-precision%29)))

(fn SendStartTransformfromOut
  (params (Axis :type E_TransformAxes%20Enum :default "NewEnumerator0")))

(fn SendEndTransformfromOut)

(fn NotifyStart)

(fn GizmoOverState
  (return false))

(fn StartTransformfromMouse)

(fn EndTransformfromMouse)

(fn GetAlignState
  (return false))

(fn ChangeUniformScaleState
  (params (NewState :type Boolean)))

(fn GetScaleUniformState
  (return false))

(fn NotifyUndoChange
  (params (Undo :type Boolean) (Redo :type Boolean)))

(fn NotifyUndoCalled)

(fn NotifyWidgetClosed)

(fn NotifyEnd)

(fn NotifyRedoCalled)

(fn TransferTransformfromGizmo
  (params (Actor :type Actor%20Object%20Reference) (Type :type String) (Transform :type Transform)))

(fn NotifyonFirstChanged)