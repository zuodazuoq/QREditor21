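; BP_DummyAxes is a stand-in axes actor for the QuietGizmo runtime editor that holds a constant on-screen size.
; Each tick it scales itself from camera distance, FOV and view-direction dot product, multiplied by ScreenSize.
; It tags itself QuietGizmo and destroys itself with its owner, or after one tick without one.
; Its gizmo query functions are stubs returning empty or default values.
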(event Custom|OnOwnerDestroyed
  (params (DestroyedActor :type Actor%20Object%20Reference))
  (Actor|DestroyActor))

(event EventBeginPlay
  (bind _returnvalue (Components|GetOwner))
  (Utilities|IsValid _returnvalue
    (:Is%20Valid
      (Game|BindEventtoOnDestroyed _returnvalue (delegate Custom|OnOwnerDestroyed))
      (Variables|Default|SetTags (Utilities|Array|MakeArray "QuietGizmo")))
    (:Is%20Not%20Valid
      (Utilities|FlowControl|DelayUntilNextTick)
      (Actor|DestroyActor))))

(event EventTick
  (params (DeltaSeconds :type Float%20%28single-precision%29))
  (CallFunction|FixSizeonViewport))

(fn ConstructionScript)

(fn FixSizeonViewport
  (bind _returnvalue (Game|GetPlayerCameraManager 0))
  (bind _returnvalue_2 (Transformation|GetActorLocation))
  (bind _transformcomponent (Variables|/Script/Engine.PlayerCameraManager|GetTransformComponent _returnvalue))
  (bind _returnvalue_3 (Transformation|GetWorldLocation _transformcomponent))
  (bind _returnvalue_4 (- _returnvalue_3 _returnvalue_2))
  (bind _returnvalue_5 (* _returnvalue_4 _returnvalue_4))
  (Transformation|SetActorScale3D (Math|Conversions|ToVector(Float) (* (* (Math|Float|Sqrt (+ (.x _returnvalue_5) (.y _returnvalue_5) (.z _returnvalue_5))) (Camera|GetFOVAngle _returnvalue) (Math|Vector|DotProduct (Transformation|GetActorForwardVector _returnvalue) (Math|Rotator|GetRotationXVector (Math|Rotator|FindLookatRotation (Transformation|GetActorLocation _returnvalue) (Transformation|GetActorLocation))))) 1e-05 (Variables|Default|GetScreenSize)))))

(fn GetAlignState
  (return false))

(fn GetDeltaStatebyType
  (return false))

(fn GetDeltaValuebyType
  (return 0.0))

(fn GetMainSelectedActor
  (return 0))

(fn GetPivotLocation
  (return false))

(fn GetRelativebyType
  (return false))

(fn GetScaleUniformState
  (return false))

(fn GetSelectedActors
  (return 0))

(fn GetTransformMode
  (return "NewEnumerator0"))

(fn GizmoOverState
  (return false))