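; Runtime translate gizmo that moves itself and its controlled actors along axes or planes, or places them freely.
; Mouse rays intersect axis planes to produce local or world offsets, with optional integer-step snapping.
; The center handle traces each actor onto surfaces under its screen position, with Left Alt aligning to normals; Left Ctrl sweeps local drag moves.
; Drag transforms route through owner messages when it replicates; externally fed axis deltas apply directly.
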(fn ConstructionScript
  (|CallParentFunction))

(fn Setup
  (bind _transformsmap (Variables|Default|GetTransformsMap))
  (|CallParentFunction)
  (Utilities|Map|Add _transformsmap (Variables|Default|GetAxis_X) "NewEnumerator0")
  (Utilities|Map|Add _transformsmap (Variables|Default|GetAxis_Y) "NewEnumerator1")
  (Utilities|Map|Add _transformsmap (Variables|Default|GetAxis_Z) "NewEnumerator2")
  (Utilities|Map|Add _transformsmap (Variables|Default|GetPlane_XY) "NewEnumerator3")
  (Utilities|Map|Add _transformsmap (Variables|Default|GetPlane_XZ) "NewEnumerator4")
  (Utilities|Map|Add _transformsmap (Variables|Default|GetPlane_YZ) "NewEnumerator5")
  (Utilities|Map|Add _transformsmap (Variables|Default|GetSphere_XYZ) "NewEnumerator6"))

(fn TransformTick
  (bind _returnvalue (Game|GetPlayerController 0))
  (bind (_worldlocation _worlddirection _returnvalue_2) (Game|Player|ConvertMouseLocationToWorldSpace _returnvalue))
  (|CallParentFunction)
  (if (Utilities|Enum|Equal(Enum) (Variables|Default|GetActiveAxis) "NewEnumerator6")
    (Gizmo|Tick|Place)
    (elif _returnvalue_2
      (bind (_newintersectlocation _success) (CallFunction|IntersectMousewithTargetPlane _worldlocation _worlddirection))
      (if _success
        (if (CallFunction|GetSnap)
          (bind (_changed _offsetdelta _snappedoffset) (CallFunction|ApplyDelta _newintersectlocation))
          (if _changed
            (if (CallFunction|GetRelative)
              (CallFunction|ApplyLocalOffset _offsetdelta)
              (CallFunction|ReturnTransformVector _snappedoffset)
              (else
                (CallFunction|ApplyWorldOffset _offsetdelta)
                (CallFunction|ReturnTransformVector (+ _snappedoffset (Variables|Default|GetStartActorLocation))))))
          (else
            (Utilities|FlowControl|Sequence
              (:then_0
                (if (CallFunction|GetRelative)
                  (CallFunction|ApplyLocalOffset (Math|Vector|UnrotateVector (- _newintersectlocation (Variables|Default|GetPreviousClickLocation)) (Transformation|GetActorRotation)))
                  (CallFunction|ReturnTransformVector (CallFunction|GetRelativeOffset _newintersectlocation))
                  (else
                    (CallFunction|ApplyWorldOffset (- _newintersectlocation (Variables|Default|GetPreviousClickLocation)))
                    (CallFunction|ReturnTransformVector (Transformation|GetActorLocation)))))
              (:then_1
                (Variables|Default|SetPreviousClickLocation _newintersectlocation)))))))))

(fn IntersectMousewithTargetPlane
  (params (MouseWorldLocation :type Vector) (MouseWorlsDirection :type Vector))
  (switch Utilities|FlowControl|Switch|SwitchonE_TransformAxes (Variables|Default|GetActiveAxis)
    (:NewEnumerator0
      (bind (_active _first _second) (CallFunction|SortAxis :!label _label))
      (bind (_wide _narrow) (CallFunction|GetAxisVectors _first _second))
      (bind (_intersection _success) (CallFunction|IntersectwithAxisPlane _wide MouseWorldLocation MouseWorlsDirection false (Transformation|GetActorLocation))) ; Intersect From Mouse To Wide Plane
      (if _success
        (bind _intersection_2 (CallFunction|ProjectPlaneIntersectiontoAxis _intersection _narrow (Transformation|GetActorLocation)))
        (return _intersection_2 true)))
    (:NewEnumerator1
      (goto _label))
    (:NewEnumerator2
      (goto _label))
    (:NewEnumerator3
      (bind (_intersection_3 _success_2) (CallFunction|IntersectwithAxisPlane (Transformation|GetActorUpVector) MouseWorldLocation MouseWorlsDirection false (Transformation|GetActorLocation))) ; Intersect From Mouse To Wide Plane
      (if _success_2
        (return _intersection_3 true)))
    (:NewEnumerator4
      (bind (_intersection_4 _success_3) (CallFunction|IntersectwithAxisPlane (Transformation|GetActorRightVector) MouseWorldLocation MouseWorlsDirection false (Transformation|GetActorLocation))) ; Intersect From Mouse To Wide Plane
      (if _success_3
        (return _intersection_4 true)))
    (:NewEnumerator5
      (bind (_intersection_5 _success_4) (CallFunction|IntersectwithAxisPlane (Transformation|GetActorForwardVector) MouseWorldLocation MouseWorlsDirection false (Transformation|GetActorLocation))) ; Intersect From Mouse To Wide Plane
      (if _success_4
        (return _intersection_5 true)))
    (:NewEnumerator6
      (return "0, 0, 0" false))))

(fn HandleMouseClick
  (bind _returnvalue (Game|GetPlayerController 0))
  (bind (_worldlocation _worlddirection _returnvalue_2) (Game|Player|ConvertMouseLocationToWorldSpace _returnvalue))
  (|CallParentFunction)
  (if _returnvalue_2
    (bind _newintersectlocation (CallFunction|IntersectMousewithTargetPlane _worldlocation _worlddirection))
    (Variables|Default|SetFirstClickLocation _newintersectlocation)
    (Variables|Default|SetPreviousClickLocation _newintersectlocation)
    (Variables|Default|SetStartActorLocation (Transformation|GetActorLocation))
    (if (Utilities|Enum|Equal(Enum) (CallFunction|GetActiveAxis) "NewEnumerator6")
      (for _array_element (Variables|Default|GetStartLocations)
        (Utilities|Array|Add (LocalVariables|GetRelativeLocations) (- _array_element (Transformation|GetActorLocation))))
      (Variables|Default|SetStartLocations (LocalVariables|GetRelativeLocations)))))

(fn ApplyDelta
  (params (WorldLocation :type Vector))
  (bind _firstclicklocation (Variables|Default|GetFirstClickLocation))
  (bind _returnvalue (- WorldLocation _firstclicklocation))
  (bind (_dividedoffsetint _dividedoffsetfloat) (CallFunction|DivisionOffsetbyDeltaValue (Math|Vector|SelectVector (Math|Vector|UnrotateVector _returnvalue (Transformation|GetActorRotation)) _returnvalue (CallFunction|GetRelative))))
  (Utilities|CompareIntVectors _dividedoffsetint (Variables|Default|GetCurrentSnapIntVector)
    (:Changed
      (bind _deltaoffset (CallFunction|DeltaSnappedOffset _dividedoffsetint (Variables|Default|GetCurrentSnapIntVector)))
      (Variables|Default|SetCurrentSnapIntVector _dividedoffsetint)
      (return true _deltaoffset _dividedoffsetfloat))
    (:Unchanged
      (return false "0, 0, 0" "0, 0, 0"))))

(fn DivisionOffsetbyDeltaValue
  (params (Offset :type Vector))
  (bind (_x _y _z) (Math|Vector|BreakVector Offset))
  (bind _snapvalue (CallFunction|GetSnapValue))
  (bind _returnvalue (Math|Float|Division(WholeandRemainder) _z _snapvalue))
  (bind _returnvalue_2 (Math|Float|Division(WholeandRemainder) _x _snapvalue))
  (bind _returnvalue_3 (Math|Float|Division(WholeandRemainder) _y _snapvalue))
  (return (Utilities|Struct|MakeIntVector _returnvalue_2 _returnvalue_3 _returnvalue) (* (Math|Vector|MakeVector (Math|Conversions|ToFloat(Integer) _returnvalue_2) (Math|Conversions|ToFloat(Integer) _returnvalue_3) (Math|Conversions|ToFloat(Integer) _returnvalue)) (CallFunction|GetSnapValue))))

(fn ApplyWorldOffset
  (params (Offset :type Vector))
  (Transformation|AddActorWorldOffset self Offset)
  (for _array_element (CallFunction|GetControlledActors)
    (if (Variables|/Script/Engine.Actor|GetbReplicates (Components|GetOwner))
      (Class|BIGizmoBlueprintInterface|TransferTransformfromGizmo(Message) (Components|GetOwner) _array_element "OffsetWorld" (Math|Transform|MakeTransform Offset "0, 0, 0" "1.000000,1.000000,1.000000"))
      (else
        (Transformation|AddActorWorldOffset _array_element Offset (Game|Player|IsInputKeyDown (Game|GetPlayerController 0) "LeftControl"))))))

(fn ApplyLocalOffset
  (params (Offset :type Vector))
  (Transformation|AddActorLocalOffset self Offset false false)
  (for _array_element (CallFunction|GetControlledActors)
    (if (Variables|/Script/Engine.Actor|GetbReplicates (Components|GetOwner))
      (Class|BIGizmoBlueprintInterface|TransferTransformfromGizmo(Message) (Components|GetOwner) _array_element "OffsetLocal" (Math|Transform|MakeTransform Offset "0, 0, 0" "1.000000,1.000000,1.000000"))
      (else
        (Transformation|AddActorLocalOffset _array_element Offset (Game|Player|IsInputKeyDown (Game|GetPlayerController 0) "LeftControl") false)))))

(fn HandleMouseRelease
  (|CallParentFunction)
  (Variables|Default|SetPreviousClickLocation "0, 0, 0")
  (Variables|Default|SetStartActorLocation "0, 0, 0")
  (Variables|Default|SetFirstClickLocation "0, 0, 0")
  (Variables|Default|SetCurrentSnapIntVector (Utilities|Struct|MakeIntVector 0 0)))

(fn DeltaSnappedOffset
  (params (First :type Int%20Vector%20Structure%20%28by%20ref%29) (Second :type Int%20Vector%20Structure%20%28by%20ref%29))
  (bind (_x _y _z) (Utilities|Struct|BreakIntVector Second))
  (bind (_x_2 _y_2 _z_2) (Utilities|Struct|BreakIntVector First))
  (return (* (Math|Vector|MakeVector (Math|Conversions|ToFloat(Integer) (- _x_2 _x)) (Math|Conversions|ToFloat(Integer) (- _y_2 _y)) (Math|Conversions|ToFloat(Integer) (- _z_2 _z))) (CallFunction|GetSnapValue))))

(fn TransformfromOut
  (params (Value :type Float%20%28double-precision%29) (AccumulatedDelta :type Float%20%28double-precision%29) (TickDelta :type Float%20%28double-precision%29))
  (bind _axis (CallFunction|GetActiveAxis))
  (bind _returnvalue (Utilities|Select :Index _axis :NewEnumerator0 (Math|Vector|MakeVector TickDelta 0.0 0.0) :NewEnumerator1 (Math|Vector|MakeVector 0.0 TickDelta 0.0) :NewEnumerator2 (Math|Vector|MakeVector 0.0 0.0 TickDelta) :NewEnumerator3 "0, 0, 0" :NewEnumerator4 "0, 0, 0" :NewEnumerator5 "0, 0, 0" :NewEnumerator6 "0, 0, 0"))
  (if (CallFunction|GetRelative)
    (Transformation|AddActorLocalOffset _returnvalue false false)
    (for _array_element (CallFunction|GetControlledActors)
      (Transformation|AddActorLocalOffset _array_element _returnvalue false false))
    (else
      (Transformation|AddActorWorldOffset _returnvalue)
      (for _array_element_2 (CallFunction|GetControlledActors)
        (Transformation|AddActorWorldOffset _array_element_2 _returnvalue)))))

(fn GetRelativeOffset
  (params (CurrentLocation :type Vector))
  (bind _returnvalue (Transformation|GetActorRotation))
  (bind _firstclicklocation (Variables|Default|GetFirstClickLocation))
  (bind _returnvalue_2 (- CurrentLocation _firstclicklocation))
  (bind _returnvalue_3 (Math|Vector|UnrotateVector _returnvalue_2 _returnvalue))
  (return (Utilities|Select :Index (CallFunction|GetActiveAxis) :NewEnumerator0 (Math|Vector|MakeVector (.x _returnvalue_3) 0.0 0.0) :NewEnumerator1 (Math|Vector|MakeVector 0.0 (.y _returnvalue_3) 0.0) :NewEnumerator2 (Math|Vector|MakeVector 0.0 0.0 (.z _returnvalue_3)) :NewEnumerator3 (Math|Vector|MakeVector (.x _returnvalue_3) (.y _returnvalue_3) 0.0) :NewEnumerator4 (Math|Vector|MakeVector (.x _returnvalue_3) 0.0 (.z _returnvalue_3)) :NewEnumerator5 (Math|Vector|MakeVector 0.0 (.y _returnvalue_3) (.z _returnvalue_3)) :NewEnumerator6 (Math|Vector|MakeVector (.x _returnvalue_3) (.y _returnvalue_3) (.z _returnvalue_3)))))

(fn Place
  (bind _returnvalue (Game|GetPlayerController 0))
  (bind (_worldlocation _worlddirection) (Game|Player|ConvertMouseLocationToWorldSpace _returnvalue))
  (Transformation|SetActorLocation (+ _worldlocation (* _worlddirection (.Distance (CallFunction|ProjectLocationtoScreenPlane (Variables|Default|GetStartActorLocation))))) false false)
  (for _array_element (CallFunction|GetControlledActors)
    (Gizmo|Tick|PlaceActor _array_element))
  (CallFunction|ReturnTransformVector (Transformation|GetActorLocation)))

(fn PlaceActor
  (params (Actor :type Actor%20Object%20Reference))
  (bind _returnvalue (Game|GetPlayerController 0))
  (bind _actors (CallFunction|GetControlledActors))
  (bind _returnvalue_2 (Transformation|GetActorLocation))
  (bind _startlocations (Variables|Default|GetStartLocations))
  (bind _returnvalue_3 (Utilities|Array|FindItem _actors Actor))
  (bind _returnvalue_4 (Game|Player|IsInputKeyDown _returnvalue "LeftAlt"))
  (bind _output (Utilities|Array|Get(acopy) _startlocations _returnvalue_3))
  (bind _returnvalue_5 (+ _returnvalue_2 _output))
  (bind (_success _worldposition _worlddirection _distance) (CallFunction|ProjectLocationtoScreenPlane _returnvalue_5))
  (bind (_success_2 _worldposition_2 _worlddirection_2) (CallFunction|ProjectLocationtoScreenPlane _returnvalue_5))
  (bind _returnvalue_6 (* _worlddirection _distance))
  (bind _returnvalue_7 (+ _worldposition _returnvalue_6))
  (bind (_outhit _returnvalue_8) (Collision|LineTraceByChannel _worldposition_2 (+ _worldposition_2 (* _worlddirection_2 (Variables|Default|GetTraceDistance))) "TraceTypeQuery1" true (CallFunction|GetControlledActors) "None"))
  (if _returnvalue_8
    (if (Variables|/Script/Engine.Actor|GetbReplicates (Components|GetOwner))
      (Class|BIGizmoBlueprintInterface|TransferTransformfromGizmo(Message) (Components|GetOwner) Actor "SetActorLocation" (Math|Transform|MakeTransform (.Location (Collision|BreakHitResult _outhit)) "0, 0, 0" "1.000000,1.000000,1.000000"))
      (if _returnvalue_4
        (Class|BIGizmoBlueprintInterface|TransferTransformfromGizmo(Message) (Components|GetOwner) Actor "SetActorRotation" (Math|Transform|MakeTransform "0, 0, 0" (Math|Rotator|MakeRotfromZX (.ImpactNormal (Collision|BreakHitResult _outhit)) (Transformation|GetActorForwardVector Actor)) "1.000000,1.000000,1.000000")))
      (else
        (Transformation|SetActorLocation Actor (.Location (Collision|BreakHitResult _outhit)) false false)
        (if _returnvalue_4
          (Transformation|SetActorRotation Actor (Math|Rotator|MakeRotfromZX (.ImpactNormal (Collision|BreakHitResult _outhit)) (Transformation|GetActorForwardVector Actor))))))
    (elif (Variables|/Script/Engine.Actor|GetbReplicates (Components|GetOwner))
      (Class|BIGizmoBlueprintInterface|TransferTransformfromGizmo(Message) (Components|GetOwner) Actor "SetActorLocation" (Math|Transform|MakeTransform _returnvalue_7 "0, 0, 0" "1.000000,1.000000,1.000000"))
      (if _returnvalue_4
        (Class|BIGizmoBlueprintInterface|TransferTransformfromGizmo(Message) (Components|GetOwner) Actor "SetActorRotation"))
      (else
        (Transformation|SetActorLocation Actor _returnvalue_7 false false)
        (if _returnvalue_4
          (Transformation|SetActorRotation Actor))))))

(fn ProjectLocationtoScreenPlane
  (params (Location :type Vector%20%28by%20ref%29))
  (bind _returnvalue (Game|GetPlayerController 0))
  (bind _returnvalue_2 (Game|GetPlayerController 0))
  (bind (_screenposition _returnvalue_3) (Class|GameplayStatics|ProjectWorldtoScreen _returnvalue Location false))
  (bind (_worldposition _worlddirection _returnvalue_4) (Class|GameplayStatics|DeprojectScreentoWorld _returnvalue_2 _screenposition))
  (if _returnvalue_3
    (return _returnvalue_4 _worldposition _worlddirection (Math|Vector|Distance(Vector) _worldposition Location))))