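; Name-keyed cache of dynamic materials for the runtime material editor.
; InjectMaterials takes a map with JSON values, reads each "Name" field and stores the map's key under that name; EjectMaterials returns the cache.
; TakeMaterialName does a reverse lookup from material to name by matching indices in the value and key arrays.
; Rename moves an entry to a new key by removing and re-adding it.
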(fn EjectMaterials
  (return (Variables|Default|GetMaterials)))

(fn InjectMaterials
  (params (Materials :type Map%20of%20Material%20Instance%20Dynamic%20Object%20References%20to%20Structs))
  (bind _keys (Utilities|Map|Keys Materials))
  (for _array_element _keys
    (bind _outvalue (|GetJsonField (.Value (Utilities|Map|Find Materials _array_element)) "Name"))
    (Utilities|Map|Add (Variables|Default|GetMaterials) _outvalue _array_element)))

(fn TakeMaterialName
  (params (ItemToFind :type Object%20Object%20Reference%20%28by%20ref%29))
  (bind _values (Utilities|Map|Values (Variables|Default|GetMaterials)))
  (bind _pinned (Utilities|Pin (Utilities|Array|FindItem _values ItemToFind)))
  (if (>= _pinned 0)
    (bind _keys (Utilities|Map|Keys (Variables|Default|GetMaterials)))
    (return (Utilities|Array|Get(acopy) _keys _pinned))))

(fn Rename
  (params (CurrentName :type String) (NewName :type String))
  (bind _pinned (Utilities|Pin (.Value (Utilities|Map|Find (Variables|Default|GetMaterials) CurrentName))))
  (Utilities|Map|Remove (Variables|Default|GetMaterials) CurrentName)
  (Utilities|Map|Add (Variables|Default|GetMaterials) NewName _pinned))